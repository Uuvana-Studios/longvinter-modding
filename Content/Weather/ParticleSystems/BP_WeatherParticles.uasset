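; BP_WeatherParticles is a weather actor that groups particle systems for rain, colliding rain, cheap ground splashes and snowfall.
; Its Construction Script pushes rain, splash and snow amount variables into named parameters on those systems.
; A shared WindSpeed vector feeds both rain systems and the snow, but not the splashes.
; The event graph has no active logic, and its rain collision event is empty.
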(event OnParticleCollide(PS_RainFall)
  (params (EventName :type Name :default "None") (EmitterTime :type Float%20%28single-precision%29) (ParticleTime :type Integer) (Location :type Vector :default "0, 0, 0") (Velocity :type Vector :default "0, 0, 0") (Direction :type Vector :default "0, 0, 0") (Normal :type Vector :default "0, 0, 0") (BoneName :type Name :default "None") (PhysMat :type Physical%20Material%20Object%20Reference)))

(event EventBeginPlay)

(event Collision|EventActorBeginOverlap
  (params (OtherActor :type Actor%20Object%20Reference)))

(event EventTick
  (params (DeltaSeconds :type Float%20%28single-precision%29)))

(fn ConstructionScript
  (bind _wind_speed (Variables|Default|GetWind%20Speed))
  (bind _ps_snowfall (Variables|Default|GetPS_SnowFall))
  (Effects|Components|ParticleSystem|SetFloatParameter (Variables|Default|GetPS_RainFall) "RainRate" (Variables|Default|GetRainAmount))
  (Effects|Components|ParticleSystem|SetFloatParameter (Variables|Default|GetPS_RainCPUCollide) "RainCPU" (Variables|Default|GetCollidingRainAmount))
  (Effects|Components|ParticleSystem|SetFloatParameter (Variables|Default|GetPS_RainCheapGroundSplashes) "GroundSplashAmount" (Variables|Default|GetGround%20Slpash%20Amount))
  (Effects|Components|ParticleSystem|SetFloatParameter _ps_snowfall "SnowFastAmount" (Variables|Default|GetSnow%20Amount%20Fast))
  (Effects|Components|ParticleSystem|SetFloatParameter _ps_snowfall "SnowSlowAmount" (Variables|Default|GetSnow%20Amount%20Slow))
  (Effects|Components|ParticleSystem|SetFloatParameter _ps_snowfall "SnowCloudsAmount" (Variables|Default|GetSnow%20Clouds%20Amount))
  (Effects|Components|ParticleSystem|SetVectorParameter (Variables|Default|GetPS_SnowFall) "WindSpeed" _wind_speed)
  (Effects|Components|ParticleSystem|SetVectorParameter (Variables|Default|GetPS_RainCPUCollide) "WindSpeed" _wind_speed)
  (Effects|Components|ParticleSystem|SetVectorParameter (Variables|Default|GetPS_RainFall) "WindSpeed" _wind_speed))