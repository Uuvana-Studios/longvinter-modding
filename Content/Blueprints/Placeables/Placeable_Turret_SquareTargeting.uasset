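; Turret placeable variant that uses a box-shaped targeting range.
; The construction script sizes the Box component from the BoxExtent variable, and GetTurretRangeColComp returns that box as the turret's range collision.
; When an actor stops overlapping the box, it is passed to PlayerLeftTurretRadius; no other turret logic is implemented in this Blueprint.
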(event OnComponentEndOverlap(Box)
  (params (OverlappedComponent :type Primitive%20Component%20Object%20Reference) (OtherActor :type Actor%20Object%20Reference) (OtherComp :type Primitive%20Component%20Object%20Reference) (OtherBodyIndex :type Integer))
  (CallFunction|PlayerLeftTurretRadius OtherActor))

(event EventBeginPlay
  (|CallParentFunction) ; This node is disabled and will not be called.\nDrag off pins to build functionality.
)

(event Collision|EventActorBeginOverlap
  (params (OtherActor :type Actor%20Object%20Reference)))

(event EventTick
  (params (DeltaSeconds :type Float%20%28single-precision%29)))

(fn ConstructionScript
  (|CallParentFunction)
  (Components|Box|SetBoxExtent (Variables|Default|GetBox) (Variables|Settings|GetBox%20Extent) true))

(fn GetTurretRangeColComp
  (return (Variables|Default|GetBox)))