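; Casino lighthouse location that unpacks its Blueprint components into standalone world actors on BeginPlay.
; The server drops the seagull and windsock components and respawns child actors, flagging placeables as unsaved game-mode spawns and hiding chicken dice table meshes.
; Remote instances copy static meshes into new actors and hide the originals.
; The main island and floor meshes use A_IslandMeshNonDistanceField; the others keep their materials and ignore the Camera channel.
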(event EventBeginPlay
  (Networking|SwitchHasAuthority
    (:Authority
      (Components|DestroyComponent (Variables|Default|GetLV_Seagul))
      (for _array_element (Actor|GetComponentsByClass self "/Script/Engine.ChildActorComponent")
        (bind _returnvalue (Game|SpawnActorfromClass (Variables|/Script/Engine.ChildActorComponent|GetChildActorClass _array_element) (Transformation|GetWorldTransform _array_element) "Undefined" 0 0))
        (bind _asa_placeable (Utilities|Casting|CastToA_Placeable _returnvalue))
        (Variables|/Game/Blueprints/Placeables/A_Placeable.A_Placeable_C|SetSavePlaceable _asa_placeable false)
        (Variables|/Game/Blueprints/Placeables/A_Placeable.A_Placeable_C|SetSpawnedByGameMode _asa_placeable true)
        (bind _asa_placeable_chicken_dice_game_table (Utilities|Casting|CastToA_Placeable_ChickenDiceGameTable _asa_placeable))
        (Development|SetHiddeninGame (Variables|/Game/Blueprints/Placeables/A_Placeable.A_Placeable_C|GetSM_Placeable _asa_placeable_chicken_dice_game_table) true false))
      (for _array_element_2 (Actor|GetComponentsByClass self "/Script/Engine.ChildActorComponent")
        (Components|DestroyComponent _array_element_2)))
    (:Remote
      (for _array_element_3 (Actor|GetComponentsByClass self "/Script/Engine.StaticMeshComponent")
        (if (Math|Boolean|ORBoolean (== _array_element_3 (Variables|Default|GetSM_CasinoLighthouse_KallioMainIsland)) (== _array_element_3 (Variables|Default|GetSM_CasinoLighthouse_CasinoSecondFloor)) (== _array_element_3 (Variables|Default|GetSM_CasinoLighthouse_CasinoFirstFloor)) (== (Variables|Default|GetSM_CasinoLighthouse_CasinoThirdFloor) _array_element_3) (== (Variables|Default|GetSM_CasinoLighthouse_FishingIsland) _array_element_3))
          (CallFunction|CreateStaticMesh _array_element_3)
          (else
            (bind _returnvalue_2 (Game|SpawnActorfromClass "/Script/Engine.StaticMeshActor" (Transformation|GetWorldTransform _array_element_3) "Undefined" 0 0))
            (Components|StaticMesh|SetStaticMesh (Variables|/Script/Engine.StaticMeshActor|GetStaticMeshComponent _returnvalue_2) (Variables|/Script/Engine.StaticMeshComponent|GetStaticMesh _array_element_3))
            (for (_array_element_4 _array_index) (Rendering|Material|GetMaterials _array_element_3)
              (Rendering|Material|SetMaterial (Variables|/Script/Engine.StaticMeshActor|GetStaticMeshComponent _returnvalue_2) _array_index _array_element_4))
            (Collision|SetCollisionResponsetoChannel (Variables|/Script/Engine.StaticMeshActor|GetStaticMeshComponent _returnvalue_2) "ECC_Camera" "ECR_Ignore")))
        (Rendering|SetVisibility _array_element_3 false false)))))

(fn ConstructionScript)

(fn CreateStaticMesh
  (params (self2 :type Static%20Mesh%20Component%20Object%20Reference))
  (bind _returnvalue (Game|SpawnActorfromClass "/Game/Meshes/LightHouseCasino/A_IslandMeshNonDistanceField.A_IslandMeshNonDistanceField_C" (Transformation|GetWorldTransform self2) "Undefined" 0 0))
  (Components|StaticMesh|SetStaticMesh (Variables|/Game/Meshes/LightHouseCasino/A_IslandMeshNonDistanceField.A_IslandMeshNonDistanceField_C|GetStaticMesh _returnvalue) (Variables|/Script/Engine.StaticMeshComponent|GetStaticMesh self2)))