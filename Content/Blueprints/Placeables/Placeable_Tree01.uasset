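; Choppable, respawning tree placeable with randomized height and yaw, and snow or autumn leaves set by flags or ground surface.
; Server-bound damage accepts allowed tool types, rolling buff-scaled, capped loot and optional extra drops, with multicast sound and squash animation.
; At zero health it drops loot, grants a woodcutter achievement and resets after a delay.
; RepNotify swaps depleted mesh and collision; overlap checks destroy trees blocked by homes or placeables.
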(event Custom|Damage
  (params (DamagedActor :type Actor%20Object%20Reference) (Damage :type Float%20%28single-precision%29) (DamageType :type Damage%20Type%20Object%20Reference) (InstigatedBy :type Controller%20Object%20Reference) (DamageCauser :type Actor%20Object%20Reference))
  (bind _returnvalue (Transformation|GetActorTransform))
  (bind _returnvalue_2 (Utilities|GetClass DamageType))
  (bind (_itemchance _extrachance) (Utilities|DamageMultipliertoChance Damage))
  (Utilities|NoSnowballProjectile DamageType
    (:No
      (bind _aspc_longvinter (Utilities|Casting|CastToPC_Longvinter DamageCauser)
        (:then
          _)
        (:CastFailed
          _))
      (CallFunction|PlayHitSoundMulticast (Transformation|GetActorLocation) (Pawn|GetControlledPawn _aspc_longvinter))
      (if (Utilities|Array|ContainsItem (Variables|Default|GetDamageTypes) _returnvalue_2)
        (if (<= (Variables|Default|GetHealth) 0.0)
          (CallFunction|SpawnLoot (Pawn|GetControlledPawn _aspc_longvinter))
          (Variables|DoNotEdit|SetDepleted true)
          (CallFunction|Reset)
          (Utilities|IsValid DamageCauser
            (:Is%20Valid
              (bind _asplayer_controller (Utilities|Casting|CastToPlayerController DamageCauser))
              (bind _asthird_person_character (Utilities|Casting|CastToThirdPersonCharacter (Pawn|GetControlledPawn _asplayer_controller)))
              (Default|GiveWoodCutterAchivement _asthird_person_character _asplayer_controller)
              (Networking|ForceNetUpdate)))
          (else
            (bind _dropmultiplier (CallFunction|GetDropBuff (Pawn|GetControlledPawn _aspc_longvinter)))
            (if (< (Math|Random|RandomFloat) (* _itemchance _dropmultiplier))
              (CallFunction|SpawnLoot (Pawn|GetControlledPawn _aspc_longvinter)))
            (Utilities|CanExtraSpawn
              (:then
                (if (< (Math|Random|RandomFloat) _extrachance)
                  (CallFunction|SpawnExtraItem (Math|Transform|MakeTransform (Math|Vector|MakeVector (+ (.x (.location _returnvalue)) (Math|Random|RandomFloatinRange -1e+02 1e+02)) (+ (.y (.location _returnvalue)) (Math|Random|RandomFloatinRange -1e+02 1e+02)) (.z (.location _returnvalue))) (.rotation _returnvalue) (.scale _returnvalue)))))
              (:false
                _))
            (Networking|ForceNetUpdate :!label _label)))
        (elif (Utilities|Array|ContainsItem (Utilities|Array|MakeArray "/Game/Blueprints/DamageType/DT_Melee.DT_Melee_C" "/Game/Blueprints/DamageType/DT_MeleeOre.DT_MeleeOre_C" "/Game/Blueprints/DamageType/DT_MeleeWood.DT_MeleeWood_C" "/Game/Blueprints/DamageType/DT_MeleeOreAdvanced.DT_MeleeOreAdvanced_C") _returnvalue_2)
          (Default|ErrorMessageOC _aspc_longvinter "Current tool can't chop this wood")
          (goto _label)
          (else
            (goto _label)))))))

(event Custom|CheckOverlaps
  (bind _overlappingactors (Collision|GetOverlappingActors "/Game/Blueprints/A_Home.A_Home_C" :!class /Script/Engine.Actor))
  ;[1 1 1] Check Overlaps
  (if (== (Utilities|Array|Length _overlappingactors) 0)
    (if (== (Utilities|Array|Length (Collision|GetOverlappingActors "/Game/Blueprints/Placeables/A_Placeable.A_Placeable_C" :!class /Script/Engine.Actor)) 0)
      (if (not true)
        (Actor|DestroyActor))
      (else
        (Actor|DestroyActor)))
    (else
      (for _array_element _overlappingactors
        (bind _asa_home (Utilities|Casting|CastToA_Home _array_element))
        (if (Class|PrimitiveComponent|IsOverlappingComponent (Variables|/Game/Blueprints/A_Home.A_Home_C|GetStaticMesh _asa_home) (Variables|Default|GetCollisionCheck))
          (Actor|DestroyActor))))))

(event Custom|SpawnLoot
  (params (Pawn :type Pawn%20Object%20Reference))
  (bind _returnvalue (Transformation|GetActorTransform))
  (bind _dropitemcap (Variables|Values|GetDropItemCap))
  (bind (_dropmultiplier _hasbuff) (CallFunction|GetDropBuff Pawn))
  (Utilities|CheckItemDropCap (select _hasbuff (Math|Float|Floor (* _dropitemcap _dropmultiplier)) _dropitemcap) (Variables|DoNotEdit|GetSpawnedItems))
  (bind _itemdata (CallFunction|GetItemwithID (Variables|Default|GetDropItemIndex)))
  (Game|SpawnActorfromClass "/Game/Blueprints/A_Item.A_Item_C" (Math|Transform|MakeTransform (Math|Vector|MakeVector (+ (.x (.location _returnvalue)) (Math|Random|RandomFloatinRange -1e+02 1e+02)) (+ (.y (.location _returnvalue)) (Math|Random|RandomFloatinRange -1e+02 1e+02)) (.z (.location _returnvalue))) (.rotation _returnvalue) (.scale _returnvalue)) "AdjustIfPossibleButAlwaysSpawn" 0 _itemdata false false 1.0 false 0 "/Game/Audio/Pickup.Pickup" false 25 false false false 140 false 0 0 0)
  (Networking|ForceNetUpdate))

(event Custom|PlayHitSoundMulticast
  (params (Location :type Vector) (DamageCauser :type Actor%20Object%20Reference))
  (Audio|PlaySoundatLocation (Variables|Default|GetHitSound) Location "0, 0, 0" 1.0 1.0 0.0 0 0 0)
  (bind _scale (Timeline|Timeline_0 PlayFromStart)
    (:Update
      (Transformation|SetWorldScale3D (Variables|Default|GetScene) (Math|Vector|MakeVector 1.0 1.0 _scale)))))

(event Custom|Reset
  (Utilities|FlowControl|Delay (* (Variables|Values|GetRespawnTimeInMinutes) 6e+01))
  (Variables|Default|SetHealth (Variables|DoNotEdit|GetSavedHealth))
  (Variables|DoNotEdit|SetDepleted false)
  (CallFunction|CheckOverlaps)
  (Networking|FlushNetDormancy)
  (Variables|DoNotEdit|SetSpawnedItems 0)
  (Variables|DoNotEdit|SetSpawnedExtraItems 0))

(event Custom|HitAnim
  ;[1 1 1] HitAnim
)

(event EventBeginPlay
  (Networking|SwitchHasAuthority
    (:Authority
      (EventDispatchers|BindEventtoOnTakeAnyDamage (delegate Custom|Damage))
      (CallFunction|CheckOverlaps)
      (Utilities|FlowControl|Delay 3e+01)
      (CallFunction|CheckOverlaps))))

(fn ConstructionScript
  (bind _returnvalue (Transformation|GetActorLocation))
  (bind _sm_placeable (Variables|Default|GetSM_Placeable))
  (bind _returnvalue_2 (Transformation|GetWorldScale _sm_placeable))
  (Utilities|FlowControl|Sequence
    (:then_0
      (Variables|DoNotEdit|SetSavedHealth (Variables|Default|GetHealth))
      (Variables|DoNotEdit|SetDefaultMesh (Variables|/Script/Engine.StaticMeshComponent|GetStaticMesh (Variables|Default|GetSM_Placeable)))
      (Transformation|SetWorldScale3D (Variables|Default|GetSM_Placeable) (Math|Vector|MakeVector (.x _returnvalue_2) (.y _returnvalue_2) (Math|Random|RandomFloatinRange 0.8 1.1)))
      (Transformation|SetWorldRotation (Variables|Default|GetSM_Placeable) (Math|Rotator|MakeRotator 0.0 0.0 (.yaw (Math|Random|RandomRotator false))) false false))
    (:then_1
      (if (Variables|Default|GetForceSnow)
        ;[1 1 1] SetSnow
        (Rendering|Material|SetMaterial (Variables|Default|GetSM_Placeable) 0 (Variables|Default|GetSnowLeavesMaterial) :!label _label)
        (Variables|Default|SetForceSnow true)
        (|CallParentFunction :!label _label_2)
        (elif (Variables|Default|GetForceAutumn)
          (Rendering|Material|SetMaterial (Variables|Default|GetSM_Placeable) 0 (Variables|Default|GetAutumnLeavesMaterial))
          (else
            (bind (_outhit _returnvalue_3) (Collision|LineTraceByChannel (+ _returnvalue "0, 0,100.000000") (- _returnvalue "0, 0,100.000000") "TraceTypeQuery3" false 0 "None" true "(R=1.000000,G=0.000000,B=0.000000,A=1.000000)" "(R=0.000000,G=1.000000,B=0.000000,A=1.000000)" 1.0))
            (if _returnvalue_3
              (switch Utilities|FlowControl|Switch|SwitchonEPhysicalSurface (Collision|GetSurfaceType _outhit)
                (:SurfaceType6
                  (goto _label))
                (:SurfaceType8
                  (Rendering|Material|SetMaterial (Variables|Default|GetSM_Placeable) 0 (Variables|Default|GetAutumnLeavesMaterial))
                  (Variables|Default|SetForceAutumn true)
                  (goto _label_2))))))))))

(fn OnRepDepleted
  (bind _sm_placeable (Variables|Default|GetSM_Placeable))
  (bind _savedmaterials (Variables|Default|GetSavedMaterials))
  (if (Variables|DoNotEdit|GetDepleted)
    (Components|StaticMesh|SetStaticMesh (Variables|Default|GetSM_Placeable) (Variables|Default|GetDepletedMesh))
    (Collision|SetActorEnableCollision false)
    (else
      (Physics|SetSimulatePhysics (Variables|Default|GetSM_Placeable) false)
      (Components|StaticMesh|SetStaticMesh _sm_placeable (Variables|DoNotEdit|GetDefaultMesh))
      (for (_ _array_index) _savedmaterials
        (Rendering|Material|SetMaterial _sm_placeable _array_index (Utilities|Array|Get(acopy) _savedmaterials _array_index)))
      (Collision|SetActorEnableCollision true))))

(fn SpawnExtraItem
  (params (SpawnTransform :type Transform))
  (Utilities|CheckItemDropCap (Variables|Values|GetExtraItemDropCap) (Variables|DoNotEdit|GetSpawnedExtraItems))
  (bind _itemdata (CallFunction|GetItemwithID (Variables|Values|GetExtraItemIndex)))
  (Game|SpawnActorfromClass "/Game/Blueprints/A_Item.A_Item_C" SpawnTransform "AdjustIfPossibleButAlwaysSpawn" 0 _itemdata false false 1.0 false 0 "/Game/Audio/Pickup.Pickup" false 25 false false false 140 false 0 0 0))

(fn OnRepForceSnow
  (if (Variables|Default|GetForceSnow)
    (Rendering|Material|SetMaterial (Variables|Default|GetSM_Placeable) 0 (Variables|Default|GetSnowLeavesMaterial))))

(fn OnRepForceAutumn
  (if (Variables|Default|GetForceAutumn)
    (Rendering|Material|SetMaterial (Variables|Default|GetSM_Placeable) 0 (Variables|Default|GetAutumnLeavesMaterial))))

(fn GetDropBuff
  (params (TPC :type Actor%20Object%20Reference))
  (bind _asthird_person_character (Utilities|Casting|CastToThirdPersonCharacter TPC))
  (bind (_returnvalue _effect_multiplier) (Default|IsBuffActive (Variables|/Game/ThirdPersonCPP/Blueprints/ThirdPersonCharacter.ThirdPersonCharacter_C|GetBuffComponent _asthird_person_character) (Utilities|Struct|MakeS_BuffValuesRename1 "NewEnumerator22")))
  (if _returnvalue
    (return (+ (/ (Math|Conversions|ToFloat(Integer) _effect_multiplier) 1e+02) 1.0) true)
    (else
      (return 1.0 false))))