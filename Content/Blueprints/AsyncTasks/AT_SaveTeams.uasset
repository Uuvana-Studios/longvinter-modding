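; AT_SaveTeams is a task object that saves the game mode's team list to disk.
; Execute copies Gamemode.TeamsList into the SaveGame object and writes it to the AllTeams slot with SaveGameToSlot, printing debug messages and the team count.
; MakeVendorStuct, which flattens a vendor into a player-vendor struct, and an unwired transform duplicate check are also present, but Execute uses neither.
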(event EventExecute
  (bind _savegame (Variables|Default|GetSaveGame))
  (Variables|/Game/Blueprints/Server/SG_TeamList.SG_TeamList_C|SetteamsList _savegame (Variables|/Game/Blueprints/Server/GM_Longvinter.GM_Longvinter_C|GetteamsList (Variables|Default|GetGamemode)))
  (Development|PrintString 0 "Start Writing")
  (SaveGame|SaveGametoSlot _savegame "AllTeams")
  (Development|PrintString 0 "Finish Writing")
  (Development|PrintString 0 (Utilities|String|Append "DONE SAVING " (Utilities|String|ToString(Integer) (Utilities|Map|Length (Variables|/Game/Blueprints/Server/GM_Longvinter.GM_Longvinter_C|GetteamsList (Variables|Default|GetGamemode)))) " TEAMS")))

(fn MakeVendorStuct
  (params (vendor :type A%20Vendor%20Player%20Placed%20Object%20Reference))
  (bind _solditems (LocalVariables|GetSoldItems))
  (bind _itemstock (LocalVariables|GetItemStock))
  (bind _prices (LocalVariables|GetPrices))
  (bind _boughtitems (LocalVariables|GetBoughtItems))
  (for _array_element (Variables|/Game/Blueprints/Vendor/A_Vendor.A_Vendor_C|GetVendorCatalogue vendor)
    (Utilities|Array|Add _solditems (.VendorItem (Utilities|Struct|BreakS_VendorListing _array_element)))
    (Utilities|Array|Add _itemstock (.remainingStock (Utilities|Struct|BreakS_VendorListing _array_element)))
    (Utilities|Array|Add _prices (.priceMultiplier (Utilities|Struct|BreakS_VendorListing _array_element)))
    (Utilities|Array|Add _boughtitems (.PlayerItem (Utilities|Struct|BreakS_VendorListing _array_element))))
  (return (Utilities|Struct|MakeStuct_PlayerVendors (Transformation|GetActorTransform vendor) (Variables|/Game/Blueprints/Vendor/A_Vendor_PlayerPlaced.A_Vendor_PlayerPlaced_C|GetOwnerId vendor) (Variables|/Game/Blueprints/Vendor/A_Vendor_PlayerPlaced.A_Vendor_PlayerPlaced_C|GetstoredMoney vendor) _solditems _itemstock _prices (Variables|/Game/Blueprints/Vendor/A_Vendor.A_Vendor_C|GetVendor%20Name vendor) (Variables|/Game/Blueprints/Vendor/A_Vendor.A_Vendor_C|GetVendorDescription vendor) (Variables|/Game/Blueprints/Vendor/A_Vendor.A_Vendor_C|GetVendorWorldColor vendor) _boughtitems (Variables|/Game/Blueprints/Vendor/A_Vendor_PlayerPlaced.A_Vendor_PlayerPlaced_C|GetStoredItems vendor) (Utilities|GetClass vendor))))