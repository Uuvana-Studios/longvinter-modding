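; Radius-based zone actor, named for blocking building, that shows a recycler selling hint to players who enter it.
; BlockingRadius sizes the BlockRadius sphere and decal, and overlap toggles characters' capsules to ignore the Pawn channel while inside.
; Zones flagged HardcoreOnly scale to zero and lose collision outside hardcore mode, with server and client each checking their own hardcore state.
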(event OnComponentBeginOverlap(BlockRadius)
  (params (OverlappedComponent :type Primitive%20Component%20Object%20Reference) (OtherActor :type Actor%20Object%20Reference) (OtherComp :type Primitive%20Component%20Object%20Reference) (OtherBodyIndex :type Integer) (bFromSweep :type Boolean) (SweepResult :type Hit%20Result%20Structure%20%28by%20ref%29))
  (bind _aspc_longvinter (Utilities|Casting|CastToPC_Longvinter (Game|GetInstigatorController OtherActor)))
  (Default|ShowGameplayHint _aspc_longvinter "All the items can be sold in James recycler machines, these are found in some outposts and points of interests.")
  (bind _asthird_person_character (Utilities|Casting|CastToThirdPersonCharacter OtherActor))
  (Collision|SetCollisionResponsetoChannel (Variables|/Script/Engine.Character|GetCapsuleComponent _asthird_person_character) "ECC_Pawn" "ECR_Ignore"))

(event OnComponentEndOverlap(BlockRadius)
  (params (OverlappedComponent :type Primitive%20Component%20Object%20Reference) (OtherActor :type Actor%20Object%20Reference) (OtherComp :type Primitive%20Component%20Object%20Reference) (OtherBodyIndex :type Integer))
  (bind _asthird_person_character (Utilities|Casting|CastToThirdPersonCharacter OtherActor))
  (Collision|SetCollisionResponsetoChannel (Variables|/Script/Engine.Character|GetCapsuleComponent _asthird_person_character) "ECC_Pawn" "ECR_Block"))

(event EventBeginPlay
  (bind _blocking_radius (Variables|Default|GetBlocking%20Radius))
  (bind _returnvalue (/ _blocking_radius 6e+01))
  (Transformation|SetWorldScale3D (Variables|Default|GetDecal) (Math|Vector|MakeVector _returnvalue _returnvalue _returnvalue))
  (CallFunction|SetHardcoreVisualsandCollision))

(event Collision|EventActorBeginOverlap
  (params (OtherActor :type Actor%20Object%20Reference)))

(fn ConstructionScript
  (bind _blocking_radius (Variables|Default|GetBlocking%20Radius))
  (bind _returnvalue (/ _blocking_radius 6e+01))
  (Components|Sphere|SetSphereRadius (Variables|Default|GetBlockRadius) (/ _blocking_radius 1e+01) true)
  (Transformation|SetWorldScale3D (Variables|Default|GetDecal) (Math|Vector|MakeVector _returnvalue _returnvalue _returnvalue)))

(fn SetHardcoreVisualsandCollision
  (if (Variables|Default|GetHardcoreOnly)
    (Networking|SwitchHasAuthority
      (:Authority
        (if (not (CallFunction|GetHardcore))
          (Transformation|SetActorScale3D "0, 0, 0" :!label _label)
          (Collision|SetActorEnableCollision false)))
      (:Remote
        (bind _aspc_longvinter (Utilities|Casting|CastToPC_Longvinter (Game|GetPlayerController 0)))
        (if (not (Variables|/Game/Blueprints/PC_Longvinter.PC_Longvinter_C|GetHardcore _aspc_longvinter))
          (goto _label))))))