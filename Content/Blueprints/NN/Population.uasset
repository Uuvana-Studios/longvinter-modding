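; Population of Specie objects with neural-network brains, evolved across generations by a genetic algorithm that records average fitness.
; NextGeneration bubble-sorts species by last fitness and, with elitist selection, keeps only the top two as parents.
; Crossover refills the population, copying each neuron's bias and synapse weights from either parent at random.
; Mutation randomly replaces or steps weights and biases, sparing the two elites unless stale, then fitness resets.
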(event Custom|Populate
  (CallFunction|MakeNSpecies (Variables|Default|GetNumber%20of%20species)))

(event Custom|Next%20Generation
  (Math|Integer|IncrementInt (Variables|Default|GetGeneration)
    (:%20%20
      (Utilities|Array|Add (Variables|Default|GetFitness%20Over%20Time) (CallFunction|AverageFitness))
      (CallFunction|Selection (/ (Variables|Default|GetNumber%20of%20species) 2) true)
      (CallFunction|Crossover (- (Variables|Default|GetNumber%20of%20species) (Utilities|Array|Length (Variables|Default|GetSpecies))))
      (for (_array_element _array_index) (Variables|Default|GetSpecies)
        (if (or (Variables|/Game/Blueprints/NN/Specie.Specie_C|GetStale _array_element) (> _array_index 1))
          (CallFunction|Mutation _array_element)))
      (for _array_element_2 (Variables|Default|GetSpecies)
        (Variables|/Game/Blueprints/NN/Specie.Specie_C|SetFitness _array_element_2 0.0))
      (Default|CallPopulationChanged))))

(event Custom|Make%20n%20Species
  (params (n :type Integer))
  (for _index (range 1 n)
    (bind _returnvalue (Game|ConstructObjectfromClass "/Game/Blueprints/NN/Specie.Specie_C" self (Variables|Default|GetNeuron%20Counts)))
    (Variables|/Game/Blueprints/NN/Specie.Specie_C|SetGeneration%20Born _returnvalue (Variables|Default|GetGeneration))
    (Variables|/Game/Blueprints/NN/Specie.Specie_C|SetNumber _returnvalue _index)
    (Default|SetupSpecie _returnvalue)
    (Utilities|Array|Add (Variables|Default|GetSpecies) _returnvalue)))

(fn Selection
  (params (Kill%20count :type Integer) (Elitist%20Selection :type Boolean))
  (bind _sorted_species (LocalVariables|GetSorted%20Species))
  ;[0 0 0] Map fitness values to species
  (for _array_element (Variables|Default|GetSpecies)
    (Utilities|Map|Add (LocalVariables|GetFitness%20Map) (Variables|/Game/Blueprints/NN/Specie.Specie_C|GetLast%20Fitness _array_element) _array_element))
  (bind _keys (Utilities|Map|Keys (LocalVariables|GetFitness%20Map)))
  (bind _output_get (LocalVariables|SetFitness%20Array _keys))
  ;[1 0.8715 0] Bubble sort, needs improvement
  (for _index (range 0 (Utilities|Array|LastIndex _output_get))
    (for _index_2 (range 0 (- (Utilities|Array|LastIndex _output_get) 1))
      (if (< (Utilities|Array|Get(acopy) (LocalVariables|GetFitness%20Array) _index_2) (Utilities|Array|Get(acopy) (LocalVariables|GetFitness%20Array) (+ _index_2 1)))
        (Utilities|Array|Swap (LocalVariables|GetFitness%20Array) _index_2 (+ _index_2 1)))))
  (for _array_element_2 (LocalVariables|GetFitness%20Array)
    (if (.ReturnValue (Utilities|Map|Find (LocalVariables|GetFitness%20Map) _array_element_2))
      (bind _returnvalue (Utilities|Array|Add _sorted_species (.Value (Utilities|Map|Find (LocalVariables|GetFitness%20Map) _array_element_2))))
      (Variables|/Game/Blueprints/NN/Specie.Specie_C|SetNumber (Utilities|Array|Get(acopy) _sorted_species _returnvalue) (+ _returnvalue 1)))
    (if (< _array_element_2 0.0)
      (Math|Integer|IncrementInt (LocalVariables|GetBelow%20Zero))))
  ;[0 0 0] Copy all sorted minus n weakest
  (Utilities|Array|Clear (Variables|Default|GetSpecies))
  (for _index_3 (range 0 (Math|Integer|SelectInt 1 (- (Utilities|Array|LastIndex (LocalVariables|GetSorted%20Species)) (Math|Integer|Max(Integer) Kill%20count (LocalVariables|GetBelow%20Zero))) Elitist%20Selection))
    (Utilities|Array|Add (Variables|Default|GetSpecies) (Utilities|Array|Get(acopy) (LocalVariables|GetSorted%20Species) _index_3))))

(fn Crossover
  (params (Offspring :type Integer))
  (bind _species (Variables|Default|GetSpecies))
  (bind _species_2 (Variables|Default|GetSpecies))
  (for _index (range 1 Offspring)
    (bind _returnvalue (Game|ConstructObjectfromClass "/Game/Blueprints/NN/Specie.Specie_C" self (Variables|Default|GetNeuron%20Counts)))
    (Variables|/Game/Blueprints/NN/Specie.Specie_C|SetGeneration%20Born _returnvalue (Variables|Default|GetGeneration))
    (Default|SetupSpecie _returnvalue)
    (for (_array_element _array_index) (Variables|/Game/Blueprints/NN/Brain.Brain_C|GetNeurons (Variables|/Game/Blueprints/NN/Specie.Specie_C|GetBrain _returnvalue))
      (bind _asneuron (Utilities|Casting|CastToNeuron _array_element))
      (if (> (Math|Random|RandomFloat) 0.5)
        (Variables|/Game/Blueprints/NN/Neuron.Neuron_C|SetBias _asneuron (Variables|/Game/Blueprints/NN/Neuron.Neuron_C|GetBias (.AsNeuron (Utilities|Casting|CastToNeuron (Utilities|Array|Get(acopy) (Variables|/Game/Blueprints/NN/Brain.Brain_C|GetNeurons (Variables|/Game/Blueprints/NN/Specie.Specie_C|GetBrain (Utilities|Array|Get(acopy) _species_2))) _array_index)))))
        (for (_array_element_2 _array_index_2) (Variables|/Game/Blueprints/NN/Neuron.Neuron_C|GetSynapses _asneuron)
          (Variables|/Game/Blueprints/NN/Synapse.Synapse_C|SetWeight _array_element_2 (Variables|/Game/Blueprints/NN/Synapse.Synapse_C|GetWeight (Utilities|Array|Get(acopy) (Variables|/Game/Blueprints/NN/Neuron.Neuron_C|GetSynapses (.AsNeuron (Utilities|Casting|CastToNeuron (Utilities|Array|Get(acopy) (Variables|/Game/Blueprints/NN/Brain.Brain_C|GetNeurons (Variables|/Game/Blueprints/NN/Specie.Specie_C|GetBrain (Utilities|Array|Get(acopy) _species_2))) _array_index)))) _array_index_2))))
        (else
          (Variables|/Game/Blueprints/NN/Neuron.Neuron_C|SetBias _asneuron (Variables|/Game/Blueprints/NN/Neuron.Neuron_C|GetBias (.AsNeuron (Utilities|Casting|CastToNeuron (Utilities|Array|Get(acopy) (Variables|/Game/Blueprints/NN/Brain.Brain_C|GetNeurons (Variables|/Game/Blueprints/NN/Specie.Specie_C|GetBrain (Utilities|Array|Get(acopy) _species_2 1))) _array_index)))))
          (for (_array_element_3 _array_index_3) (Variables|/Game/Blueprints/NN/Neuron.Neuron_C|GetSynapses _asneuron)
            (Variables|/Game/Blueprints/NN/Synapse.Synapse_C|SetWeight _array_element_3 (Variables|/Game/Blueprints/NN/Synapse.Synapse_C|GetWeight (Utilities|Array|Get(acopy) (Variables|/Game/Blueprints/NN/Neuron.Neuron_C|GetSynapses (.AsNeuron (Utilities|Casting|CastToNeuron (Utilities|Array|Get(acopy) (Variables|/Game/Blueprints/NN/Brain.Brain_C|GetNeurons (Variables|/Game/Blueprints/NN/Specie.Specie_C|GetBrain (Utilities|Array|Get(acopy) _species_2 1))) _array_index)))) _array_index_3)))))))
    (bind _returnvalue_2 (Utilities|Array|Add _species _returnvalue))
    (Variables|/Game/Blueprints/NN/Specie.Specie_C|SetNumber (Utilities|Array|Get(acopy) _species _returnvalue_2) (+ _returnvalue_2 1))))

(fn Mutation
  (params (Specie :type Specie%20Object%20Reference))
  (Variables|/Game/Blueprints/NN/Specie.Specie_C|SetStale Specie false)
  (for _array_element (Variables|/Game/Blueprints/NN/Brain.Brain_C|GetNeurons (Variables|/Game/Blueprints/NN/Specie.Specie_C|GetBrain Specie))
    (bind _asneuron (Utilities|Casting|CastToNeuron _array_element))
    ;[0 0 0] Mutate all synapses
    (for _array_element_2 (Variables|/Game/Blueprints/NN/Neuron.Neuron_C|GetSynapses _asneuron)
      (if (< (Math|Random|RandomFloat) (Variables|Default|GetSynapse%20Mutation%20Chance))
        (Variables|/Game/Blueprints/NN/Synapse.Synapse_C|SetWeight _array_element_2 (Math|Float|SelectFloat (Math|Random|RandomFloatinRange -5.0 5.0) (+ (Variables|/Game/Blueprints/NN/Synapse.Synapse_C|GetWeight _array_element_2) (* (Math|Float|Sign(Float) (Math|Random|RandomFloatinRange -1.0 1.0)) (Variables|Default|GetMutation%20Step))) (< (Math|Random|RandomFloat) (Variables|Default|GetPerturb%20Chance))))))
    ;[0 0 0] Mutate all biases
    (if (< (Math|Random|RandomFloat) (Variables|Default|GetNeuron%20Mutation%20Chance))
      (Variables|/Game/Blueprints/NN/Neuron.Neuron_C|SetBias _asneuron (Math|Float|SelectFloat (Math|Random|RandomFloatinRange -5.0 5.0) (+ (Variables|/Game/Blueprints/NN/Neuron.Neuron_C|GetBias _asneuron) (* (Math|Float|Sign(Float) (Math|Random|RandomFloatinRange -1.0 1.0)) (Variables|Default|GetMutation%20Step))) (< (Math|Random|RandomFloat) (Variables|Default|GetPerturb%20Chance)))))))

(fn AverageFitness
  (bind _species (Variables|Default|GetSpecies))
  (for _array_element _species
    (LocalVariables|SetFitness%20Sum (+ (Variables|/Game/Blueprints/NN/Specie.Specie_C|GetFitness _array_element) (LocalVariables|GetFitness%20Sum))))
  (return (/ (LocalVariables|GetFitness%20Sum) (Math|Conversions|ToFloat(Integer) (Utilities|Array|Length _species)))))