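; VinterNetComponent is a player marketplace component that keeps replicated listings, mailboxes, pending payments and sale history.
; Adding a listing stores it and immediately grants the seller a fixed currency amount through their character, found by Steam ID.
; A purchase moves the matching listing into pending money and history, then puts the item in the buyer's mailbox, creating one if needed.
; The RepNotify handlers are empty, and pending money is never paid out here.
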(event Custom|vinterNetEvent
  (Development|PrintString "hello from vinter net"))

(event Custom|addNewListing
  (params (item :type Integer) (price :type Integer) (steamId :type String))
  (Utilities|Array|Add (Variables|Default|Getlistings) (Utilities|Struct|MakeitemListing_Struct steamId item price))
  (CallFunction|AddCurrencytoPlayer steamId 20))

(event Custom|buyItemFromListing
  (params (buyerId :type String) (SellerId :type String) (itemId :type Integer))
  (bind (_array_element _array_index) (Utilities|Array|ForEachLoopwithBreak (Variables|Default|Getlistings) :!label _label)
    (:LoopBody
      (if (and (Utilities|Enum|Equal(Enum) (.steamid _array_element) SellerId) (== itemId (.itemidd _array_element)))
        (Utilities|Array|Add (Variables|Default|GetpendingMoneys) (Utilities|Struct|MakependingMoney_Struct (.steamid _array_element) (.price _array_element)))
        (Utilities|Array|Add (Variables|Default|Gethistory) (Utilities|Struct|MakeitemListing_Struct (.steamid _array_element) (.itemidd _array_element) (.price _array_element)))
        (Utilities|Array|RemoveIndex (Variables|Default|Getlistings) _array_index)
        (bind (_success _mailboxindex) (CallFunction|FindUserMailBox buyerId))
        (if _success
          (Utilities|Array|Add (.items (Utilities|Array|Get(acopy) (Variables|Default|Getmails) _mailboxindex)) (.itemidd _array_element))
          (goto _label Break)
          (else
            (Utilities|Array|Add (Variables|Default|Getmails) (Utilities|Struct|MakemailBox_Struct buyerId (Utilities|Array|MakeArray (.itemidd _array_element))))
            (goto _label Break)))))))

(event EventBeginPlay)

(event EventTick
  (params (DeltaSeconds :type Float%20%28single-precision%29)))

(fn OnRepListings)

(fn OnRepMails)

(fn OnRepPendingMoneys)

(fn OnRepHistory)

(fn FindUserMailBox
  (params (buyerId :type String))
  (bind (_array_element _array_index) (Utilities|Array|ForEachLoopwithBreak (Variables|Default|Getmails))
    (:LoopBody
      (if (Utilities|Enum|Equal(Enum) (.steamid _array_element) buyerId)
        (return true _array_index)))
    (:Completed
      (return false 0))))

(fn AddCurrencytoPlayer
  (params (steamID :type String) (amount :type Integer))
  (bind _array_element (Utilities|Array|ForEachLoopwithBreak (Variables|/Script/Engine.GameStateBase|GetPlayerArray (Game|GetGameState)) :!label _label)
    (:LoopBody
      (if (Utilities|Enum|Equal(Enum) steamID (Class|AdvancedSessionsLibrary|UniqueNetIdtoString (Class|AdvancedSessionsLibrary|GetUniqueNetIDfromPlayerState _array_element)))
        (bind _asthird_person_character (Utilities|Casting|CastToThirdPersonCharacter (Variables|/Script/Engine.PlayerState|GetPawnPrivate _array_element)))
        (bind _hasauth (Default|HasNetworkAuth _asthird_person_character))
        (if _hasauth
          (Default|AddCurrencyServer _asthird_person_character amount)
          (goto _label Break))))))