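; Placeable laser turret that shoots players in its radius, optionally cycling on and off.
; The server sphere-traces overlapping players, rotates toward the first visible one and fires when aligned.
; Shots multicast a hidden server projectile and cosmetic client effects; clients also run idle sweeps, beam traces and rep-notify activation animations.
; Repeated player hits briefly disable it; zero health can explode it, granting quest progress, random drops and optional respawn.
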(event OnComponentBeginOverlap(Sphere)
  (params (OverlappedComponent :type Primitive%20Component%20Object%20Reference) (OtherActor :type Actor%20Object%20Reference) (OtherComp :type Primitive%20Component%20Object%20Reference) (OtherBodyIndex :type Integer) (bFromSweep :type Boolean) (SweepResult :type Hit%20Result%20Structure%20%28by%20ref%29))
  (Networking|SwitchHasAuthority
    (:Authority
      (Utilities|UpdatePlayerinRange))))

(event OnComponentEndOverlap(Sphere)
  (params (OverlappedComponent :type Primitive%20Component%20Object%20Reference) (OtherActor :type Actor%20Object%20Reference) (OtherComp :type Primitive%20Component%20Object%20Reference) (OtherBodyIndex :type Integer))
  (Networking|SwitchHasAuthority
    (:Authority
      (Utilities|UpdatePlayerinRange))))

(event Custom|ShootMulticast
  (params (SpawnTransform :type Transform))
  (bind _damage (Variables|Settings|GetDamage))
  (bind _weaponstats2 (Utilities|Struct|MakeweaponStats2 0 0 false "NewEnumerator0" "/Game/Audio/Gun/Shot.Shot" 0 _damage 7e+02 true 1 1 1 0.0 2e+02 1.0 1e+02 0.0 1e+01 3e+01 2e+02 0.4445 false true "NewEnumerator1" "NewEnumerator1" false "/Game/Blueprints/DamageType/DT_Melee.DT_Melee_C"))
  ;[1 1 1] 2.5. Shoot
  (Networking|SwitchHasAuthority
    (:Authority
      (Game|SpawnActorfromClass "/Game/Blueprints/Projectile/A_Projectile_Laser.A_Projectile_Laser_C" SpawnTransform "AlwaysSpawn" 0 0 self "0.000000,0.000000,0.000000" true "/Game/Blueprints/DamageType/DT_PlayerTurret.DT_PlayerTurret_C" true _weaponstats2 0)
      (Variables|Default|SetAllowShoot false)
      (Utilities|FlowControl|Delay 0.5)
      (Variables|Default|SetAllowShoot true))
    (:Remote
      (Game|SpawnActorfromClass "/Game/Blueprints/Projectile/A_MuzzleFlash_Laser.A_MuzzleFlash_Laser_C" SpawnTransform "AlwaysSpawn" self 0.04 false 0)
      (Audio|SpawnSoundatLocation "/Game/Audio/Gun/LaserShot.LaserShot" (Transformation|GetActorLocation) "0, 0, 0" 1.0 1.0 0.0 0 0)
      (Components|Animation|PlayAnimation (Variables|Default|GetSkeletalMesh) "/Game/Meshes/Mines/turret/anim/Anim_MineTurret_Shoot.Anim_MineTurret_Shoot" false)
      (Game|SpawnActorfromClass "/Game/Blueprints/Projectile/A_Projectile_Laser.A_Projectile_Laser_C" SpawnTransform "AlwaysSpawn" 0 0 self "0.000000,0.000000,0.000000" true "/Game/Blueprints/DamageType/DT_PlayerTurret.DT_PlayerTurret_C" false _weaponstats2 0))))

(event Custom|RespawnTurret
  (Utilities|FlowControl|Delay 3e+02)
  (Variables|Default|SetDestroyed false)
  (Variables|Default|SetDisabled false)
  (CallFunction|ActivateTurret)
  (Variables|Default|SetHealth 5e+01)
  ;[1 1 1] Damage
  (Utilities|FlowControl|DoOnce false) ; enters at Reset
)

(event Custom|SetRotation
  (Utilities|IsValid (Variables|Default|GetCurrentPlayer)
    (:Is%20Valid
      (Variables|Default|SetTargetRotation (- (.yaw (Math|Rotator|FindLookatRotation (Transformation|GetWorldLocation (Variables|Default|GetSkeletalMesh)) (Transformation|GetActorLocation (Variables|Default|GetCurrentPlayer)))) 9e+01)))))

(event Custom|TurretBeep
  (params (PlayerInSight :type Boolean))
  (bind _returnvalue (Transformation|GetActorLocation))
  (if PlayerInSight
    (Audio|PlaySoundatLocation "/Game/Audio/Turret/WAV_TurretBeep.WAV_TurretBeep" _returnvalue "0, 0, 0" 1.0 0.9 0.0 "/Game/Audio/BasicAttennuation.BasicAttennuation" 0 0)
    (else
      (Audio|PlaySoundatLocation "/Game/Audio/Turret/WAV_TurretBeep.WAV_TurretBeep" _returnvalue "0, 0, 0" 1.0 0.7 0.0 "/Game/Audio/BasicAttennuation.BasicAttennuation" 0 0))))

(event Custom|CycleState
  (if (Variables|Default|GetDestroyed) :!label _label
    (Utilities|FlowControl|Delay 0.2 :!label _label_2)
    (goto _label)
    (elif (Variables|Default|GetDisabled)
      (goto _label_2)
      (else
        (if (Variables|Default|GetTurretState)
          (CallFunction|DeactivateTurret)
          (Utilities|FlowControl|Delay (Variables|Cycle|GetCycleOffDelay))
          (else
            (CallFunction|ActivateTurret)
            (Utilities|FlowControl|Delay (+ (Variables|Cycle|GetCycleOnDelay) 1.0) :!label _label_3)
            (Utilities|IsValid (Variables|Default|GetCurrentPlayer)
              (:Is%20Valid
                (goto _label_3))
              (:Is%20Not%20Valid
                _))))
        (CallFunction|CycleState)))))

(event Custom|SetLaserState
  (params (Condition :type Boolean))
  (bind _p_laser (Variables|Default|GetP_Laser))
  (if Condition
    (Utilities|FlowControl|Delay 1.0)
    (if (Variables|Default|GetTurretState)
      (Components|Activation|Activate _p_laser false)
      (else
        (Components|Activation|Deactivate _p_laser :!label _label)))
    (else
      (goto _label))))

(event Custom|Shoot
  ;[1 1 1] 2.5. Shoot
  (CallFunction|ShootMulticast (Transformation|GetWorldTransform (Variables|Default|GetMuzzleSpawn))))

(event Custom|ActivateTurret
  ;[1 1 1] Activate/Deactivate
  (if (not (Variables|Default|GetDestroyed))
    (Variables|Default|SetTurretState true)
    (Networking|ForceNetUpdate)
    (Utilities|FlowControl|Delay 1.0)
    (Variables|Default|SetFullyActive true)
    (Networking|ForceNetUpdate)))

(event Custom|DeactivateTurret
  ;[1 1 1] Activate/Deactivate
  (if (not (Variables|Default|GetDestroyed))
    (Variables|Default|SetTurretState false)
    (Variables|Default|SetFullyActive false)
    (Networking|ForceNetUpdate)))

(event Custom|Explode
  (bind _returnvalue (Transformation|GetActorTransform))
  (bind _returnvalue_2 (Transformation|GetActorLocation))
  (bind _returnvalue_3 (+ (.location _returnvalue) "0, 0,50.000000"))
  (bind _returnvalue_4 (Math|Transform|MakeTransform _returnvalue_3 "0, 0, 0" (.scale _returnvalue)))
  ;[1 1 1] Explode
  (Variables|Default|SetTurretState false)
  (Variables|Default|SetFullyActive false)
  (Networking|SwitchHasAuthority
    (:Authority
      (CallFunction|DropItems)
      (Utilities|FlowControl|Delay 6e+01)
      (Game|SpawnActorfromClass "/Game/Particles/A_Impact_NoGravity.A_Impact_NoGravity_C" _returnvalue_4 "Undefined" 0 0)
      (Game|SpawnActorfromClass "/Game/Particles/A_Impact_NoGravity.A_Impact_NoGravity_C" _returnvalue_4 "Undefined" 0 0)
      (if (Variables|Settings|GetRespawn)
        (CallFunction|RespawnTurret)
        (else
          (Actor|DestroyActor))))
    (:Remote
      (Components|Animation|PlayAnimation (Variables|Default|GetSkeletalMesh) (Utilities|Select :Index (Math|Random|RandomInteger 2) :Option%200 "/Game/Meshes/Mines/turret/anim/Anim_MineTurret_Death01.Anim_MineTurret_Death01" :Option%201 "/Game/Meshes/Mines/turret/anim/Anim_MineTurret_Death02.Anim_MineTurret_Death02" :Option%202 "/Game/Meshes/Mines/turret/anim/Anim_MineTurret_Death03.Anim_MineTurret_Death03") false)
      (Utilities|FlowControl|Delay 0.8)
      (Effects|SpawnEmitteratLocation "/Game/Particles/Explosions/P_Explosion_Electric.P_Explosion_Electric" _returnvalue_2)
      (Audio|SpawnSoundatLocation "/Game/Audio/Explosion/WAV_GrenadeExplosion_01.WAV_GrenadeExplosion_01" _returnvalue_2 "0, 0, 0" 1.0 1.0 0.0 "/Game/Audio/BasicAttennuation.BasicAttennuation" 0))))

(event Custom|DropItems
  (bind _returnvalue (Transformation|GetActorTransform))
  (bind (_location _rotation _scale) (Math|Transform|BreakTransform _returnvalue))
  (bind (_x _y _z) (Math|Vector|BreakVector _location))
  ;[1 1 1] DropItems
  (if (< _z 3e+03)
    _
    (else
      _))
  (Variables|Default|SetspawnHeigth _z)
  (Utilities|FlowControl|DoOnce false
    (:Completed
      (if (== (Math|Random|RandomIntegerinRange 1 5) 1)
        (bind _itemdata (CallFunction|GetItemwithID 51))
        (Game|SpawnActorfromClass "/Game/Blueprints/A_Item.A_Item_C" (Math|Transform|MakeTransform (Math|Vector|MakeVector _x _y (Variables|Default|GetspawnHeigth)) _rotation _scale) "AdjustIfPossibleButAlwaysSpawn" 0 _itemdata false false 1.0 false 0 "/Game/Audio/Pickup.Pickup" false 25 false false false 140 false 0 0 0))
      (if (== (Math|Random|RandomIntegerinRange 1 8) 1)
        (bind _itemdata_2 (CallFunction|GetItemwithID 269))
        (Game|SpawnActorfromClass "/Game/Blueprints/A_Item.A_Item_C" (Math|Transform|MakeTransform (Math|Vector|MakeVector _x _y (Variables|Default|GetspawnHeigth)) _rotation _scale) "AdjustIfPossibleButAlwaysSpawn" 0 _itemdata_2 false false 1.0 false 0 "/Game/Audio/Pickup.Pickup" false 25 false false false 140 false 0 0 0)))))

(event Game|Damage|EventAnyDamage
  (params (Damage :type Float%20%28single-precision%29) (DamageType :type Damage%20Type%20Object%20Reference) (InstigatedBy :type Controller%20Object%20Reference) (DamageCauser :type Actor%20Object%20Reference))
  (bind _timesshotat (Variables|Default|GetTimesShotAt))
  ;[1 1 1] Damage
  (if (Variables|Default|GetTurretState)
    (bind _ascontroller (Utilities|Casting|CastToController DamageCauser))
    (bind _asthird_person_character (Utilities|Casting|CastToThirdPersonCharacter (Pawn|GetControlledPawn _ascontroller)))
    (bind _output_get (Variables|Default|SetHealth (- (Variables|Default|GetHealth) Damage)))
    (if (<= _output_get 0.0)
      (if (Variables|Default|GetCantBeDestroyed)
        (if (>= _timesshotat 2) :!label _label
          (CallFunction|DeactivateTurret)
          (Variables|Default|SetDisabled true)
          (Utilities|FlowControl|Sequence
            (:then_0
              (Networking|ForceNetUpdate :!label _label_2)
              (if (Variables|Default|GetEnableDamageFlash)
                (CallFunction|DamageFlashEffect (Variables|Default|GetSkeletalMesh))))
            (:then_1
              (Utilities|FlowControl|Delay 3.0)
              (CallFunction|ActivateTurret)
              (Variables|Default|SetDisabled false)))
          (else
            (Math|Integer|IncrementInt _timesshotat
              (:%20%20
                (goto _label_2)))))
        (else
          (Utilities|FlowControl|DoOnce false
            (:Completed
              (if (Variables|Default|GetDestroyAtZeroHealth)
                (Variables|Default|SetDestroyed true)
                (Networking|ForceNetUpdate)
                (CallFunction|Explode)
                (Default|AddTaskProgression (Variables|/Game/ThirdPersonCPP/Blueprints/ThirdPersonCharacter.ThirdPersonCharacter_C|GetQuestComponent _asthird_person_character) "NewEnumerator70"))))))
      (else
        (goto _label)))))

(event EventDropItemonDestruction)

(event EventStartDecay)

(event EventDestroyed)

(event EventTick
  (params (DeltaSeconds :type Float%20%28single-precision%29))
  (if (not (Variables|Default|GetDestroyed))
    (Networking|SwitchHasAuthority
      (:Authority
        (if (Math|Boolean|ANDBoolean (Variables|Default|GetTurretState) (Variables|Default|GetPlayerInRange) (Variables|Default|GetFullyActive))
          (Utilities|FlowControl|Sequence
            (:then_0
              (Utilities|CheckLineOfSight
                (:Completed
                  (Utilities|BeepRotateShoot :!label _label))))
            (:then_1
              (Utilities|IsValid (Variables|Default|GetCurrentPlayer)
                (:Is%20Valid
                  (Utilities|SmoothRotatetoTarget DeltaSeconds 2e+01 :!label _label_2)))))
          (else
            (goto _label PlayerNotInRange))))
      (:Remote
        (Utilities|SetLaserEnd)
        (Utilities|IsValid (Variables|Default|GetCurrentPlayer)
          (:Is%20Valid
            (goto _label_2))
          (:Is%20Not%20Valid
            (CallFunction|IdleAnimation DeltaSeconds)))))))

(event EventBeginPlay
  (Networking|SwitchHasAuthority
    (:Authority
      (Variables|Default|SetTargetRotation (.yaw (Transformation|GetWorldRotation (Variables|Default|GetSM_Placeable))))
      (if (Variables|Cycle|GetCycle)
        (Utilities|FlowControl|Delay (Variables|Cycle|GetCycleStartDelay))
        (CallFunction|CycleState)))))

(fn ConstructionScript
  (|CallParentFunction)
  (Components|Sphere|SetSphereRadius (Variables|Default|GetSphere) (Variables|Settings|GetRadius) true)
  (Variables|Settings|SetoriginalDamage (Variables|Settings|GetDamage))
  (Utilities|SetLaserEnd))

(fn OnRepPlacedbyPlayer
  (if true
    (Rendering|Material|SetMaterial (Variables|Default|GetSM_Placeable) 1 "/Game/Meshes/Container/Materials/Common/M_Container.M_Container")))

(fn OnRepTurretState
  (if (Variables|Default|GetTurretState)
    (Components|Animation|PlayAnimation (Variables|Default|GetSkeletalMesh) "/Game/Meshes/Mines/turret/anim/Anim_MineTurret_Activate.Anim_MineTurret_Activate" false)
    (CallFunction|SetLaserState true)
    (else
      (Variables|Default|SetTimesShotAt 0)
      (Components|Animation|PlayAnimation (Variables|Default|GetSkeletalMesh) "/Game/Meshes/Mines/turret/anim/Anim_MineTurret_Deactivate.Anim_MineTurret_Deactivate" false)
      (CallFunction|SetLaserState false))))

(fn IdleAnimation
  (params (DeltaTime :type Float%20%28single-precision%29))
  (bind _sm_placeable (Variables|Default|GetSM_Placeable))
  (bind _returnvalue (Transformation|GetWorldRotation _sm_placeable))
  (if (Variables|Default|GetFullyActive)
    (Utilities|IsValid (Variables|Default|GetCurrentPlayer)
      (:Is%20Not%20Valid
        (if (Variables|Default|GetLeftRight)
          (Variables|Default|SetTargetRotation (+ (.yaw _returnvalue) 3e+01))
          (else
            (Variables|Default|SetTargetRotation (- (.yaw _returnvalue) 3e+01))))
        (Utilities|SmoothRotatetoTarget DeltaTime 1.0)
        (if (<= (Math|Float|Absolute(Float) (.yaw (Math|Rotator|Delta(Rotator) (Math|Rotator|MakeRotator 0.0 0.0 (.yaw (Transformation|GetWorldRotation (Variables|Default|GetSkeletalMesh)))) (Math|Rotator|MakeRotator 0.0 0.0 (Variables|Default|GetTargetRotation))))) 1e+01)
          (Variables|Default|SetLeftRight (not (Variables|Default|GetLeftRight))))))))

(fn OnRepDontDestroy)