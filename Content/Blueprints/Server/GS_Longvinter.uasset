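; Longvinter game state that spawns world nodes and chooses players' outpost spawn points.
; On BeginPlay it caches starter travel points and starts a looping timer that replaces A_NodeSpawn markers with A_Node actors.
; GetWorldSpawnPoint picks an outpost from the co-op spawn setting, or otherwise from one SteamID digit to spread players out.
; SpawnWorldLoot turns loot markers into unsaved chests via the UGC override registry, but its timer is disconnected.
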(event EventBeginPlay
  (Utilities|FlowControl|Sequence
    (:then_0
      ;[1 1 1] SpawnNodes
      (Utilities|Time|SetTimerbyFunctionName 0 "SpawnNodes" 1e+01 true))
    (:then_1
      ;[1 1 1] Get spawnpoints
      (bind _outactors (Actor|GetAllActorsOfClass "/Game/Blueprints/BoatTravel/A_TravelPoint.A_TravelPoint_C"))
      (for _array_element _outactors
        (if (Math|Integer|InRange(Integer) (Variables|/Game/Blueprints/BoatTravel/A_TravelPoint.A_TravelPoint_C|GetStarterPointInteger _array_element) 0 9)
          (Utilities|Array|Add (Variables|Default|GetSpawnPoints) _array_element))))
    (:then_3
      (bind _asgi_advanced_sessions (Utilities|Casting|CastToGI_AdvancedSessions (Game|GetGameInstance)))
      (Variables|Default|SetAs%20GI%20Advanced%20Sessions _asgi_advanced_sessions))))

(fn ConstructionScript)

(fn SpawnNodes
  (bind _outactors (Actor|GetAllActorsOfClass "/Game/Blueprints/A_NodeSpawn.A_NodeSpawn_C"))
  (for _array_element _outactors
    (Game|SpawnActorfromClass "/Game/Blueprints/A_Node.A_Node_C" (Math|Conversions|ToTransform(Vector) (Transformation|GetWorldLocation (Variables|/Game/Blueprints/A_NodeSpawn.A_NodeSpawn_C|GetDefaultSceneRoot _array_element))) "Undefined" 0 (Variables|/Game/Blueprints/A_NodeSpawn.A_NodeSpawn_C|GetIndex _array_element) 0)
    (Development|PrintString (Utilities|String|Append "GS: " (Utilities|String|ToString(Integer) 0)) true true "(R=1.000000,G=0.062529,B=0.000000,A=1.000000)" 2e+01)
    (Actor|DestroyActor _array_element)))

(fn GetWorldSpawnPoint
  (params (SteamID :type String))
  (bind _asgm_longvinter (Utilities|Casting|CastToGM_Longvinter (Game|GetGameMode)))
  (if (Variables|/Game/Blueprints/Server/GM_Longvinter.GM_Longvinter_C|GetCoopPlay _asgm_longvinter)
    (switch int (Variables|/Game/Blueprints/Server/GM_Longvinter.GM_Longvinter_C|GetCoopSpawn _asgm_longvinter)
      (:Default
        (LocalVariables|SetOutpostInteger 1 :!label _label))
      (:0
        (LocalVariables|SetOutpostInteger 3))
      (:1
        (goto _label))
      (:2
        (LocalVariables|SetOutpostInteger 4)))
    (else
      (switch int (Math|Conversions|ToInteger(Byte) (Utilities|String|GetSubstring SteamID 14))
        (:Default
          (LocalVariables|SetOutpostInteger 1 :!label _label_2))
        (:0
          (goto _label_2))
        (:1
          (goto _label_2))
        (:2
          (LocalVariables|SetOutpostInteger 4 :!label _label_3))
        (:3
          (LocalVariables|SetOutpostInteger 3 :!label _label_4))
        (:4
          (LocalVariables|SetOutpostInteger 2 :!label _label_5))
        (:5
          (goto _label_5))
        (:6
          (goto _label_4))
        (:7
          (LocalVariables|SetOutpostInteger 5 :!label _label_6))
        (:8
          (goto _label_3))
        (:9
          (goto _label_6)))))
  (for _array_element (Variables|Default|GetSpawnPoints)
    (if (== (LocalVariables|GetOutpostInteger) (Variables|/Game/Blueprints/BoatTravel/A_TravelPoint.A_TravelPoint_C|GetStarterPointInteger _array_element))
      (bind _output_get (LocalVariables|SetSpawnLoc (Transformation|GetActorTransform _array_element)))
      (return _output_get))))

(fn SpawnWorldLoot
  (bind _outactors (Actor|GetAllActorsOfClass "/Game/Blueprints/A_Chest/A_LootSpawn.A_LootSpawn_C"))
  (for _array_element _outactors
    (bind _asa_chest (Utilities|Casting|CastToA_ChestClass (Class|UGCRegistry|GetOverrideforActorClass (Class|UGCBlueprintLibrary|GetUGCRegistry) "/Game/Blueprints/A_Chest/A_Chest.A_Chest_C")))
    (Game|SpawnActorfromClass _asa_chest (Transformation|GetActorTransform _array_element) "AlwaysSpawn" 0 true 0 10 "Container" false "" 1 false 0 (Variables|/Game/Blueprints/A_Chest/A_LootSpawn.A_LootSpawn_C|GetcommonLootTable _array_element) (Variables|/Game/Blueprints/A_Chest/A_LootSpawn.A_LootSpawn_C|GetCommonRareRarityChance _array_element) 1 (Variables|/Game/Blueprints/A_Chest/A_LootSpawn.A_LootSpawn_C|GetLootCategory _array_element) (Variables|/Game/Blueprints/A_Chest/A_LootSpawn.A_LootSpawn_C|GetrareLootTable _array_element) (Variables|/Game/Blueprints/A_Chest/A_LootSpawn.A_LootSpawn_C|GetExtraLootChance _array_element) 0 "" 6 6e+02 "" true true false 0)
    (Actor|DestroyActor _array_element)))