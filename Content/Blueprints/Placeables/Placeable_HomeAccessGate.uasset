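; Placeable gate that restricts who can open it based on a nearby player home.
; CheckPlayerAccess takes the first A_Home overlapping CollisionCheck and, if its Tier is above zero, opens only for players whose Steam ID is in that home's saved list.
; With no home nearby or a tier-zero home, it opens for anyone and sends an explanatory message; locked-out players are told to enter the house to unlock.
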(event EventBeginPlay
  (|CallParentFunction) ; This node is disabled and will not be called.\nDrag off pins to build functionality.
)

(event Collision|EventActorBeginOverlap
  (params (OtherActor :type Actor%20Object%20Reference))
  (|CallParentFunction OtherActor) ; This node is disabled and will not be called.\nDrag off pins to build functionality.
)

(event EventTick
  (params (DeltaSeconds :type Float%20%28single-precision%29))
  (|CallParentFunction DeltaSeconds) ; This node is disabled and will not be called.\nDrag off pins to build functionality.
)

(event EventCheckPlayerAccess
  (params (Player :type Third%20Person%20Character%20Object%20Reference))
  (bind _collisioncheck (Variables|Default|GetCollisionCheck))
  (bind _overlappingactors (Collision|GetOverlappingActors _collisioncheck "/Game/Blueprints/A_Home.A_Home_C" :!class /Script/Engine.PrimitiveComponent))
  (if (Utilities|Array|IsValidIndex _overlappingactors)
    (bind _asa_home (Utilities|Casting|CastToA_Home (Utilities|Array|Get(acopy) _overlappingactors)))
    (if (> (Variables|/Game/Blueprints/A_Home.A_Home_C|GetTier _asa_home) 0)
      (if (Utilities|Array|ContainsItem (Variables|/Game/Blueprints/A_Home.A_Home_C|GetsavedSteamID's _asa_home) (Class|AdvancedSessionsLibrary|UniqueNetIdtoString (Class|AdvancedSessionsLibrary|GetUniqueNetIDfromPlayerState (Variables|/Script/Engine.Pawn|GetPlayerState Player))))
        (CallFunction|OpenGate :!label _label)
        (else
          (Default|RunonClientErrorMessage Player "This gate is locked, enter the house to unlock")))
      (else
        (Default|RunonClientErrorMessage Player "Shared gate is only locked when you upgrade your tent to a house with workbench")
        (goto _label)))
    (else
      (Default|RunonClientErrorMessage Player "This gate can be accessed by anyone, no house near it")
      (goto _label))))

(fn ConstructionScript
  (|CallParentFunction))