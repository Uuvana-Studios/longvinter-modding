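; Async task that saves the world's placeable actors to the AllPlaceables save slot.
; Execute filters Placeables by their SavePlaceable flag and by a transform check meant to skip duplicates.
; It gathers transform, class, comment, placer Steam ID and item data into parallel arrays.
; These are copied into the SaveGame object and written once, with debug prints reporting progress and count.
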(event EventExecute
  (bind _placeableclass (Variables|Default|GetPlaceableClass))
  (bind _savegame (Variables|Default|GetSaveGame))
  (for _array_element (Variables|Default|GetPlaceables)
    (Utilities|ShouldSavePlaceable _array_element
      (:true
        (Utilities|Array|Add (Variables|Default|GetPlaceableDuplicationCheckTransforms) (Transformation|GetActorTransform _array_element))
        (Utilities|Array|Add (Variables|Default|GetPlaceableTransforms) (Transformation|GetActorTransform _array_element))
        (Utilities|Array|Add (Variables|Default|GetPlaceableClass) (Utilities|GetClass _array_element))
        (Utilities|Array|Add (Variables|Default|GetPlaceableComments) (Variables|/Game/Blueprints/Placeables/A_Placeable.A_Placeable_C|GetComment _array_element))
        (Utilities|Array|Add (Variables|Default|GetPlaceableIDs) (Variables|/Game/Blueprints/Placeables/A_Placeable.A_Placeable_C|GetPlacerSteamID _array_element))
        (Utilities|Array|Add (Variables|Default|GetPlaceableItemDatas) (Variables|/Game/Blueprints/Placeables/A_Placeable.A_Placeable_C|GetItemData _array_element)))))
  (Variables|/Game/Blueprints/Placeables/SG_Placeable.SG_Placeable_C|SetClasses _savegame _placeableclass)
  (Variables|/Game/Blueprints/Placeables/SG_Placeable.SG_Placeable_C|SetComments _savegame (Variables|Default|GetPlaceableComments))
  (Variables|/Game/Blueprints/Placeables/SG_Placeable.SG_Placeable_C|SetIDs _savegame (Variables|Default|GetPlaceableIDs))
  (Variables|/Game/Blueprints/Placeables/SG_Placeable.SG_Placeable_C|SetTransforms _savegame (Variables|Default|GetPlaceableTransforms))
  (Variables|/Game/Blueprints/Placeables/SG_Placeable.SG_Placeable_C|SetItemDatas _savegame (Variables|Default|GetPlaceableItemDatas))
  (Development|PrintString 0 "Start Writing")
  (SaveGame|SaveGametoSlot _savegame "AllPlaceables")
  (Development|PrintString 0 "Finish Writing")
  (Development|PrintString 0 (Utilities|String|Append "DONE SAVING " (Utilities|String|ToString(Integer) (Utilities|Array|Length _placeableclass)) " PLACEABLES")))