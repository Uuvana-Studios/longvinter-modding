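; Main menu player controller that handles joining a multiplayer server from a session search result.
; JoinServer routes through a queue screen when fewer than six slots remain, then an optional password prompt, then Workshop mod installation.
; It then saves server history and last server, joins the session and travels by console "open", using localhost when IPs match.
; If travel stalls, a delayed fallback destroys the session and retries before showing an error.
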(event Custom|CloseRequested)

(event Custom|loadGlobalBans)

(event Custom|vintercoinCallback
  (params (Request :type Va%20Rest%20Request%20JSON%20Object%20Reference)))

(event Custom|OpenAdvancedSettings)

(event Custom|loadBanCallback
  (params (Request :type Va%20Rest%20Request%20JSON%20Object%20Reference)))

(event Custom|ipCallback
  (params (Request :type Va%20Rest%20Request%20JSON%20Object%20Reference)))

(event Custom|CheckVinterCoin)

(event EventBeginPlay
  (Utilities|FlowControl|Sequence))

(event Custom|UpdateInstalledMods)

(event Custom|CheckModsCopied
  (params (HostServer :type Boolean)))

(event Custom|InstallMissingMods)

(event Custom|ExitGameMods)

(event Custom|DownloadWorkshopItem
  (params (FileID :type String) (Title :type String)))

(event Custom|GetServerMods
  (params (SearchResult :type Online%20Session%20Search%20Result%20BP%20Structure%20%28by%20ref%29)))

(event Custom|GetModTitles)

(event Custom|ContinueAfterCheckMods)

(event Custom|DownloadAndRestart)

(event Custom|SaveServerName
  (bind _servername (Variables|ServerJoining|GetServerName))
  (bind _savegame (|AsyncLoadGamefromSlot "ServerHistory")
    (:Completed
      (bind _assg_server_history (Utilities|Casting|CastToSG_ServerHistory _savegame)
        (:then
          (Utilities|Array|Add (Variables|/Game/Widgets/MainMenu/ServerBrowser/SG_ServerHistory.SG_ServerHistory_C|GetServerNames _assg_server_history) _servername)
          (|AsyncSaveGametoSlot _assg_server_history "ServerHistory"))
        (:CastFailed
          (bind _returnvalue (SaveGame|CreateSaveGameObject "/Game/Widgets/MainMenu/ServerBrowser/SG_ServerHistory.SG_ServerHistory_C"))
          (Utilities|Array|Add (Variables|/Game/Widgets/MainMenu/ServerBrowser/SG_ServerHistory.SG_ServerHistory_C|GetServerNames _returnvalue) _servername)
          (|AsyncSaveGametoSlot _returnvalue "ServerHistory"))))))

(event Custom|JoinServer
  (params (SearchResult :type Online%20Session%20Search%20Result%20BP%20Structure))
  (bind _session (Utilities|Struct|BreakOnlineSessionSearchResultBP SearchResult))
  (bind _sessionsettings (Utilities|Struct|BreakOnlineSessionBP _session))
  (bind (_numpublicconnections _settings) (Utilities|Struct|BreakOnlineSessionSettingsBP _sessionsettings))
  (Variables|ServerJoining|SetSearch%20Result SearchResult)
  (Variables|ServerJoining|SetServerName (Utilities|GetStringfromServerSettings (.Value (Utilities|Map|Find _settings "ServerName"))))
  (Variables|ServerJoining|SetCurrentPlayers (Math|Conversions|ToInteger(Byte) (Utilities|GetStringfromServerSettings (.Value (Utilities|Map|Find _settings "TOTPLAYING")))))
  (Variables|ServerJoining|SetMaxPlayers _numpublicconnections)
  (CallFunction|GetIpandPort)
  (if (< (- (Variables|ServerJoining|GetMaxPlayers) (Variables|ServerJoining|GetCurrentPlayers)) 6)
    (bind _returnvalue (UserInterface|CreateWidget "/Game/Widgets/MainMenu/UMG_QueueScreen.UMG_QueueScreen_C" 0 (Variables|ServerJoining|GetServerName) (.ReturnValue (Utilities|GetBoolValuefromSettings (Utilities|Name|MakeLiteralName "IsExperimental") (Variables|ServerJoining|GetSearch%20Result)))))
    (EventDispatchers|BindEventtoJoinfromQueue _returnvalue (delegate Custom|JoinFromQueue))
    (UserInterface|Viewport|AddtoViewport _returnvalue 0)
    (elif (.ReturnValue (Utilities|GetBoolValuefromSettings (Utilities|Name|MakeLiteralName "HasPassword") (Variables|ServerJoining|GetSearch%20Result)))
      (bind _returnvalue_2 (UserInterface|CreateWidget "/Game/Widgets/MainMenu/UMG_Password.UMG_Password_C" 0 0 0))
      (UserInterface|Viewport|AddtoViewport _returnvalue_2 0)
      (else
        (Variables|ServerJoining|SetPassword (stale Custom|ContinueAfterPassword Password))
        (Audio|PlaySound2D "/Game/Audio/WAV_ItemClick.WAV_ItemClick" 1.0 1.0 0.0 0 0)
        (CallFunction|InstallMissingMods)))))

(event Custom|JoinFromQueue
  (Audio|PlaySound2D "/Game/Audio/Wav_Dice_Win.Wav_Dice_Win" 1.0 1.0 0.0 0 0)
  (if (.ReturnValue (Utilities|GetBoolValuefromSettings (Utilities|Name|MakeLiteralName "HasPassword") (Variables|ServerJoining|GetSearch%20Result)))
    (bind _returnvalue (UserInterface|CreateWidget "/Game/Widgets/MainMenu/UMG_Password.UMG_Password_C" 0 0 0))
    (UserInterface|Viewport|AddtoViewport _returnvalue 0)
    (else
      (Variables|ServerJoining|SetPassword (stale Custom|ContinueAfterPassword Password))
      (Audio|PlaySound2D "/Game/Audio/WAV_ItemClick.WAV_ItemClick" 1.0 1.0 0.0 0 0)
      (CallFunction|InstallMissingMods))))

(event Custom|SaveLastServer
  (bind _returnvalue (SaveGame|CreateSaveGameObject "/Game/Widgets/MainMenu/ServerBrowser/SG_LastServer.SG_LastServer_C"))
  (Variables|/Game/Widgets/MainMenu/ServerBrowser/SG_LastServer.SG_LastServer_C|SetserverName _returnvalue (Utilities|Text|ToText(String) (Variables|ServerJoining|GetServerName)))
  (Variables|/Game/Widgets/MainMenu/ServerBrowser/SG_LastServer.SG_LastServer_C|Setpassword _returnvalue (Variables|ServerJoining|GetPassword))
  (Variables|/Game/Widgets/MainMenu/ServerBrowser/SG_LastServer.SG_LastServer_C|SetserverAddress _returnvalue (Utilities|String|Append (Variables|ServerJoining|GetServerIp) ":" (Variables|ServerJoining|GetServerport)))
  (|AsyncSaveGametoSlot _returnvalue "lastServer"))

(event Custom|JoinSession
  (bind _returnvalue (Subsystems|GetOnlineSessionSubsystem))
  (bind _self self)
  (bind _servername (Variables|ServerJoining|GetServerName))
  (bind _returnvalue_2 (Utilities|String|StringToName _servername))
  (|MakeLoadingScreen (Utilities|Text|ToText(String) _servername))
  (Variables|ServerJoining|SetConnectAttemps 3)
  (bind (_sessionname _result) (|JoinSession _returnvalue (Class|OnlineIdentitySubsystem|GetUniquePlayerId (Subsystems|GetOnlineIdentitySubsystem)) _returnvalue_2 (Variables|ServerJoining|GetSearch%20Result) :!label _label)
    (:OnCallFailed
      (|DestroySession
        (:OnSuccess
          _)
        (:OnFailure
          _))
      (|DestroySession _returnvalue _sessionname :!label _label_2
        (:OnCallFailed
          _)
        (:OnDestroySessionComplete
          _)))
    (:OnJoinSessionComplete
      (if (Utilities|Name|Equal(Name) _returnvalue_2 _sessionname)
        (switch Utilities|FlowControl|Switch|SwitchonEOnJoinSessionCompleteResult_ _result
          (:Success
            (Development|PrintString "JOINING SUCCEEDED")
            (Utilities|LocalorPublicServer
              (:local
                (Development|ExecuteConsoleCommand (Utilities|String|Append "open " "127.0.0.1:" (Variables|ServerJoining|GetServerport)) _self))
              (:public
                (Development|ExecuteConsoleCommand (Utilities|String|Append "open " (Utilities|String|Append (Variables|ServerJoining|GetServerIp) ":" (Variables|ServerJoining|GetServerport))) _self)))
            (Utilities|FlowControl|Delay 15.0)
            (Audio|PlaySound2D "/Game/Audio/Wav_Dice_Win.Wav_Dice_Win" 1.0 1.0 0.0 0 0)
            (|DestroySession _returnvalue _sessionname
              (:OnCallFailed
                _)
              (:OnDestroySessionComplete
                _))
            (if (<= (Variables|ServerJoining|GetConnectAttemps) 0)
              _
              (else
                (Math|Integer|DecrementInt (Variables|ServerJoining|GetConnectAttemps)
                  (:%20%20
                    (goto _label))))))
          (:SessionIsFull
            (Development|PrintString (Utilities|String|EnumtoString _result) :!label _label_3)
            (goto _label_2))
          (:SessionDoesNotExist
            (goto _label_3))
          (:CouldNotRetrieveAddress
            (goto _label_3))
          (:AlreadyInSession
            (goto _label_2))
          (:UnknownError
            (goto _label_2)))
        (else
          (goto _label_2)))))
  (Utilities|FlowControl|Delay 1.0)
  (Widget|RemovefromParent (Variables|ServerJoining|GetLoadingScreen))
  (bind _returnvalue_3 (UserInterface|CreateWidget "/Game/Widgets/MainMenu/UMG_NetworkErrorMessage.UMG_NetworkErrorMessage_C" (Game|GetPlayerController 0) "Connection Failed" "Unknown Reason.  
 
If this continues, please restart the game. "))
  (UserInterface|Viewport|AddtoViewport _returnvalue_3 0))

(event Custom|ContinueAfterPassword
  (params (Password :type String))
  (Variables|ServerJoining|SetPassword Password)
  (Audio|PlaySound2D "/Game/Audio/WAV_ItemClick.WAV_ItemClick" 1.0 1.0 0.0 0 0)
  (CallFunction|InstallMissingMods))

(event Custom|ContinueAfterInstallMods
  (CallFunction|SaveServerName)
  (CallFunction|SaveLastServer)
  (CallFunction|JoinSession))

(fn ConstructionScript)

(fn ErrorMessage
  (params (Message :type Text) (Title :type Text) (NotificationType :type Enum_NotificationType%20Enum :default "NewEnumerator0") (NotificationImage :type Texture%202D%20Object%20Reference) (ClearBeforeAdding :type Boolean)))

(fn GetFileIDs
  (params (ServerMods :type Array%20of%20Strings)))

(fn GetIpandPort)

(fn FindVintercoinItem
  (params (Array :type Array%20of%20Steam%20Item%20Details%20Structures)))