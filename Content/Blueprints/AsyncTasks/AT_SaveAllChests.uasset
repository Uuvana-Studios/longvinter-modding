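; Async task that saves the world's chests to the AllChests save slot.
; Execute filters the Chests array, skipping any flagged DontSave or sharing a transform with one already kept; the duplicate check starts only once two transforms are recorded.
; Each kept chest becomes a struct of class, transform, name, inventory and placeable params, and the array is written to SaveGame with debug prints around the write.
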(event EventExecute
  (bind _savegame (Variables|Default|GetSaveGame))
  (bind _chestsforsave (Variables|Default|GetChestsForSave))
  (Utilities|Array|Clear (Variables|Default|GetChestsForSave))
  (Utilities|Array|Clear (Variables|Default|GetPlaceableDuplicationCheckTransforms))
  (for _array_element (Variables|Default|GetChests)
    (Utilities|ShouldSaveChest _array_element
      (:true
        (Utilities|Array|Add (Variables|Default|GetPlaceableDuplicationCheckTransforms) (Transformation|GetActorTransform _array_element))
        (Utilities|Array|Add (Variables|Default|GetChestsForSave) (Utilities|MakeChestStruct _array_element)))))
  (Development|PrintString 0 "Start Writing")
  (Variables|/Game/Blueprints/A_Chest/SG_ChestStructs.SG_ChestStructs_C|SetChests _savegame _chestsforsave)
  (SaveGame|SaveGametoSlot _savegame "AllChests")
  (Development|PrintString 0 "Finish Writing")
  (Development|PrintString 0 (Utilities|String|Append "DONE SAVING " (Utilities|String|ToString(Integer) (Utilities|Array|Length _chestsforsave)) " CHESTS")))