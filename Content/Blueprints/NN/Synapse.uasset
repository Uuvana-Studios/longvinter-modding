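; Synapse Blueprint that models a weighted connection between a source and a target in a neural network.
; SetupSynapse runs once to store both endpoints and pick a random starting weight within a fixed range.
; GetWeightedValue returns the source's value multiplied by the weight, or prints a red error and returns zero when the source is invalid.
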(event Custom|Setup%20Synapse
  (params (Source :type Node%20Object%20Reference) (Target :type Node%20Object%20Reference))
  (Utilities|FlowControl|DoOnce false
    (:Completed
      (Variables|Default|SetSource Source)
      (Variables|Default|SetTarget Target)
      (Variables|Default|SetWeight (Math|Random|RandomFloatinRange -5.0 5.0)))))

(fn GetWeightedValue
  (bind _source (Variables|Default|GetSource))
  (Utilities|IsValid _source
    (:Is%20Valid
      (return (* (Variables|/Game/Blueprints/NN/Node.Node_C|GetValue _source) (Variables|Default|GetWeight))))
    (:Is%20Not%20Valid
      (Development|PrintString 0 "Synapse has no source!" true true "(R=1.000000,G=0.000000,B=0.000000,A=1.000000)" 0.0)
      (return 0.0))))