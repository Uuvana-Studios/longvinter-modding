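; Async task that checks whether an online session with the configured ServerName exists, and starts a session if none does.
; Execute runs a search capped at 200 results, then CheckIfSessionFound compares each result's ServerName setting to the target.
; A match only prints a message; otherwise it calls StartSession.
; The IsExperimental search filter is disconnected, and GetStringValueFromSettings contains only unused lookup nodes.
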(event EventExecute
  (Development|PrintString 0 "Check session")
  (bind _returnvalue (Game|ConstructObjectfromClass "/Script/OnlineSubsystemBlueprints.OnlineSessionSearch" self))
  (bind _output_get (Variables|Default|SetSearch%20Settings _returnvalue))
  (Variables|/Script/OnlineSubsystemBlueprints.OnlineSessionSearch|SetMaxSearchResults _output_get 200)
  (|FindSessions (Variables|Default|GetOnlineSession) (Class|OnlineIdentitySubsystem|GetUniquePlayerId (Variables|Default|GetOnlineIdentity)) _output_get
    (:OnFindSessionsComplete
      (bind _found (CallFunction|CheckifSessionFound))
      (if _found
        (Development|PrintString 0 "Session Found")
        (else
          (Default|StartSession (Variables|Default|GetAdvancedSessions)))))))

(fn CheckifSessionFound
  (for _array_element (Class|OnlineSessionSearch|GetSearchResults (Variables|Default|GetSearch%20Settings))
    (if (Utilities|Enum|Equal(Enum) (Utilities|GetStringValuefromSettings (Utilities|Name|MakeLiteralName "ServerName") _array_element) (Variables|Default|GetServerName))
      (return true)))
  (return false))