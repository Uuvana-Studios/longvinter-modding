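; Async task that saves the world's chests to disk across four save slots.
; Execute filters out chests flagged DontSave or, once two are recorded, sharing an already recorded transform, then converts the rest to structs.
; SplitChestsToBatches divides them by array index into four roughly equal groups, with overflow going to the first.
; One reused SaveGame object writes each group to an AllChestsBatch_ slot numbered by an incrementing BatchIndex.
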(event EventExecute
  (bind _chestsforsave (Variables|Default|GetChestsForSave))
  (bind _savegame (Variables|Default|GetSaveGame))
  (bind _batchindex (Variables|Default|GetBatchIndex))
  (bind _returnvalue (Utilities|String|ToString(Integer) _batchindex))
  (bind _returnvalue_2 (Utilities|String|Append "AllChestsBatch_" _returnvalue))
  (Utilities|Array|Clear (Variables|Default|GetChestsForSave))
  (Utilities|Array|Clear (Variables|Default|GetPlaceableDuplicationCheckTransforms))
  (for _array_element (Variables|Default|GetChests)
    (Utilities|ShouldSaveChest _array_element
      (:true
        (Utilities|Array|Add (Variables|Default|GetPlaceableDuplicationCheckTransforms) (Transformation|GetActorTransform _array_element))
        (Utilities|Array|Add (Variables|Default|GetChestsForSave) (Utilities|MakeChestStruct _array_element)))))
  (Development|PrintString 0 "Start Writing")
  (bind (_batch1 _batch2 _batch3 _batch4) (CallFunction|SplitCheststoBatches _chestsforsave))
  (Variables|/Game/Blueprints/A_Chest/SG_ChestStructs.SG_ChestStructs_C|SetChests _savegame _batch1)
  (SaveGame|SaveGametoSlot _savegame _returnvalue_2)
  (Math|Integer|IncrementInt (Variables|Default|GetBatchIndex)
    (:%20%20
      (Variables|/Game/Blueprints/A_Chest/SG_ChestStructs.SG_ChestStructs_C|SetChests _savegame _batch2)
      (SaveGame|SaveGametoSlot _savegame _returnvalue_2)
      (Math|Integer|IncrementInt (Variables|Default|GetBatchIndex)
        (:%20%20
          (Variables|/Game/Blueprints/A_Chest/SG_ChestStructs.SG_ChestStructs_C|SetChests _savegame _batch3)
          (SaveGame|SaveGametoSlot _savegame _returnvalue_2)
          (Math|Integer|IncrementInt (Variables|Default|GetBatchIndex)
            (:%20%20
              (Variables|/Game/Blueprints/A_Chest/SG_ChestStructs.SG_ChestStructs_C|SetChests _savegame _batch4)
              (SaveGame|SaveGametoSlot _savegame _returnvalue_2)
              (Development|PrintString 0 "Finish Writing")
              (Development|PrintString 0 (Utilities|String|Append "DONE SAVING " (Utilities|String|ToString(Integer) (Utilities|Array|Length _chestsforsave)) " CHESTS TO BATCHES")))))))))

(fn SplitCheststoBatches
  (params (Chests :type Array%20of%20Struct%20Chest%20Structures))
  (for (_array_element _array_index) Chests
    (switch int (Math|Float|Floor (/ (Math|Conversions|ToFloat(Integer) _array_index) (Math|Conversions|ToFloat(Integer) (Math|Float|Floor (/ (Math|Conversions|ToFloat(Integer) (- (Utilities|Array|Length Chests) 1)) 4.0)))))
      (:Default
        (Utilities|Array|Add (LocalVariables|GetBatch1Temp) _array_element :!label _label))
      (:0
        (goto _label))
      (:1
        (Utilities|Array|Add (LocalVariables|GetBatch2Temp) _array_element))
      (:2
        (Utilities|Array|Add (LocalVariables|GetBatch3Temp) _array_element))
      (:3
        (Utilities|Array|Add (LocalVariables|GetBatch4Temp) _array_element))))
  (return (LocalVariables|GetBatch1Temp) (LocalVariables|GetBatch2Temp) (LocalVariables|GetBatch3Temp) (LocalVariables|GetBatch4Temp)))