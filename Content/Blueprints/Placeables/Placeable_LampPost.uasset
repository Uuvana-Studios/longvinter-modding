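; Placeable lamp post that switches its light on and off when the game mode signals it.
; On BeginPlay the server resets LightsOn to false and binds handlers to GM_Longvinter's lights-on and lights-off events, which set that flag.
; The LightsOn RepNotify sets the light intensity, swaps the mesh's lamp material between lit and off, and flushes net dormancy.
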(event Custom|SetLightsOn
  (Variables|Default|SetLightsOn true))

(event Custom|SetLightsOff
  (Variables|Default|SetLightsOn false))

(event EventBeginPlay
  (|CallParentFunction)
  (Utilities|FlowControl|Sequence
    (:then_0
      (Networking|SwitchHasAuthority
        (:Authority
          (Variables|Default|SetLightsOn false)
          (bind _asgm_longvinter (Utilities|Casting|CastToGM_Longvinter (Game|GetGameMode)))
          (EventDispatchers|BindEventtoSetLightsON _asgm_longvinter (delegate Custom|SetLightsOn))
          (EventDispatchers|BindEventtoSetLightsOff _asgm_longvinter (delegate Custom|SetLightsOff)))))))

(event Collision|EventActorBeginOverlap
  (params (OtherActor :type Actor%20Object%20Reference)))

(event EventTick
  (params (DeltaSeconds :type Float%20%28single-precision%29)))

(fn ConstructionScript
  (|CallParentFunction))

(fn OnRepLightson
  (bind _lightmaterialindex (Variables|Default|GetLightMaterialIndex))
  (bind _light (Variables|Default|GetLight))
  (bind _sm_placeable (Variables|Default|GetSM_Placeable))
  (if (Variables|Default|GetLightsOn)
    (Rendering|Components|Light|SetIntensity _light (Variables|Default|GetLightIntensity))
    (Networking|FlushNetDormancy)
    (Rendering|Material|SetMaterial _sm_placeable _lightmaterialindex "/Game/Meshes/LampWPost/MI_LampWPost_Light.MI_LampWPost_Light")
    (else
      (Rendering|Components|Light|SetIntensity _light 0.0)
      (Networking|FlushNetDormancy)
      (Rendering|Material|SetMaterial _sm_placeable _lightmaterialindex "/Game/Meshes/LampWPost/MI_LampWPost_OFF.MI_LampWPost_OFF"))))