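; Player-placeable gate that only its owner can toggle on click, storing the placer's Steam ID in Comment and checking it on the server.
; Toggling uses a cooldown and FlipFlop to play a timeline swing with sound and set GateOpen.
; GateOpen's OnRep switches Pawn collision and snaps the door's final rotation, clearing the cooldown after a delay.
; OpenPublicDoor toggles without the owner check; material and mesh-array overrides include the Door mesh.
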(event Custom|SetGateClosed
  (Utilities|FlowControl|Delay 0.5)
  (Collision|SetCollisionResponsetoChannel (Variables|Default|GetSM_Placeable) "ECC_Pawn" "ECR_Block")
  (Collision|SetCollisionResponsetoChannel (Variables|Default|GetDoor) "ECC_Pawn" "ECR_Block")
  (Transformation|SetRelativeRotation (Variables|Default|GetDoor) "0, 0, 0" false false)
  (Variables|Default|SetCooldown false))

(event Custom|SetGateOpen
  (Collision|SetCollisionResponsetoChannel (Variables|Default|GetSM_Placeable) "ECC_Pawn" "ECR_Overlap")
  (Collision|SetCollisionResponsetoChannel (Variables|Default|GetDoor) "ECC_Pawn" "ECR_Overlap")
  (Utilities|FlowControl|Delay 0.5)
  (Transformation|SetRelativeRotation (Variables|Default|GetDoor) "0,160.000000, 0" false false)
  (Variables|Default|SetCooldown false))

(event Custom|checkPlayerAccess
  (params (Player :type Third%20Person%20Character%20Object%20Reference))
  (Networking|SwitchHasAuthority
    (:Authority
      (if (Utilities|Enum|Equal(Enum) (Class|AdvancedSessionsLibrary|UniqueNetIdtoString (Class|AdvancedSessionsLibrary|GetUniqueNetIDfromPlayerState (Variables|/Script/Engine.Pawn|GetPlayerState Player))) (Utilities|String|ToString(Text) (Variables|Default|GetComment)))
        (CallFunction|OpenGate)
        (else
          (Default|RunonClientErrorMessage Player "This gate is locked"))))))

(event Custom|RotateAnim
  (params (Reverse :type Boolean))
  (bind _returnvalue (Transformation|GetActorLocation))
  (if Reverse
    (Audio|PlaySoundatLocation "/Game/Audio/Misc/WAV_DoorOpen_02.WAV_DoorOpen_02" _returnvalue "0, 0, 0" 1.0 1.0 0.0 0 0 0)
    (Utilities|FlowControl|Sequence
      (:then_0
        (bind _rotation (Timeline|DoorRotate Stop)
          (:Update
            (Transformation|SetRelativeRotation (Variables|Default|GetDoor) (Math|Rotator|MakeRotator 0.0 0.0 _rotation) false false))))
      (:then_1
        (Timeline|DoorRotate ReverseFromEnd)))
    (else
      (Audio|PlaySoundatLocation "/Game/Audio/Misc/WAV_DoorOpen_01.WAV_DoorOpen_01" _returnvalue "0, 0, 0" 1.0 1.0 0.0 0 0 0)
      (Utilities|FlowControl|Sequence
        (:then_0
          (Timeline|DoorRotate Stop))
        (:then_1
          (Timeline|DoorRotate PlayFromStart))))))

(event Custom|OpenPublicDoor
  (params (Player :type Third%20Person%20Character%20Object%20Reference))
  (if (not (Variables|Default|GetCooldown))
    (Variables|Default|SetCooldown true)
    (Utilities|FlowControl|FlipFlop
      (:A
        (CallFunction|RotateAnim false)
        (Variables|Default|SetGateOpen true))
      (:B
        (CallFunction|RotateAnim true)
        (Variables|Default|SetGateOpen false)))))

(event Custom|OpenGate
  (if (not (Variables|Default|GetCooldown))
    (Variables|Default|SetCooldown true)
    (Utilities|FlowControl|FlipFlop
      (:A
        (CallFunction|RotateAnim false)
        (Variables|Default|SetGateOpen true))
      (:B
        (CallFunction|RotateAnim true)
        (Variables|Default|SetGateOpen false)))
    (Networking|FlushNetDormancy)
    (Networking|ForceNetUpdate)))

(event EventBeginPlay
  (|CallParentFunction)
  (Variables|Default|SetGateOpen (Variables|Default|GetGateOpen)))

(event Collision|EventActorBeginOverlap
  (params (OtherActor :type Actor%20Object%20Reference))
  (|CallParentFunction OtherActor) ; This node is disabled and will not be called.\nDrag off pins to build functionality.
)

(event EventTick
  (params (DeltaSeconds :type Float%20%28single-precision%29))
  (|CallParentFunction DeltaSeconds) ; This node is disabled and will not be called.\nDrag off pins to build functionality.
)

(event EventPlaced
  (params (SteamID :type String))
  (Variables|Default|SetComment (Utilities|Text|ToText(String) SteamID)))

(event EventClicked
  (params (Player :type Third%20Person%20Character%20Object%20Reference))
  (CallFunction|CheckPlayerAccess Player))

(fn ConstructionScript
  (|CallParentFunction))

(fn OnRepGateOpen
  (if (Variables|Default|GetGateOpen)
    (CallFunction|SetGateOpen)
    (else
      (CallFunction|SetGateClosed))))

(fn ChangeMaterial
  (params (Material :type Material%20Interface%20Object%20Reference))
  (bind _door (Variables|Default|GetDoor))
  (for _index (range 0 (Rendering|Material|GetNumMaterials (Variables|Default|GetSM_Placeable)))
    (Rendering|Material|SetMaterial (Variables|Default|GetSM_Placeable) _index Material))
  (for _index_2 (range 0 (Rendering|Material|GetNumMaterials _door))
    (Rendering|Material|SetMaterial _door _index_2 Material))
  (|CallParentFunction Material))

(fn AddMeshestoArray
  (|CallParentFunction)
  (Utilities|Array|Add (Variables|Default|GetPlaceablesMeshes) (Variables|Default|GetDoor)))