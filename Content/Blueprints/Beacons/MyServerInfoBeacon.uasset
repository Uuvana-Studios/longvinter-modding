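; MyServerInfoBeacon is a one-shot beacon that fetches the server's current gamemode and map for a client.
; On connection it requests info; the server side reads both values from ServerInfoGamemode and returns them to the client.
; The response or a connection failure fires the OnServerInfoReceived delegate with a success flag, then disconnects the beacon.
; A failed game mode cast sends no response.
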(event Custom|Request%20Server%20Info
  ;[1 1 1] We are now on the server, we can cast to game mode and get all necessary information and return it to the client.
  (bind _asserver_info_gamemode (Utilities|Casting|CastToServerInfoGamemode (Game|GetGameMode)))
  (CallFunction|OnServerResponse (Variables|/BlueprintableOnlineBeacons/Examples/ServerInfoGamemode.ServerInfoGamemode_C|GetGamemode _asserver_info_gamemode) (Variables|/BlueprintableOnlineBeacons/Examples/ServerInfoGamemode.ServerInfoGamemode_C|GetMap _asserver_info_gamemode)))

(event Custom|On%20Server%20Response
  (params (Gamemode :type Name) (Map :type Name))
  ;[1 1 1] When we receive the Info from the Server, call a delegate to dispatch info.
  ; Since this is a one-shot beacon, we disconnect as well.
  (Default|CallOnServerInfoReceived true Gamemode Map)
  (Class|OnlineBeaconBlueprint|Disconnect))

(event EventOnConnectedBlueprint
  ;[1 1 1] When we connect, request server info.
  (CallFunction|RequestServerInfo))

(event EventOnConnectionFailureBlueprint
  ;[1 1 1] On the case we failed to connect, return our delegate with a fail and destroy this beacon.
  (Default|CallOnServerInfoReceived false)
  (Class|OnlineBeaconBlueprint|Disconnect))

(fn ConstructionScript)