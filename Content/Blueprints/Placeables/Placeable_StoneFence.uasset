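; Placeable stone fence segment with two end pillars, which hides duplicate pillars where neighboring fences meet.
; Shortly after BeginPlay and on CollisionCheck2 overlap changes, CheckPillar runs on non-authority instances only.
; It sets each pillar's visibility from whether the overlapping pillar on another stone fence is flagged as shown.
; Both pillars also join the parent's placeable mesh array and follow its material changes.
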(event OnComponentBeginOverlap(CollisionCheck2)
  (params (OverlappedComponent :type Primitive%20Component%20Object%20Reference) (OtherActor :type Actor%20Object%20Reference) (OtherComp :type Primitive%20Component%20Object%20Reference) (OtherBodyIndex :type Integer) (bFromSweep :type Boolean) (SweepResult :type Hit%20Result%20Structure%20%28by%20ref%29))
  (CallFunction|CheckPillar))

(event OnComponentEndOverlap(CollisionCheck2)
  (params (OverlappedComponent :type Primitive%20Component%20Object%20Reference) (OtherActor :type Actor%20Object%20Reference) (OtherComp :type Primitive%20Component%20Object%20Reference) (OtherBodyIndex :type Integer))
  (CallFunction|CheckPillar))

(event Custom|CheckPillar
  (bind _sm_pillar2 (Variables|Default|GetSM_Pillar2))
  (bind _sm_pillar1 (Variables|Default|GetSM_Pillar1))
  (Networking|SwitchHasAuthority
    (:Remote
      (Utilities|FlowControl|Sequence
        (:then_0
          (bind _array_element (Utilities|Array|ForEachLoopwithBreak (Collision|GetOverlappingActors _sm_pillar1 "Placeable_StoneFence_C" :!class /Script/Engine.PrimitiveComponent))
            (:LoopBody
              (bind _asplaceable_stone_fence (Utilities|Casting|CastToPlaceable_StoneFence _array_element))
              (if (Class|PrimitiveComponent|IsOverlappingComponent _sm_pillar1 (Variables|Placeable_StoneFence_C|GetSM_Pillar1 _asplaceable_stone_fence))
                (if (Variables|Placeable_StoneFence_C|GetShowPillar1 _asplaceable_stone_fence)
                  (Variables|Default|SetShowPillar1 false)
                  (else
                    (Variables|Default|SetShowPillar1 true)))
                (elif (Class|PrimitiveComponent|IsOverlappingComponent _sm_pillar1 (Variables|Placeable_StoneFence_C|GetSM_Pillar2 _asplaceable_stone_fence))
                  (if (Variables|Placeable_StoneFence_C|GetShowPillar2 _asplaceable_stone_fence)
                    (Variables|Default|SetShowPillar1 false)
                    (else
                      (Variables|Default|SetShowPillar1 true :!label _label)))
                  (else
                    (goto _label)))))
            (:Completed
              (Rendering|SetVisibility (Variables|Default|GetSM_Pillar1) (Variables|Default|GetShowPillar1) false))))
        (:then_1
          (bind _array_element_2 (Utilities|Array|ForEachLoopwithBreak (Collision|GetOverlappingActors _sm_pillar2 "Placeable_StoneFence_C" :!class /Script/Engine.PrimitiveComponent))
            (:LoopBody
              (bind _asplaceable_stone_fence_2 (Utilities|Casting|CastToPlaceable_StoneFence _array_element_2))
              (if (Class|PrimitiveComponent|IsOverlappingComponent _sm_pillar2 (Variables|Placeable_StoneFence_C|GetSM_Pillar1 _asplaceable_stone_fence_2))
                (if (Variables|Placeable_StoneFence_C|GetShowPillar1 _asplaceable_stone_fence_2)
                  (Variables|Default|SetShowPillar2 false)
                  (else
                    (Variables|Default|SetShowPillar2 true)))
                (elif (Class|PrimitiveComponent|IsOverlappingComponent _sm_pillar2 (Variables|Placeable_StoneFence_C|GetSM_Pillar2 _asplaceable_stone_fence_2))
                  (if (Variables|Placeable_StoneFence_C|GetShowPillar2 _asplaceable_stone_fence_2)
                    (Variables|Default|SetShowPillar2 false)
                    (else
                      (Variables|Default|SetShowPillar2 true :!label _label_2)))
                  (else
                    (goto _label_2)))))
            (:Completed
              (Rendering|SetVisibility (Variables|Default|GetSM_Pillar2) (Variables|Default|GetShowPillar2) false))))))))

(event EventBeginPlay
  (|CallParentFunction)
  (Utilities|FlowControl|Delay 0.2)
  (CallFunction|CheckPillar))

(fn ConstructionScript
  (|CallParentFunction))

(fn ChangeMaterial
  (params (Material :type Material%20Interface%20Object%20Reference))
  (bind _sm_pillar1 (Variables|Default|GetSM_Pillar1))
  (for _index (range 0 (Rendering|Material|GetNumMaterials (Variables|Default|GetSM_Placeable)))
    (Rendering|Material|SetMaterial (Variables|Default|GetSM_Placeable) _index Material))
  (for _index_2 (range 0 (Rendering|Material|GetNumMaterials _sm_pillar1))
    (Rendering|Material|SetMaterial _sm_pillar1 _index_2 Material))
  (|CallParentFunction Material))

(fn AddMeshestoArray
  (bind _placeablesmeshes (Variables|Default|GetPlaceablesMeshes))
  (|CallParentFunction)
  (Utilities|Array|Add _placeablesmeshes (Variables|Default|GetSM_Pillar1))
  (Utilities|Array|Add _placeablesmeshes (Variables|Default|GetSM_Pillar2)))