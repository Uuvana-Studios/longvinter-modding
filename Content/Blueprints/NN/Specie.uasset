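; Specie is one member of a neural-network evolution system, owning a Brain and tracking its fitness.
; SetupSpecie constructs the Brain from the layer neuron counts; SetInputs writes values into the first-layer neurons and fires it, and GetOutputs returns the result.
; EndRun marks the specie dead and counts consecutive generations in which Fitness fails to beat the previous run's value.
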(event Custom|Set%20Inputs
  (params (Inputs :type Array%20of%20Floats%20%28single-precision%29))
  (for _index (range 0 (- (Utilities|Array|Get(acopy) (Variables|Default|GetNeuron%20Counts)) 1))
    (Variables|/Game/Blueprints/NN/Node.Node_C|SetValue (Utilities|Array|Get(acopy) (Variables|/Game/Blueprints/NN/Brain.Brain_C|GetNeurons (Variables|Default|GetBrain)) _index) (Utilities|Array|Get(acopy) Inputs _index)))
  (Default|Fire (Variables|Default|GetBrain)))

(event Custom|End%20Run
  (Variables|Default|SetAlive false)
  (if (> (Variables|Default|GetFitness) (Variables|Default|GetLast%20Fitness))
    (Variables|Default|SetUnderperforming%20for%20Generations 0)
    (else
      (Math|Integer|IncrementInt (Variables|Default|GetUnderperforming%20for%20Generations)
        (:%20%20
          _))))
  (Variables|Default|SetLast%20Fitness (Variables|Default|GetFitness)))

(event Custom|Setup%20Specie
  (bind _returnvalue (Game|ConstructObjectfromClass "/Game/Blueprints/NN/Brain.Brain_C" self (Variables|Default|GetNeuron%20Counts)))
  (Default|SetupBrain _returnvalue)
  (Variables|Default|SetBrain _returnvalue))

(fn GetOutputs
  (return (Default|GetOutputs (Variables|Default|GetBrain))))