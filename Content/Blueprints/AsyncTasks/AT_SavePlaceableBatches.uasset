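; Async task that saves the world's placeables, with class, transform, comment, placer Steam ID and item data, across four save slots.
; Execute gathers placeables flagged for saving, using a transform check meant to skip duplicates, into parallel arrays.
; Matching split functions divide each array into four batches by index, with overflow indices falling into the first.
; WriteToBatch copies each batch into the SaveGame object and saves it to its slot.
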(event EventExecute
  (for _array_element (Variables|Default|GetPlaceables)
    (Utilities|ShouldSavePlaceable _array_element
      (:true
        (Utilities|Array|Add (Variables|Default|GetPlaceableDuplicationCheckTransforms) (Transformation|GetActorTransform _array_element))
        (Utilities|Array|Add (Variables|Default|GetPlaceableTransforms) (Transformation|GetActorTransform _array_element))
        (Utilities|Array|Add (Variables|Default|GetPlaceableClass) (Utilities|GetClass _array_element))
        (Utilities|Array|Add (Variables|Default|GetPlaceableComments) (Variables|/Game/Blueprints/Placeables/A_Placeable.A_Placeable_C|GetComment _array_element))
        (Utilities|Array|Add (Variables|Default|GetPlaceableIDs) (Variables|/Game/Blueprints/Placeables/A_Placeable.A_Placeable_C|GetPlacerSteamID _array_element))
        (Utilities|Array|Add (Variables|Default|GetPlaceableItemDatas) (Variables|/Game/Blueprints/Placeables/A_Placeable.A_Placeable_C|GetItemData _array_element)))))
  (Development|PrintString 0 "Start Writing")
  (bind (_batch1 _batch2 _batch3 _batch4) (CallFunction|SplitClassestoBatches (Variables|Default|GetPlaceableClass)))
  (bind (_batch1_2 _batch2_2 _batch3_2 _batch4_2) (CallFunction|SplitTransformstoBatches (Variables|Default|GetPlaceableTransforms)))
  (bind (_batch1_3 _batch2_3 _batch3_3 _batch4_3) (CallFunction|SplitCommentstoBatches (Variables|Default|GetPlaceableComments)))
  (bind (_batch1_4 _batch2_4 _batch3_4 _batch4_4) (CallFunction|SplitIDstoBatches (Variables|Default|GetPlaceableIDs)))
  (bind (_batch1_5 _batch2_5 _batch3_5 _batch4_5) (CallFunction|SplitItemDatastoBatches (Variables|Default|GetPlaceableItemDatas)))
  (Utilities|FlowControl|Sequence
    (:then_0
      (CallFunction|WritetoBatch "AllPlaceablesBatch_0" _batch1 _batch1_3 _batch1_4 _batch1_2 _batch1_5))
    (:then_1
      (CallFunction|WritetoBatch "AllPlaceablesBatch_1" _batch2 _batch2_3 _batch2_4 _batch2_2 _batch2_5))
    (:then_2
      (CallFunction|WritetoBatch "AllPlaceablesBatch_2" _batch3 _batch3_3 _batch3_4 _batch3_2 _batch3_5))
    (:then_3
      (CallFunction|WritetoBatch "AllPlaceablesBatch_3" _batch4 _batch4_3 _batch4_4 _batch4_2 _batch4_5))
    (:then_4
      (Development|PrintString 0 "Finish Writing")
      (Development|PrintString 0 (Utilities|String|Append "DONE SAVING " (Utilities|String|ToString(Integer) (Utilities|Array|Length (Variables|Default|GetPlaceableClass))) " PLACEABLES")))))

(fn SplitClassestoBatches
  (params (Classes :type Array%20of%20A%20Placeable%20Class%20References))
  (for (_array_element _array_index) Classes
    (switch int (Math|Float|Floor (/ (Math|Conversions|ToFloat(Integer) _array_index) (Math|Conversions|ToFloat(Integer) (Math|Float|Floor (/ (Math|Conversions|ToFloat(Integer) (- (Utilities|Array|Length Classes) 1)) 4.0)))))
      (:Default
        (Utilities|Array|Add (LocalVariables|GetBatch1Temp) _array_element :!label _label))
      (:0
        (goto _label))
      (:1
        (Utilities|Array|Add (LocalVariables|GetBatch2Temp) _array_element))
      (:2
        (Utilities|Array|Add (LocalVariables|GetBatch3Temp) _array_element))
      (:3
        (Utilities|Array|Add (LocalVariables|GetBatch4Temp) _array_element))))
  (return (LocalVariables|GetBatch1Temp) (LocalVariables|GetBatch2Temp) (LocalVariables|GetBatch3Temp) (LocalVariables|GetBatch4Temp)))

(fn SplitTransformstoBatches
  (params (Transforms :type Array%20of%20Transforms))
  (for (_array_element _array_index) Transforms
    (switch int (Math|Float|Floor (/ (Math|Conversions|ToFloat(Integer) _array_index) (Math|Conversions|ToFloat(Integer) (Math|Float|Floor (/ (Math|Conversions|ToFloat(Integer) (- (Utilities|Array|Length Transforms) 1)) 4.0)))))
      (:Default
        (Utilities|Array|Add (LocalVariables|GetBatch1Temp) _array_element :!label _label))
      (:0
        (goto _label))
      (:1
        (Utilities|Array|Add (LocalVariables|GetBatch2Temp) _array_element))
      (:2
        (Utilities|Array|Add (LocalVariables|GetBatch3Temp) _array_element))
      (:3
        (Utilities|Array|Add (LocalVariables|GetBatch4Temp) _array_element))))
  (return (LocalVariables|GetBatch1Temp) (LocalVariables|GetBatch2Temp) (LocalVariables|GetBatch3Temp) (LocalVariables|GetBatch4Temp)))

(fn SplitCommentstoBatches
  (params (Comments :type Array%20of%20Texts))
  (for (_array_element _array_index) Comments
    (switch int (Math|Float|Floor (/ (Math|Conversions|ToFloat(Integer) _array_index) (Math|Conversions|ToFloat(Integer) (Math|Float|Floor (/ (Math|Conversions|ToFloat(Integer) (- (Utilities|Array|Length Comments) 1)) 4.0)))))
      (:Default
        (Utilities|Array|Add (LocalVariables|GetBatch1Temp) _array_element :!label _label))
      (:0
        (goto _label))
      (:1
        (Utilities|Array|Add (LocalVariables|GetBatch2Temp) _array_element))
      (:2
        (Utilities|Array|Add (LocalVariables|GetBatch3Temp) _array_element))
      (:3
        (Utilities|Array|Add (LocalVariables|GetBatch4Temp) _array_element))))
  (return (LocalVariables|GetBatch1Temp) (LocalVariables|GetBatch2Temp) (LocalVariables|GetBatch3Temp) (LocalVariables|GetBatch4Temp)))

(fn SplitIDstoBatches
  (params (IDs :type Array%20of%20Strings))
  (for (_array_element _array_index) IDs
    (switch int (Math|Float|Floor (/ (Math|Conversions|ToFloat(Integer) _array_index) (Math|Conversions|ToFloat(Integer) (Math|Float|Floor (/ (Math|Conversions|ToFloat(Integer) (- (Utilities|Array|Length IDs) 1)) 4.0)))))
      (:Default
        (Utilities|Array|Add (LocalVariables|GetBatch1Temp) _array_element :!label _label))
      (:0
        (goto _label))
      (:1
        (Utilities|Array|Add (LocalVariables|GetBatch2Temp) _array_element))
      (:2
        (Utilities|Array|Add (LocalVariables|GetBatch3Temp) _array_element))
      (:3
        (Utilities|Array|Add (LocalVariables|GetBatch4Temp) _array_element))))
  (return (LocalVariables|GetBatch1Temp) (LocalVariables|GetBatch2Temp) (LocalVariables|GetBatch3Temp) (LocalVariables|GetBatch4Temp)))

(fn SplitItemDatastoBatches
  (params (ItemDatas :type Array%20of%20S%20Item%20Data%20Rename%202%20Structures))
  (for (_array_element _array_index) ItemDatas
    (switch int (Math|Float|Floor (/ (Math|Conversions|ToFloat(Integer) _array_index) (Math|Conversions|ToFloat(Integer) (Math|Float|Floor (/ (Math|Conversions|ToFloat(Integer) (- (Utilities|Array|Length ItemDatas) 1)) 4.0)))))
      (:Default
        (Utilities|Array|Add (LocalVariables|GetBatch1Temp) _array_element :!label _label))
      (:0
        (goto _label))
      (:1
        (Utilities|Array|Add (LocalVariables|GetBatch2Temp) _array_element))
      (:2
        (Utilities|Array|Add (LocalVariables|GetBatch3Temp) _array_element))
      (:3
        (Utilities|Array|Add (LocalVariables|GetBatch4Temp) _array_element))))
  (return (LocalVariables|GetBatch1Temp) (LocalVariables|GetBatch2Temp) (LocalVariables|GetBatch3Temp) (LocalVariables|GetBatch4Temp)))

(fn WritetoBatch
  (params (SlotName :type String) (Classes :type Array%20of%20A%20Placeable%20Class%20References) (Comments :type Array%20of%20Texts) (IDs :type Array%20of%20Strings) (Transforms :type Array%20of%20Transforms) (ItemDatas :type Array%20of%20S%20Item%20Data%20Rename%202%20Structures))
  (bind _savegame (Variables|Default|GetSaveGame))
  (Variables|/Game/Blueprints/Placeables/SG_Placeable.SG_Placeable_C|SetClasses _savegame Classes)
  (Variables|/Game/Blueprints/Placeables/SG_Placeable.SG_Placeable_C|SetComments _savegame Comments)
  (Variables|/Game/Blueprints/Placeables/SG_Placeable.SG_Placeable_C|SetIDs _savegame IDs)
  (Variables|/Game/Blueprints/Placeables/SG_Placeable.SG_Placeable_C|SetTransforms _savegame Transforms)
  (Variables|/Game/Blueprints/Placeables/SG_Placeable.SG_Placeable_C|SetItemDatas _savegame ItemDatas)
  (SaveGame|SaveGametoSlot _savegame SlotName))