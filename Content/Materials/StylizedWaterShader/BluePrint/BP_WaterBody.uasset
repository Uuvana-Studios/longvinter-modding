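; Stylized water body actor that flags third-person characters as being in water.
; Begin and end overlap on its WaterMovementSpeed component cast the other actor to ThirdPersonCharacter and set or clear InWater directly.
; Unconnected nodes hold server/client setters, walk-speed reduction, aim disabling and a timer for RemoveEnergy.
; RemoveEnergy would drain a stored Player's energy, but no live path calls it.
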(event OnComponentBeginOverlap(WaterMovementSpeed)
  (params (OverlappedComponent :type Primitive%20Component%20Object%20Reference) (OtherActor :type Actor%20Object%20Reference) (OtherComp :type Primitive%20Component%20Object%20Reference) (OtherBodyIndex :type Integer) (bFromSweep :type Boolean) (SweepResult :type Hit%20Result%20Structure%20%28by%20ref%29))
  (bind _asthird_person_character (Utilities|Casting|CastToThirdPersonCharacter OtherActor))
  (Variables|/Game/ThirdPersonCPP/Blueprints/ThirdPersonCharacter.ThirdPersonCharacter_C|SetInWater _asthird_person_character true))

(event OnComponentEndOverlap(WaterMovementSpeed)
  (params (OverlappedComponent :type Primitive%20Component%20Object%20Reference) (OtherActor :type Actor%20Object%20Reference) (OtherComp :type Primitive%20Component%20Object%20Reference) (OtherBodyIndex :type Integer))
  (bind _asthird_person_character (Utilities|Casting|CastToThirdPersonCharacter OtherActor))
  (Variables|/Game/ThirdPersonCPP/Blueprints/ThirdPersonCharacter.ThirdPersonCharacter_C|SetInWater _asthird_person_character false))

(event EventBeginPlay)

(event Collision|EventActorBeginOverlap
  (params (OtherActor :type Actor%20Object%20Reference)))

(event EventTick
  (params (DeltaSeconds :type Float%20%28single-precision%29)))

(fn ConstructionScript)

(fn RemoveEnergy
  (bind _player (Variables|Default|GetPlayer))
  (Utilities|IsValid _player
    (:Is%20Valid
      (Default|RemoveEnergyServer _player 1.0 0 true))))