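; Spectator pawn that lets the local player adjust camera zoom and return to their original pawn.
; On BeginPlay it stores its instigator as the pawn to return to.
; X and Z narrow or widen the camera field of view in fixed, unclamped steps.
; R shows the cursor, prints a debug string, then calls RePossess to possess the stored pawn and destroy the spectator; other cursor and input-mode logic is unwired.
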(event Custom|RePossess
  (params (Target :type Controller%20Object%20Reference) (InPawn :type Pawn%20Object%20Reference))
  (Pawn|Possess (Game|GetPlayerController 0) InPawn)
  (Actor|DestroyActor))

(event EventBeginPlay
  (Variables|Default|SetPlayerPawn (Game|GetInstigator)))

(event EventTick
  (params (DeltaSeconds :type Float%20%28single-precision%29)))

(event Input|KeyboardEvents|R
  (params (Key :type Key%20Structure :default "None"))
  (:Pressed
    (Variables|/Script/Engine.PlayerController|SetbShowMouseCursor (Game|GetPlayerController 0) true)
    (Development|PrintString "Hello")
    (CallFunction|RePossess 0 (Variables|Default|GetPlayerPawn))))

(event Input|KeyboardEvents|Z
  (params (Key :type Key%20Structure :default "None"))
  (bind _camera (Variables|Default|GetCamera))
  (:Pressed
    (Camera|SetFieldOfView _camera (+ (Variables|/Script/Engine.CameraComponent|GetFieldOfView _camera) 5.0))))

(event Input|KeyboardEvents|X
  (params (Key :type Key%20Structure :default "None"))
  (bind _camera (Variables|Default|GetCamera))
  (:Pressed
    (Camera|SetFieldOfView _camera (- (Variables|/Script/Engine.CameraComponent|GetFieldOfView _camera) 5.0))))

(event Input|KeyboardEvents|LeftShift
  (params (Key :type Key%20Structure :default "None")))

(fn ConstructionScript)