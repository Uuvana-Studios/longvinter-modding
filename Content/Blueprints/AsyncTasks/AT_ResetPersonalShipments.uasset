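; Async task that resets personal shipments in the save of each listed player whose first shipment value is 1.
; If all three are completed, a stored counter sets the new items' rarity tier; otherwise it clears, completed shipments add a half-price payout, and the lowest tier applies.
; Random items are filtered by rarity, price, slot and exclusions, with price-scaled amounts.
; Results update the save slot, matching PlayerState and cached PlayerSaves.
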(event EventExecute
  (bind _playersaves (Variables|Default|GetplayerSaves))
  (for _array_element (Variables|Default|GetPlayerIDs)
    (bind _returnvalue (SaveGame|LoadGamefromSlot _array_element))
    (bind _assg_player_data (Utilities|Casting|CastToSG_PlayerData _returnvalue))
    (bind _output_get (Variables|Default|SetSG_PlayerData _assg_player_data))
    (bind _output_get_2 (Variables|Default|SetShipment (.Shipments (Utilities|Struct|BreakStuct_PlayerData1 (Variables|/Game/Blueprints/SG_PlayerData.SG_PlayerData_C|GetData _output_get)))))
    (if (== (Utilities|Array|Get(acopy) _output_get_2) 1)
      (if (Math|Boolean|ANDBoolean (.Completed (Utilities|GetShipmentValues (Variables|Default|GetShipment) 13 "NewEnumerator0")) (.Completed (Utilities|GetShipmentValues (Variables|Default|GetShipment) 12 "NewEnumerator0")) (.Completed (Utilities|GetShipmentValues (Variables|Default|GetShipment) 11 "NewEnumerator0")))
        (if (> (Utilities|Array|Get(acopy) (Variables|Default|GetShipment) 4) 4)
          (if (> (Utilities|Array|Get(acopy) (Variables|Default|GetShipment) 4) 8)
            (bind _updatedshipment (CallFunction|AddNewRandomItemtoShipments 11 "NewEnumerator2" (Variables|Default|GetShipment)))
            (bind _updatedshipment_2 (CallFunction|AddNewRandomItemtoShipments 12 "NewEnumerator2" _updatedshipment))
            (bind _updatedshipment_3 (CallFunction|AddNewRandomItemtoShipments 13 "NewEnumerator2" _updatedshipment_2))
            (Variables|Default|SetShipment _updatedshipment_3)
            (else
              (bind _updatedshipment_4 (CallFunction|AddNewRandomItemtoShipments 11 "NewEnumerator1" (Variables|Default|GetShipment)))
              (bind _updatedshipment_5 (CallFunction|AddNewRandomItemtoShipments 12 "NewEnumerator1" _updatedshipment_4))
              (bind _updatedshipment_6 (CallFunction|AddNewRandomItemtoShipments 13 "NewEnumerator2" _updatedshipment_5))
              (Variables|Default|SetShipment _updatedshipment_6)))
          (else
            (bind _updatedshipment_7 (CallFunction|AddNewRandomItemtoShipments 11 "NewEnumerator0" (Variables|Default|GetShipment) :!label _label))
            (bind _updatedshipment_8 (CallFunction|AddNewRandomItemtoShipments 12 "NewEnumerator0" _updatedshipment_7))
            (bind _updatedshipment_9 (CallFunction|AddNewRandomItemtoShipments 13 "NewEnumerator1" _updatedshipment_8))
            (Variables|Default|SetShipment _updatedshipment_9)))
        (else
          (Utilities|Array|SetArrayElem (Variables|Default|GetShipment) 4 0 true)
          (bind _payouttopay (CallFunction|GetPartiallyFilledPersonalShipmentPayout (Variables|Default|GetShipment)))
          (Utilities|Array|SetArrayElem (Variables|Default|GetShipment) 5 (+ _payouttopay (Utilities|Array|Get(acopy) (Variables|Default|GetShipment) 5)) true)
          (goto _label)))
      (bind _structout (Utilities|Struct|SetmembersinStuct_PlayerData1 (Variables|/Game/Blueprints/SG_PlayerData.SG_PlayerData_C|GetData _output_get) (Variables|Default|GetShipment)))
      (Variables|/Game/Blueprints/SG_PlayerData.SG_PlayerData_C|SetData (Variables|Default|GetSG_PlayerData) _structout)
      (SaveGame|SaveGametoSlot (Variables|Default|GetSG_PlayerData) _array_element)
      (bind _array_element_2 (Utilities|Array|ForEachLoopwithBreak (Variables|Default|GetPlayers) :!label _label_2)
        (:LoopBody
          (if (Utilities|Enum|Equal(Enum) _array_element (Class|AdvancedSessionsLibrary|UniqueNetIdtoString (Class|AdvancedSessionsLibrary|GetUniqueNetIDfromPlayerState _array_element_2)))
            (bind _asps_longvinter (Utilities|Casting|CastToPS_Longvinter _array_element_2))
            (Variables|/Game/Blueprints/PS_Longvinter.PS_Longvinter_C|SetShipments _asps_longvinter (Variables|Default|GetShipment))
            (goto _label_2 Break)))
        (:Completed
          (if (.ReturnValue (Utilities|Map|Find _playersaves _array_element))
            (bind _structout_2 (Utilities|Struct|SetmembersinStuct_PlayerData1 (.Value (Utilities|Map|Find _playersaves _array_element)) (Variables|Default|GetShipment)))
            (Utilities|Map|Add _playersaves _array_element _structout_2)))))))

(fn AddNewRandomItemtoShipments
  (params (PersonalShipmentIndex :type Integer) (Rarity :type itemRarityEnum%20Enum :default "NewEnumerator0") (Shipment :type Array%20of%20Integers))
  (bind (_item _amount) (CallFunction|RandomShipmentItem (Variables|Default|GetItems) Rarity))
  (Utilities|Array|SetArrayElem Shipment PersonalShipmentIndex _item true)
  (Utilities|Array|SetArrayElem Shipment (+ PersonalShipmentIndex 3) _amount true)
  (Utilities|Array|SetArrayElem Shipment (- PersonalShipmentIndex 10) 0 true)
  (return Shipment))

(fn GetPartiallyFilledPersonalShipmentPayout
  (params (Shipments :type Array%20of%20Integers))
  (bind (_maximum _currentprogress _amountleft _itemindex _completed) (Utilities|GetShipmentValues Shipments 11 "NewEnumerator0"))
  (bind (_maximum_2 _currentprogress_2 _amountleft_2 _itemindex_2 _completed_2) (Utilities|GetShipmentValues Shipments 12 "NewEnumerator0"))
  (bind (_maximum_3 _currentprogress_3 _amountleft_3 _itemindex_3 _completed_3) (Utilities|GetShipmentValues Shipments 13 "NewEnumerator0"))
  (bind _items (Variables|Default|GetItems))
  (if _completed
    (LocalVariables|Setpayout (+ (* (Math|Float|Round (* (.defaultPrice (Utilities|Struct|BreakS_ItemData_Rename2 (Utilities|Array|Get(acopy) _items _itemindex))) 0.5)) _currentprogress) (LocalVariables|Getpayout))))
  (if _completed_2
    (LocalVariables|Setpayout (+ (* (Math|Float|Round (* (.defaultPrice (Utilities|Struct|BreakS_ItemData_Rename2 (Utilities|Array|Get(acopy) _items _itemindex_2))) 0.5)) _currentprogress_2) (LocalVariables|Getpayout))))
  (if _completed_3
    (LocalVariables|Setpayout (+ (* _currentprogress_3 (Math|Float|Round (* (.defaultPrice (Utilities|Struct|BreakS_ItemData_Rename2 (Utilities|Array|Get(acopy) _items _itemindex_3))) 0.5))) (LocalVariables|Getpayout))))
  (return (LocalVariables|Getpayout)))

(fn RandomShipmentItem
  (params (Items :type Array%20of%20S%20Item%20Data%20Rename%202%20Structures) (Rarity :type itemRarityEnum%20Enum :default "NewEnumerator0"))
  (bind _output_get (LocalVariables|SetItemsLocal Items))
  (for (_array_element _array_index) _output_get
    (if (Math|Boolean|ANDBoolean (Utilities|Enum|Equal(Enum) (.rarity (Utilities|Struct|BreakS_ItemData_Rename2 _array_element)) Rarity) (> (.defaultPrice (Utilities|Struct|BreakS_ItemData_Rename2 _array_element)) 98) (< (.defaultPrice (Utilities|Struct|BreakS_ItemData_Rename2 _array_element)) 1995) (not (Utilities|Array|ContainsItem (Utilities|Array|MakeArray 235 249 250 8 66 67) _array_index)) (!= (.Slot (Utilities|Struct|BreakS_ItemData_Rename2 _array_element)) 1))
      (Utilities|Array|Add (LocalVariables|GetItemsToSchoose) _array_index)))
  (bind _output_get_2 (LocalVariables|SetRandomItem (.OutItem (Utilities|Array|Random (LocalVariables|GetItemsToSchoose)))))
  (return (LocalVariables|GetRandomItem) (Math|Integer|Max(Integer) (/ 3000 (.defaultPrice (Utilities|Struct|BreakS_ItemData_Rename2 (Utilities|Array|Get(acopy) (LocalVariables|GetItemsLocal) _output_get_2)))) 2)))