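; Pawn used in the character creation menu that detects whether the player is on keyboard or controller.
; Keyboard presses clear the UsingController flag on PC_CharacterMenu, while controller presses or axis movement of at least half magnitude set it.
; Each detection then calls SetupUMG on GM_CharacterCreation with the matching flag so the UI is set up for that input type.
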(event EventBeginPlay)

(event Collision|EventActorBeginOverlap
  (params (OtherActor :type Actor%20Object%20Reference)))

(event EventTick
  (params (DeltaSeconds :type Float%20%28single-precision%29)))

(event Input|ActionEvents|InputActionControllerInput
  (params (Key :type Key%20Structure))
  (:Pressed
    (bind _aspc_character_menu (Utilities|Casting|CastToPC_CharacterMenu (Game|GetPlayerController 0)))
    (Variables|/Game/Blueprints/CharacterCreation/PC_CharacterMenu.PC_CharacterMenu_C|SetUsingController _aspc_character_menu true)
    (bind _asgm_character_creation (Utilities|Casting|CastToGM_CharacterCreation (Game|GetGameMode)))
    (Default|SetupUMG _asgm_character_creation true)))

(event Input|ActionEvents|InputActionKeyboardInput
  (params (Key :type Key%20Structure))
  (:Pressed
    (bind _aspc_character_menu (Utilities|Casting|CastToPC_CharacterMenu (Game|GetPlayerController 0)))
    (Variables|/Game/Blueprints/CharacterCreation/PC_CharacterMenu.PC_CharacterMenu_C|SetUsingController _aspc_character_menu false)
    (bind _asgm_character_creation (Utilities|Casting|CastToGM_CharacterCreation (Game|GetGameMode)))
    (Default|SetupUMG _asgm_character_creation false)))

(event Input|AxisEvents|InputAxisControllerAxisInput
  (params (AxisValue :type Float%20%28single-precision%29))
  (if (>= (Math|Float|Absolute(Float) AxisValue) 0.5)
    (bind _aspc_character_menu (Utilities|Casting|CastToPC_CharacterMenu (Game|GetPlayerController 0)))
    (Variables|/Game/Blueprints/CharacterCreation/PC_CharacterMenu.PC_CharacterMenu_C|SetUsingController _aspc_character_menu true)
    (bind _asgm_character_creation (Utilities|Casting|CastToGM_CharacterCreation (Game|GetGameMode)))
    (Default|SetupUMG _asgm_character_creation true)))

(fn ConstructionScript)