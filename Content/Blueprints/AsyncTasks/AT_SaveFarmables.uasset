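; Async task that saves the world's farmable items to the "AllFarmables" save slot.
; Execute filters Farmables through ShouldSaveFarmable, which skips non-farmable items and, once two are collected, duplicate transforms.
; It gathers transforms, classes, drop indices and custom mesh data into parallel arrays, copies them into SaveGame and writes the slot, printing debug progress around the write.
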(event EventExecute
  (bind _farmableitemclasses (Variables|Default|GetfarmableItemClasses))
  (bind _savegame (Variables|Default|GetSaveGame))
  (for _array_element (Variables|Default|GetFarmables)
    (Utilities|ShouldSaveFarmable _array_element
      (:true
        (Utilities|Array|Add (Variables|Default|GetfarmableItemTransforms) (Transformation|GetActorTransform _array_element))
        (Utilities|Array|Add (Variables|Default|GetfarmableItemClasses) (Utilities|GetClass _array_element))
        (Utilities|Array|Add (Variables|Default|GetfarmableItemDropIndex) (Utilities|Struct|BreakS_ItemData_Rename2 (Variables|/Game/Blueprints/A_Item.A_Item_C|GetItemData2 _array_element)))
        (Utilities|Array|Add (Variables|Default|GetfarmableItemFarmableDropIndex) (Variables|/Game/Blueprints/A_Item.A_Item_C|GetFarmableDropIndex _array_element))
        (Utilities|Array|Add (Variables|Default|GetfarmableItemCustomMesh) (Variables|/Game/Blueprints/A_Item.A_Item_C|GetCustomMesh01 _array_element))
        (Utilities|Array|Add (Variables|Default|GetfarmableItemHasCustomMesh) (Variables|/Game/Blueprints/A_Item.A_Item_C|GetCustomMesh _array_element)))))
  (Variables|/Game/Blueprints/SG_Farmables.SG_Farmables_C|SetTransfrom _savegame (Variables|Default|GetfarmableItemTransforms))
  (Variables|/Game/Blueprints/SG_Farmables.SG_Farmables_C|SetitemClass _savegame _farmableitemclasses)
  (Variables|/Game/Blueprints/SG_Farmables.SG_Farmables_C|SetfarmableIndex _savegame (Variables|Default|GetfarmableItemDropIndex))
  (Variables|/Game/Blueprints/SG_Farmables.SG_Farmables_C|SetfarmableDropIndex _savegame (Variables|Default|GetfarmableItemFarmableDropIndex))
  (Variables|/Game/Blueprints/SG_Farmables.SG_Farmables_C|SetcustomMesh _savegame (Variables|Default|GetfarmableItemCustomMesh))
  (Variables|/Game/Blueprints/SG_Farmables.SG_Farmables_C|SethasCustomMesh _savegame (Variables|Default|GetfarmableItemHasCustomMesh))
  (Development|PrintString 0 "Start Writing")
  (SaveGame|SaveGametoSlot _savegame "AllFarmables")
  (Development|PrintString 0 "Finish Writing")
  (Development|PrintString 0 (Utilities|String|Append "DONE SAVING " (Utilities|String|ToString(Integer) (Utilities|Array|Length _farmableitemclasses)) " FARMABLES")))