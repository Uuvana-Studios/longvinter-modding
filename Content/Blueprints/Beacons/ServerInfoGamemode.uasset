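; ServerInfoGamemode is a demonstration game mode for broadcasting server info through an online beacon.
; A toggle event starts or stops hosting ServerInfoBeacon through the Online Beacon Subsystem, depending on whether it is already hosting.
; A separate demo-only event picks random placeholder values for the Gamemode and Map variables from hard-coded lists.
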(event Custom|Toggle%20Server%20Info%20Broadcast
  (bind _returnvalue (Subsystems|GetOnlineBeaconSubsystem))
  ;[1 1 1] Toggle Beacon Host.
  (if (Class|OnlineBeaconSubsystem|IsHostingBeacon _returnvalue "/BlueprintableOnlineBeacons/Examples/ServerInfoBeacon.ServerInfoBeacon_C")
    (Class|OnlineBeaconSubsystem|StopHostingBeacon _returnvalue "/BlueprintableOnlineBeacons/Examples/ServerInfoBeacon.ServerInfoBeacon_C")
    (else
      (Class|OnlineBeaconSubsystem|StartHostingBeacon _returnvalue "/BlueprintableOnlineBeacons/Examples/ServerInfoBeacon.ServerInfoBeacon_C"))))

(event Custom|Randomize%20Gamemode%20and%20Map
  (bind _array (Utilities|Array|MakeArray "TheRoom" "TheTemple" "TheUndefinedLocation"))
  (bind _array_2 (Utilities|Array|MakeArray "CaptureTheFlag" "Deathmatch" "BattleRoyale"))
  ;[1 1 1] Randomize a Gamemode and Map Name (For Demonstration Purposes Only).
  ;;[1 1 1] Randomize a Gamemode.
  (Variables|Default|SetGamemode (Utilities|Array|Get(acopy) _array_2 (Math|Random|RandomInteger (Utilities|Array|Length _array_2))))
  ;;[1 1 1] Randomize a Map.
  (Variables|Default|SetMap (Utilities|Array|Get(acopy) _array (Math|Random|RandomInteger (Utilities|Array|Length _array)))))

(fn ConstructionScript)