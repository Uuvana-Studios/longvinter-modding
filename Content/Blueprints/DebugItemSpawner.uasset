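; Debug actor that spawns A_Item pickups at its own location when play begins.
; A SpawnSpecificItem flag chooses between repeatedly spawning one configured item ID and spawning every ID from 1 to ItemCount.
; Each path runs once, fetching item data by ID and passing it to the new actor with a pickup sound.
; In the all-items path, spawn positions step along world X after each block of 21 IDs.
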(event Custom|SpawnOneItem
  (bind _defaultsceneroot (Variables|Default|GetDefaultSceneRoot))
  (bind _returnvalue (Transformation|GetWorldTransform _defaultsceneroot))
  (Utilities|FlowControl|DoOnce false
    (:Completed
      (for _index (range 0 (Variables|Default|GethowManyToSpawn))
        (bind _itemdata (CallFunction|GetItemwithID (Variables|Default|GetspecificItemIndex)))
        (Game|SpawnActorfromClass "/Game/Blueprints/A_Item.A_Item_C" (Math|Transform|MakeTransform (+ (.location _returnvalue) (Math|Vector|MakeVector (* (/ (stale Custom|Spawn%20Items%20Server _index) 21) 2e+02) 0.0 0.0)) (.rotation _returnvalue) (.scale _returnvalue)) "AdjustIfPossibleButAlwaysSpawn" 0 _itemdata false false 1.0 false 0 "/Game/Audio/Pickup.Pickup" false 25 false false false 140 false 0 0 0)))))

(event Custom|Spawn%20Items%20Server
  (bind _defaultsceneroot (Variables|Default|GetDefaultSceneRoot))
  (bind _returnvalue (Transformation|GetWorldTransform _defaultsceneroot))
  (Utilities|FlowControl|DoOnce false
    (:Completed
      (for _index (range 1 (Variables|Default|GetitemCount))
        (bind _itemdata (CallFunction|GetItemwithID _index))
        (Game|SpawnActorfromClass "/Game/Blueprints/A_Item.A_Item_C" (Math|Transform|MakeTransform (+ (.location _returnvalue) (Math|Vector|MakeVector (* (/ _index 21) 2e+02) 0.0 0.0)) (.rotation _returnvalue) (.scale _returnvalue)) "AdjustIfPossibleButAlwaysSpawn" 0 _itemdata false false 1.0 false 0 "/Game/Audio/Pickup.Pickup" false 25 false false false 140 false 0 0 0)))))

(event EventBeginPlay
  (if (Variables|Default|GetSpawnSpecificItem)
    (CallFunction|SpawnOneItem)
    (else
      (CallFunction|SpawnItemsServer))))

(event Collision|EventActorBeginOverlap
  (params (OtherActor :type Actor%20Object%20Reference)))

(event EventTick
  (params (DeltaSeconds :type Float%20%28single-precision%29)))

(fn ConstructionScript)