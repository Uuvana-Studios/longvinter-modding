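; Placeable container that turns into a chest actor once a player places it.
; On the server, Placed resolves A_Chest through the UGC registry's class overrides and spawns it at the placeable mesh's transform, passing the player's Steam ID.
; After a short delay the placeable destroys itself, then calls FlushNetDormancy.
; The right-click and drop-item-on-destruction events are empty.
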(event EventRightClicked
  (params (Player :type Third%20Person%20Character%20Object%20Reference) (SteamId :type String)))

(event EventDropItemonDestruction)

(event EventPlaced
  (params (SteamID :type String))
  (Networking|SwitchHasAuthority
    (:Authority
      (bind _asa_chest (Utilities|Casting|CastToA_ChestClass (Class|UGCRegistry|GetOverrideforActorClass (Class|UGCBlueprintLibrary|GetUGCRegistry) "/Game/Blueprints/A_Chest/A_Chest.A_Chest_C")))
      (Game|SpawnActorfromClass _asa_chest (Transformation|GetWorldTransform (Variables|Default|GetSM_Placeable)) "AlwaysSpawn" 0 false 0 24 "Container" false "" 0 false 0 0 75.0 1 "NewEnumerator0" 0 5e+01 0 SteamID 6 6e+02 0)
      (Utilities|FlowControl|Delay 0.2)
      (Actor|DestroyActor)
      (Networking|FlushNetDormancy))))

(fn ConstructionScript
  (|CallParentFunction))