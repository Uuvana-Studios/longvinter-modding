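; Async task that saves Longvinter player data to save slots.
; Execute snapshots each controlled player into the Gamemode's PlayerSaves map by Steam ID, then writes the ID list to "AllPlayers" and every map entry to its own slot.
; Snapshots clear dead players' inventory, gear and respawn point, and store boat travelers at their travel point or an outpost spawn.
; A vendor struct builder is defined but not called here.
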(event EventExecute
  (bind _savegamedata (Variables|Default|GetSaveGameData))
  (bind _savegame (Variables|Default|GetSaveGame))
  (bind _gamemode (Variables|Default|GetGamemode))
  (bind _playersaves (Variables|/Game/Blueprints/Server/GM_Longvinter.GM_Longvinter_C|GetplayerSaves _gamemode))
  (for _array_element (Variables|Default|GetPlayers)
    (bind _aspc_longvinter (Utilities|Casting|CastToPC_Longvinter (Pawn|GetController _array_element)))
    (bind (_steamid _stuct_playerdata) (CallFunction|CreateStructfromTCP _array_element _aspc_longvinter))
    (Utilities|Map|Add _playersaves _steamid _stuct_playerdata))
  (bind _output_get (Variables|/Game/Blueprints/SG_PlayerList.SG_PlayerList_C|SetPlayers _savegame (Variables|/Game/Blueprints/Server/GM_Longvinter.GM_Longvinter_C|GetPlayersIDs _gamemode)))
  (Development|PrintString 0 "Start Writing")
  (SaveGame|SaveGametoSlot _savegame "AllPlayers")
  (bind _keys (Utilities|Map|Keys _playersaves))
  (for _array_element_2 _keys
    (Variables|/Game/Blueprints/SG_PlayerData.SG_PlayerData_C|SetData _savegamedata (.Value (Utilities|Map|Find _playersaves _array_element_2)))
    (SaveGame|SaveGametoSlot _savegamedata _array_element_2))
  (Development|PrintString 0 "Finish Writing")
  (Development|PrintString 0 (Utilities|String|Append "DONE SAVING " (Utilities|String|ToString(Integer) (Utilities|Array|Length _output_get)) " PLAYERS")))

(fn MakeVendorStuct
  (params (vendor :type A%20Vendor%20Player%20Placed%20Object%20Reference))
  (bind _solditems (LocalVariables|GetSoldItems))
  (bind _itemstock (LocalVariables|GetItemStock))
  (bind _prices (LocalVariables|GetPrices))
  (bind _boughtitems (LocalVariables|GetBoughtItems))
  (for _array_element (Variables|/Game/Blueprints/Vendor/A_Vendor.A_Vendor_C|GetVendorCatalogue vendor)
    (Utilities|Array|Add _solditems (.VendorItem (Utilities|Struct|BreakS_VendorListing _array_element)))
    (Utilities|Array|Add _itemstock (.remainingStock (Utilities|Struct|BreakS_VendorListing _array_element)))
    (Utilities|Array|Add _prices (.priceMultiplier (Utilities|Struct|BreakS_VendorListing _array_element)))
    (Utilities|Array|Add _boughtitems (.PlayerItem (Utilities|Struct|BreakS_VendorListing _array_element))))
  (return (Utilities|Struct|MakeStuct_PlayerVendors (Transformation|GetActorTransform vendor) (Variables|/Game/Blueprints/Vendor/A_Vendor_PlayerPlaced.A_Vendor_PlayerPlaced_C|GetOwnerId vendor) (Variables|/Game/Blueprints/Vendor/A_Vendor_PlayerPlaced.A_Vendor_PlayerPlaced_C|GetstoredMoney vendor) _solditems _itemstock _prices (Variables|/Game/Blueprints/Vendor/A_Vendor.A_Vendor_C|GetVendor%20Name vendor) (Variables|/Game/Blueprints/Vendor/A_Vendor.A_Vendor_C|GetVendorDescription vendor) (Variables|/Game/Blueprints/Vendor/A_Vendor.A_Vendor_C|GetVendorWorldColor vendor) _boughtitems (Variables|/Game/Blueprints/Vendor/A_Vendor_PlayerPlaced.A_Vendor_PlayerPlaced_C|GetStoredItems vendor) (Utilities|GetClass vendor))))

(fn CreateStructfromTCP
  (params (thirdPersonCharacter :type Third%20Person%20Character%20Object%20Reference) (PlayerController :type PC%20Longvinter%20Object%20Reference))
  (bind _travelpoint (Variables|/Game/ThirdPersonCPP/Blueprints/ThirdPersonCharacter.ThirdPersonCharacter_C|GetTravelPoint thirdPersonCharacter))
  (bind _asps_longvinter (Utilities|Casting|CastToPS_Longvinter (Variables|/Script/Engine.Controller|GetPlayerState PlayerController)))
  (if (Variables|/Game/Blueprints/PC_Longvinter.PC_Longvinter_C|GetIsPlayerDead PlayerController)
    (Utilities|Array|Clear (Variables|/Game/Blueprints/PS_Longvinter.PS_Longvinter_C|GetPlayerInv _asps_longvinter))
    (Utilities|Array|Clear (Variables|/Game/Blueprints/PS_Longvinter.PS_Longvinter_C|GetPlayerGear _asps_longvinter))
    (Variables|/Game/Blueprints/PC_Longvinter.PC_Longvinter_C|SetRespawnLocation PlayerController "0, 0, 0"))
  (if (Variables|/Game/ThirdPersonCPP/Blueprints/ThirdPersonCharacter.ThirdPersonCharacter_C|GetUsingBoatTravel thirdPersonCharacter)
    (bind (_transform _outpostindex) (CallFunction|GetRandomSpawnLocation (Class|AdvancedSessionsLibrary|UniqueNetIdtoString (Class|AdvancedSessionsLibrary|GetUniqueNetID PlayerController))))
    (LocalVariables|SetPlayerLocation (select (Utilities|IsValid _travelpoint) (+ (Transformation|GetActorLocation _travelpoint) "0, 0,50.000000") (.location _transform)))
    (else
      (LocalVariables|SetPlayerLocation (Transformation|GetActorLocation thirdPersonCharacter))))
  (return (Class|AdvancedSessionsLibrary|UniqueNetIdtoString (Class|AdvancedSessionsLibrary|GetUniqueNetID PlayerController)) (Utilities|Struct|MakeStuct_PlayerData1 (LocalVariables|GetPlayerLocation) (Variables|/Game/Blueprints/PS_Longvinter.PS_Longvinter_C|GetEnergy _asps_longvinter) (Variables|/Game/Blueprints/PS_Longvinter.PS_Longvinter_C|GetCurrencyAmount _asps_longvinter) (Variables|/Game/Blueprints/PS_Longvinter.PS_Longvinter_C|GetPlayerScore _asps_longvinter) (Variables|/Game/Blueprints/PS_Longvinter.PS_Longvinter_C|GetPlayerInv _asps_longvinter) (Variables|/Game/ThirdPersonCPP/Blueprints/ThirdPersonCharacter.ThirdPersonCharacter_C|GetHasHome thirdPersonCharacter) (Variables|/Game/Blueprints/PS_Longvinter.PS_Longvinter_C|GetPlayerGear _asps_longvinter) (Variables|/Game/Blueprints/PS_Longvinter.PS_Longvinter_C|GetSavedPlayerScore _asps_longvinter) (Variables|/Game/ThirdPersonCPP/Blueprints/ThirdPersonCharacter.ThirdPersonCharacter_C|GetCurrentlyWearing thirdPersonCharacter) (Variables|/Game/Blueprints/PC_Longvinter.PC_Longvinter_C|GetRespawnLocation PlayerController) (Variables|/Game/ThirdPersonCPP/Blueprints/ThirdPersonCharacter.ThirdPersonCharacter_C|GetAmmo thirdPersonCharacter) (Variables|/Game/Blueprints/PS_Longvinter.PS_Longvinter_C|GetFoundItems _asps_longvinter) (Variables|/Game/ThirdPersonCPP/Blueprints/BuffComponent.BuffComponent_C|GetbuffsArray (Variables|/Game/ThirdPersonCPP/Blueprints/ThirdPersonCharacter.ThirdPersonCharacter_C|GetBuffComponent thirdPersonCharacter)) (Variables|/Game/Blueprints/PC_Longvinter.PC_Longvinter_C|GetlastVisitedHouseID PlayerController) (Variables|/Game/Blueprints/PC_Longvinter.PC_Longvinter_C|GetplayerTeamId PlayerController) (Variables|/Game/Blueprints/PC_Longvinter.PC_Longvinter_C|GetlastOwnHomeId PlayerController) (Variables|/Game/Blueprints/PC_Longvinter.PC_Longvinter_C|GetQuests PlayerController) (Variables|/Game/Blueprints/PC_Longvinter.PC_Longvinter_C|GetCompletedQuests PlayerController) 0 (Variables|/Game/ThirdPersonCPP/Blueprints/ThirdPersonCharacter.ThirdPersonCharacter_C|GetArrows thirdPersonCharacter) (Variables|/Game/Blueprints/PC_Longvinter.PC_Longvinter_C|GetReceivedAdminItems PlayerController) (Variables|/Game/Blueprints/PS_Longvinter.PS_Longvinter_C|GethouseCap _asps_longvinter) (Variables|/Game/Blueprints/PS_Longvinter.PS_Longvinter_C|GetglobalInventory _asps_longvinter) (Variables|/Game/Blueprints/PS_Longvinter.PS_Longvinter_C|GetShipments _asps_longvinter) (Variables|/Game/Blueprints/PS_Longvinter.PS_Longvinter_C|GetMount _asps_longvinter) (Variables|/Game/Blueprints/PS_Longvinter.PS_Longvinter_C|GetItemCompetitionSaveValues _asps_longvinter) (PlayerState|GetPlayerName _asps_longvinter) (Variables|/Game/Blueprints/PS_Longvinter.PS_Longvinter_C|GetPersistentScore _asps_longvinter) _outpostindex)))

(fn GetRandomSpawnLocation
  (params (SteamID :type String))
  (bind _gamemode (Variables|Default|GetGamemode))
  (bind _playersaves (Variables|/Game/Blueprints/Server/GM_Longvinter.GM_Longvinter_C|GetplayerSaves _gamemode))
  (bind (_value _returnvalue) (Utilities|Map|Find _playersaves SteamID))
  (bind _asgs_longvinter (Utilities|Casting|CastToGS_Longvinter (Variables|Default|GetGameState)))
  (bind _output_get (LocalVariables|SetOutpostInteger (select _returnvalue (Utilities|Struct|BreakStuct_PlayerData1 _value) (Math|Random|RandomIntegerinRange 1 5))))
  (for _array_element (Variables|/Game/Blueprints/Server/GS_Longvinter.GS_Longvinter_C|GetSpawnPoints _asgs_longvinter)
    (if (== (Variables|/Game/Blueprints/BoatTravel/A_TravelPoint.A_TravelPoint_C|GetStarterPointInteger _array_element) (LocalVariables|GetOutpostInteger))
      (bind _output_get_2 (LocalVariables|SetSpawnLoc (Transformation|GetActorTransform _array_element)))
      (return _output_get_2 _output_get))))