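; Player controller for the character style editor menu, handling the preview character and Steam item data.
; BeginPlay shows a loading screen, spawns the preview character at a random CameraPoint scene and possesses a separate camera pawn.
; It also requests Steam prices, inventory and item definitions, retrying failed price and inventory calls, then signals updates.
; Events swap clothing and skin through dynamic material instances, set music volume and confirm purchases.
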(event Custom|ChangeClothingMaterial
  (params (Parent :type Material%20Interface%20Object%20Reference) (SkinColor :type Linear%20Color%20Structure))
  (bind _charactereditorpawn (Variables|Default|GetCharacterEditorPawn))
  (bind _mesh (Variables|/Script/Engine.Character|GetMesh _charactereditorpawn))
  (bind _returnvalue (Rendering|Material|CreateDynamicMaterialInstance Parent "None" "None" :!class /Script/Engine.KismetMaterialLibrary))
  (bind _output_get (Variables|Default|SetchracterMaterial _returnvalue))
  (Rendering|Material|SetMaterial _mesh 0 _returnvalue)
  (Rendering|Material|SetMaterial _mesh 1 _returnvalue)
  (Rendering|Material|SetVectorParameterValue _returnvalue "SkinColor" SkinColor :!class /Script/Engine.MaterialInstanceDynamic)
  (Rendering|Material|SetScalarParameterValue _output_get "DisableHat" 0.0 :!class /Script/Engine.MaterialInstanceDynamic))

(event Custom|GetAllItemDefsCallback
  (bind _itemdefs (Class|Inventory|GetItemDefinitionIDs))
  (Variables|Default|SetAllSteamItems _itemdefs)
  (Default|CallSteamItemsUpdated))

(event Custom|LoadAllSteamItems
  (EventDispatchers|AssignSteamInventoryDefinitionUpdate (Subsystems|GetInventory) (delegate Custom|GetAllItemDefsCallback))
  (Class|Inventory|LoadItemDefinitions))

(event Custom|ItemPurchaseMessage
  (bind _returnvalue (UserInterface|CreateWidget "/Game/Widgets/UMG_WarningMessage.UMG_WarningMessage_C" 0 "Purchase Completed" "Item has now been added to your account" "Continue" false "Cancel" "/Game/Widgets/Icons/UI/checkmark.checkmark" "(R=0.003922,G=0.254902,B=0.129412,A=1.000000)"))
  (UserInterface|Viewport|AddtoViewport _returnvalue 0)
  (Default|CallItemPurchased))

(event Custom|UpdateSteamInventory
  (bind (_handle _returnvalue) (Class|Inventory|GetAllItems :!label _label))
  (if _returnvalue
    (Variables|Default|SetHandle _handle)
    (bind (_items _returnvalue_2) (Class|Inventory|GetResultItems _handle :!label _label_2))
    (if _returnvalue_2
      (Variables|Default|SetSteamInventory _items)
      (Default|CallInventoryUpdated)
      (else
        (Utilities|FlowControl|Delay 0.2)
        (goto _label_2)))
    (else
      (Utilities|FlowControl|Delay 0.2)
      (goto _label))))

(event Custom|ChangeSkinColor
  (params (Color :type Linear%20Color%20Structure))
  (bind _charactereditorpawn (Variables|Default|GetCharacterEditorPawn))
  (bind _returnvalue (Rendering|Material|CreateDynamicMaterialInstance "/Game/Character/Materials/MI_Character_01.MI_Character_01" "None" "None" :!class /Script/Engine.KismetMaterialLibrary))
  (Rendering|Material|SetMaterial (Variables|/Game/Blueprints/CharacterCreation/A_CharacterEditorPawn.A_CharacterEditorPawn_C|GetEars _charactereditorpawn) 0 _returnvalue)
  (bind _returnvalue_2 (Rendering|Material|CreateDynamicMaterialInstance "/Game/Character/LV_Character_UES/LV_Character02/LV_Character01_head_02/M_Character01_Skin.M_Character01_Skin" "None" "None" :!class /Script/Engine.KismetMaterialLibrary))
  (Rendering|Material|SetMaterial (Variables|/Game/Blueprints/CharacterCreation/A_CharacterEditorPawn.A_CharacterEditorPawn_C|GetHead _charactereditorpawn) 0 _returnvalue_2)
  (Rendering|Material|SetVectorParameterValue _returnvalue_2 "SkinColor" Color :!class /Script/Engine.MaterialInstanceDynamic))

(event Custom|SetGi_advancedMusicVolume
  (params (Volume :type Float%20%28single-precision%29))
  (bind _asgi_advanced_sessions (Utilities|Casting|CastToGI_AdvancedSessions (Game|GetGameInstance)))
  (Audio|Components|Audio|SetVolumeMultiplier (Variables|/Game/Blueprints/Server/GI_AdvancedSessions.GI_AdvancedSessions_C|GetMusic _asgi_advanced_sessions) Volume :!class /Script/Engine.AudioComponent))

(event EventBeginPlay
  (Utilities|FlowControl|Sequence
    (:then_0
      (CallFunction|SetGiAdvancedMusicVolume 0.0)
      (bind _returnvalue (UserInterface|CreateWidget "/Game/Widgets/MainMenu/UMG_LoadingScreen.UMG_LoadingScreen_C" self "Style editor"))
      (Utilities|IsValid _returnvalue :!label _label
        (:Is%20Valid
          (bind _output_get (Variables|Default|SetLoading%20Screen _returnvalue))
          (UserInterface|Viewport|AddtoViewport _output_get 0)
          (Utilities|FlowControl|Sequence
            (:then_0
              (Input|SetInputModeUIOnly self 0 "DoNotLock")
              (Variables|Default|SetbShowMouseCursor true))
            (:then_1
              (bind _outactors (Actor|GetAllActorswithTag "CameraPoint"))
              (bind _output_get_2 (Variables|Default|SetcameraLocation (Utilities|Array|Get(acopy) _outactors (Math|Random|RandomIntegerinRange 0 (- (Utilities|Array|Length _outactors) 1)))))
              (bind _asa_character_edit_scene (Utilities|Casting|CastToA_CharacterEditScene _output_get_2))
              (bind _returnvalue_2 (Game|SpawnActorfromClass "/Game/Blueprints/CharacterCreation/A_CharacterEditorPawn.A_CharacterEditorPawn_C" (Transformation|GetActorTransform _output_get_2) "AlwaysSpawn" 0 "/Game/Blueprints/CharacterCreation/hats/A_Hat20.A_Hat20_C" false 0))
              (Variables|Default|SetCharacterEditorPawn _returnvalue_2)
              (bind _returnvalue_3 (Game|SpawnActorfromClass "/Game/Blueprints/CharacterCreation/Pawn_CharacterEditor.Pawn_CharacterEditor_C" (Transformation|GetWorldTransform (Variables|/Game/Blueprints/CharacterCreation/UiRenders/A_CharacterEditScene.A_CharacterEditScene_C|GetCameraLocation _asa_character_edit_scene)) "AlwaysSpawn" 0 0))
              (Pawn|Possess _returnvalue_3)
              (Widget|RemovefromParent (Variables|Default|GetLoading%20Screen)))
            (:then_3
              (bind _returnvalue_4 (Rendering|Material|CreateDynamicMaterialInstance "/Game/Character/Materials/MI_Character_01.MI_Character_01" "None" "None" :!class /Script/Engine.KismetMaterialLibrary))
              (bind _output_get_3 (Variables|Default|SetchracterMaterial _returnvalue_4))
              (Rendering|Material|SetMaterial (Variables|/Script/Engine.Character|GetMesh (Variables|Default|GetCharacterEditorPawn)) 0 _output_get_3)
              (Rendering|Material|SetMaterial (Variables|/Script/Engine.Character|GetMesh (Variables|Default|GetCharacterEditorPawn)) 1 _output_get_3)
              (Rendering|Material|SetVectorParameterValue _output_get_3 "SkinColor" "(R=0.863157,G=0.412543,B=0.262251,A=1.000000)" :!class /Script/Engine.MaterialInstanceDynamic)
              (Rendering|Material|SetScalarParameterValue _output_get_3 "DisableHat" 0.0 :!class /Script/Engine.MaterialInstanceDynamic))
            (:then_4
              (bind _returnvalue_5 (Rendering|Material|CreateDynamicMaterialInstance "/Game/Character/Materials/MI_Face01.MI_Face01" "None" "None" :!class /Script/Engine.KismetMaterialLibrary))
              (bind _output_get_4 (Variables|Default|SetfaceMaterial _returnvalue_5))
              (Rendering|Material|SetMaterial (Variables|/Game/Blueprints/CharacterCreation/A_CharacterEditorPawn.A_CharacterEditorPawn_C|GetHead (Variables|Default|GetCharacterEditorPawn)) 1 _output_get_4))))
        (:Is%20Not%20Valid
          (Utilities|FlowControl|Delay 0.1)
          (goto _label))))
    (:then_1
      (bind _returnvalue_6 (Class|UserStats|GetAchievement "START_GAME_1"))
      (if _returnvalue_6
        (bind _bwassuccessful (|RequestPricesAsync 1e+01 :!label _label_2)
          (:OnCallback
            (if (not _bwassuccessful)
              (goto _label_2))))))
    (:then_2
      (CallFunction|UpdateSteamInventory))
    (:then_3
      (CallFunction|LoadAllSteamItems))))

(event EventTick
  (params (DeltaSeconds :type Float%20%28single-precision%29)))

(fn ConstructionScript)