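; Async task that settles the global shipment in Longvinter, crediting payouts and clearing contributions in players' saved shipment data.
; For flagged players, all four shipment slots completed pays a boosted item price per contribution, otherwise only completed slots pay at a reduced rate.
; It loads each save slot by player ID, adds the payout, saves, then mirrors the result to matching player states and the PlayerSaves map.
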(event EventExecute
  (bind _returnvalue (Math|Float|MakeLiteralFloat 1.45))
  (bind _items (Variables|Default|GetItems))
  (bind _playersaves (Variables|Default|GetplayerSaves))
  (bind _globalshipment (Variables|Default|GetGlobalShipment))
  (bind (_maximum _currentprogress _amountleft _itemindex _completed) (Utilities|GetShipmentValues _globalshipment 9 "NewEnumerator1"))
  (bind (_maximum_2 _currentprogress_2 _amountleft_2 _itemindex_2 _completed_2) (Utilities|GetShipmentValues _globalshipment 6 "NewEnumerator1"))
  (bind (_maximum_3 _currentprogress_3 _amountleft_3 _itemindex_3 _completed_3) (Utilities|GetShipmentValues _globalshipment 0 "NewEnumerator1"))
  (bind (_maximum_4 _currentprogress_4 _amountleft_4 _itemindex_4 _completed_4) (Utilities|GetShipmentValues _globalshipment 3 "NewEnumerator1"))
  (for _array_element (Variables|Default|GetPlayerIDs)
    (bind _returnvalue_2 (SaveGame|LoadGamefromSlot _array_element))
    (bind _assg_player_data (Utilities|Casting|CastToSG_PlayerData _returnvalue_2))
    (bind _output_get (Variables|Default|SetSG_PlayerData _assg_player_data))
    (bind _output_get_2 (Variables|Default|SetPersonalShipment (.Shipments (Utilities|Struct|BreakStuct_PlayerData1 (Variables|/Game/Blueprints/SG_PlayerData.SG_PlayerData_C|GetData _output_get)))))
    (if (== (Utilities|Array|Get(acopy) _output_get_2) 1)
      (if (Math|Boolean|ANDBoolean _completed_3 _completed_4 _completed_2 _completed)
        (Utilities|Array|SetArrayElem (Variables|Default|GetPersonalShipment) 10 (Math|Float|Round (+ (* (Utilities|Array|Get(acopy) (Variables|Default|GetPersonalShipment) 6) (* (.defaultPrice (Utilities|Struct|BreakS_ItemData_Rename2 (Utilities|Array|Get(acopy) _items _itemindex_3))) _returnvalue)) (* (Utilities|Array|Get(acopy) (Variables|Default|GetPersonalShipment) 7) (* (.defaultPrice (Utilities|Struct|BreakS_ItemData_Rename2 (Utilities|Array|Get(acopy) _items _itemindex_4))) _returnvalue)) (* (Utilities|Array|Get(acopy) (Variables|Default|GetPersonalShipment) 8) (* (.defaultPrice (Utilities|Struct|BreakS_ItemData_Rename2 (Utilities|Array|Get(acopy) _items _itemindex_2))) _returnvalue)) (* (Utilities|Array|Get(acopy) (Variables|Default|GetPersonalShipment) 9) (* (.defaultPrice (Utilities|Struct|BreakS_ItemData_Rename2 (Utilities|Array|Get(acopy) _items _itemindex))) _returnvalue)) (Math|Conversions|ToFloat(Integer) (Utilities|Array|Get(acopy) (Variables|Default|GetPersonalShipment) 10)))) true)
        (else
          (bind _payouttopay (CallFunction|GetPartiallyFilledGlobalShipmentPayout (Variables|Default|GetPersonalShipment)))
          (Utilities|Array|SetArrayElem (Variables|Default|GetPersonalShipment) 10 (+ _payouttopay (Utilities|Array|Get(acopy) (Variables|Default|GetPersonalShipment) 10)) true)))
      (Utilities|Array|SetArrayElem (Variables|Default|GetPersonalShipment) 6 0 true)
      (Utilities|Array|SetArrayElem (Variables|Default|GetPersonalShipment) 7 0 true)
      (Utilities|Array|SetArrayElem (Variables|Default|GetPersonalShipment) 8 0 true)
      (Utilities|Array|SetArrayElem (Variables|Default|GetPersonalShipment) 9 0 true)
      (bind _structout (Utilities|Struct|SetmembersinStuct_PlayerData1 (Variables|/Game/Blueprints/SG_PlayerData.SG_PlayerData_C|GetData _output_get) (Variables|Default|GetPersonalShipment)))
      (Variables|/Game/Blueprints/SG_PlayerData.SG_PlayerData_C|SetData (Variables|Default|GetSG_PlayerData) _structout)
      (SaveGame|SaveGametoSlot (Variables|Default|GetSG_PlayerData) _array_element)
      (bind _array_element_2 (Utilities|Array|ForEachLoopwithBreak (Variables|Default|GetPlayers) :!label _label)
        (:LoopBody
          (if (Utilities|Enum|Equal(Enum) _array_element (Class|AdvancedSessionsLibrary|UniqueNetIdtoString (Class|AdvancedSessionsLibrary|GetUniqueNetIDfromPlayerState _array_element_2)))
            (bind _asps_longvinter (Utilities|Casting|CastToPS_Longvinter _array_element_2))
            (Variables|/Game/Blueprints/PS_Longvinter.PS_Longvinter_C|SetShipments _asps_longvinter (Variables|Default|GetPersonalShipment))
            (goto _label Break)))
        (:Completed
          (if (.ReturnValue (Utilities|Map|Find _playersaves _array_element))
            (bind _structout_2 (Utilities|Struct|SetmembersinStuct_PlayerData1 (.Value (Utilities|Map|Find _playersaves _array_element)) (Variables|Default|GetPersonalShipment)))
            (Utilities|Map|Add _playersaves _array_element _structout_2)))))))

(fn GetPartiallyFilledGlobalShipmentPayout
  (params (PersonalShipments :type Array%20of%20Integers))
  (bind _globalshipment (Variables|Default|GetGlobalShipment))
  (bind _items (Variables|Default|GetItems))
  (bind _items_2 (Variables|Default|GetItems))
  (bind (_maximum _currentprogress _amountleft _itemindex _completed) (Utilities|GetShipmentValues _globalshipment 0 "NewEnumerator1"))
  (bind (_maximum_2 _currentprogress_2 _amountleft_2 _itemindex_2 _completed_2) (Utilities|GetShipmentValues _globalshipment 3 "NewEnumerator1"))
  (bind (_maximum_3 _currentprogress_3 _amountleft_3 _itemindex_3 _completed_3) (Utilities|GetShipmentValues _globalshipment 6 "NewEnumerator1"))
  (bind (_maximum_4 _currentprogress_4 _amountleft_4 _itemindex_4 _completed_4) (Utilities|GetShipmentValues _globalshipment 9 "NewEnumerator1"))
  (if _completed
    (LocalVariables|Setpayout (+ (* (Utilities|Array|Get(acopy) PersonalShipments 6) (Math|Float|Round (* (.defaultPrice (Utilities|Struct|BreakS_ItemData_Rename2 (Utilities|Array|Get(acopy) _items _itemindex))) 0.5))) (LocalVariables|Getpayout))))
  (if _completed_2
    (LocalVariables|Setpayout (+ (* (Utilities|Array|Get(acopy) PersonalShipments 7) (Math|Float|Round (* (.defaultPrice (Utilities|Struct|BreakS_ItemData_Rename2 (Utilities|Array|Get(acopy) _items _itemindex_2))) 0.5))) (LocalVariables|Getpayout))))
  (if _completed_3
    (LocalVariables|Setpayout (+ (* (Utilities|Array|Get(acopy) PersonalShipments 8) (Math|Float|Round (* (.defaultPrice (Utilities|Struct|BreakS_ItemData_Rename2 (Utilities|Array|Get(acopy) _items_2 _itemindex_3))) 0.5))) (LocalVariables|Getpayout))))
  (if _completed_4
    (LocalVariables|Setpayout (+ (* (Utilities|Array|Get(acopy) PersonalShipments 9) (Math|Float|Round (* (.defaultPrice (Utilities|Struct|BreakS_ItemData_Rename2 (Utilities|Array|Get(acopy) _items_2 _itemindex_4))) 0.5))) (LocalVariables|Getpayout))))
  (return (LocalVariables|Getpayout)))