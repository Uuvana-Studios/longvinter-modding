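; MyPingBeacon is a beacon that measures round-trip ping between a client and the server.
; On connection it stores a start time and sends ServerPing, which the server answers with ClientPong.
; ClientPong caches the elapsed milliseconds as LastPing, fires the OnPingCalculated dispatcher, then restarts the measurement after a one-second delay, creating a continuous loop.
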(event Custom|Server%20Ping
  ;[1 1 1] Received from the Client.
  ; Call Client Pong, so we can calculate the ping.
  (CallFunction|ClientPong))

(event Custom|Client%20Pong
  ;[1 1 1] Called by the Server for the Client to calculate the Ping.
  ;;[1 1 1] Set Last Ping Cache and Call Calculated Dispatcher.
  (bind _output_get (Variables|Default|SetLast%20Ping (Math|Float|Floor (Class|KismetMathLibrary|GetTotalMilliseconds (- (Math|DateTime|Now) (Variables|Default|GetPing%20Start%20Time))))))
  (Default|CallOnPingCalculated _output_get)
  ;;[1 1 1] Calculate Ping Once Again after a second.
  (Utilities|FlowControl|Delay 1.0)
  (CallFunction|CalculatePing))

(event Custom|Calculate%20Ping
  ;[1 1 1] Call this anytime you want to calculate ping.
  ; Sets the Ping Start Time and sends a Ping RPC to the Server.
  (Variables|Default|SetPing%20Start%20Time (Math|DateTime|Now))
  (CallFunction|ServerPing))

(event EventOnConnectedBlueprint
  ;[1 1 1] When Connection Success, Calculate Ping.
  (CallFunction|CalculatePing))

(fn ConstructionScript)