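; NNSaveGame is a SaveGame that saves and loads a neural-network evolution Population in a single slot.
; Save flattens species into structs of stats, neuron biases and synapses, replacing object references with neuron indices.
; Load reads the struct back and reconstructs the Population, with code to rebuild each brain's input Nodes, Neurons and Synapses.
; That species-rebuild loop has an empty hard-coded range, so as written no species are restored.
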(event Custom|Save
  (params (Population :type Population%20Object%20Reference))
  (Variables|Default|SetPopulation Population)
  (CallFunction|ProcessPopulation)
  (SaveGame|SaveGametoSlot self "SlotOne")
  (Variables|Default|SetPopulation 0))

(event Custom|Load
  (bind _returnvalue (SaveGame|LoadGamefromSlot "SlotOne"))
  (bind _asnnsave_game (Utilities|Casting|CastToNNSaveGame _returnvalue))
  (Variables|Default|SetPopulationStruct2 (Variables|NNSaveGame_C|GetPopulationStruct2 _asnnsave_game))
  (CallFunction|RestorePopulation))

(fn ProcessPopulation
  (bind _population (Variables|Default|GetPopulation))
  (for _array_element (Variables|/Game/Blueprints/NN/Population.Population_C|GetSpecies (Variables|Default|GetPopulation))
    (Utilities|Array|Clear (LocalVariables|GetNeuron%20Biases))
    (Utilities|Array|Clear (LocalVariables|GetSynapses))
    (for _array_element_2 (Variables|/Game/Blueprints/NN/Brain.Brain_C|GetNeurons (Variables|/Game/Blueprints/NN/Specie.Specie_C|GetBrain _array_element))
      (bind _asneuron (Utilities|Casting|CastToNeuron _array_element_2))
      (Utilities|Array|Add (LocalVariables|GetNeuron%20Biases) (Variables|/Game/Blueprints/NN/Neuron.Neuron_C|GetBias _asneuron))
      (for _array_element_3 (Variables|/Game/Blueprints/NN/Neuron.Neuron_C|GetSynapses _asneuron)
        (Utilities|Array|Add (LocalVariables|GetSynapses) (Utilities|Struct|MakeSynapseStruct (Utilities|Array|FindItem (Variables|/Game/Blueprints/NN/Brain.Brain_C|GetNeurons (Variables|/Game/Blueprints/NN/Specie.Specie_C|GetBrain _array_element)) (Variables|/Game/Blueprints/NN/Synapse.Synapse_C|GetSource _array_element_3)) (Utilities|Array|FindItem (Variables|/Game/Blueprints/NN/Brain.Brain_C|GetNeurons (Variables|/Game/Blueprints/NN/Specie.Specie_C|GetBrain _array_element)) (Variables|/Game/Blueprints/NN/Synapse.Synapse_C|GetTarget _array_element_3)) (Variables|/Game/Blueprints/NN/Synapse.Synapse_C|GetWeight _array_element_3)))))
    (Utilities|Array|Add (LocalVariables|GetSpecies) (Utilities|Struct|MakeSpecieStruct (Variables|/Game/Blueprints/NN/Specie.Specie_C|GetGeneration%20Born _array_element) (Variables|/Game/Blueprints/NN/Specie.Specie_C|GetNumber _array_element) (Variables|/Game/Blueprints/NN/Specie.Specie_C|GetLast%20Fitness _array_element) (Variables|/Game/Blueprints/NN/Specie.Specie_C|GetStale _array_element) (Variables|/Game/Blueprints/NN/Specie.Specie_C|GetUnderperforming%20for%20Generations _array_element) (LocalVariables|GetNeuron%20Biases) (LocalVariables|GetSynapses))))
  (Variables|Default|SetPopulationStruct2 (Utilities|Struct|MakePopulationStruct (Variables|/Game/Blueprints/NN/Population.Population_C|GetGeneration _population) (Variables|/Game/Blueprints/NN/Population.Population_C|GetNumber%20of%20species _population) (Variables|/Game/Blueprints/NN/Population.Population_C|GetNeuron%20Counts _population) (Variables|/Game/Blueprints/NN/Population.Population_C|GetFitness%20Over%20Time _population) (LocalVariables|GetSpecies) (Variables|/Game/Blueprints/NN/Population.Population_C|GetSynapse%20Mutation%20Chance _population) (Variables|/Game/Blueprints/NN/Population.Population_C|GetNeuron%20Mutation%20Chance _population) (Variables|/Game/Blueprints/NN/Population.Population_C|GetPerturb%20Chance _population) (Variables|/Game/Blueprints/NN/Population.Population_C|GetMutation%20Step _population))))

(fn RestorePopulation
  (bind _populationstruct2 (Variables|Default|GetPopulationStruct2))
  (bind _returnvalue (Game|ConstructObjectfromClass "/Game/Blueprints/NN/Population.Population_C" self (.numberofspecies _populationstruct2) (.neuroncounts _populationstruct2) (.synapsemutationchance _populationstruct2) (.neuronmutationchance _populationstruct2) (.perturbchance _populationstruct2) (.mutationstep _populationstruct2)))
  (bind _output_get (Variables|Default|SetPopulation _returnvalue))
  (Variables|/Game/Blueprints/NN/Population.Population_C|SetGeneration _output_get (.generation _populationstruct2))
  (Variables|/Game/Blueprints/NN/Population.Population_C|SetNumber%20of%20species _output_get (.numberofspecies _populationstruct2))
  (Variables|/Game/Blueprints/NN/Population.Population_C|SetFitness%20Over%20Time _output_get (.fitnessovertime _populationstruct2))
  (for _index (range 0 (- 0 1))
    (bind _returnvalue_2 (Game|ConstructObjectfromClass "/Game/Blueprints/NN/Specie.Specie_C" (Variables|Default|GetPopulation) (Variables|/Game/Blueprints/NN/Population.Population_C|GetNeuron%20Counts (Variables|Default|GetPopulation))))
    (Utilities|Array|Add (Variables|/Game/Blueprints/NN/Population.Population_C|GetSpecies (Variables|Default|GetPopulation)) _returnvalue_2)
    (Variables|/Game/Blueprints/NN/Specie.Specie_C|SetGeneration%20Born _returnvalue_2 (.generationborn (Utilities|Array|Get(acopy) (.species _populationstruct2) _index)))
    (Variables|/Game/Blueprints/NN/Specie.Specie_C|SetNumber _returnvalue_2 (.number (Utilities|Array|Get(acopy) (.species _populationstruct2) _index)))
    (Variables|/Game/Blueprints/NN/Specie.Specie_C|SetLast%20Fitness _returnvalue_2 (.lastfitness (Utilities|Array|Get(acopy) (.species _populationstruct2) _index)))
    (Variables|/Game/Blueprints/NN/Specie.Specie_C|SetStale _returnvalue_2 (.stale (Utilities|Array|Get(acopy) (.species _populationstruct2) _index)))
    (Variables|/Game/Blueprints/NN/Specie.Specie_C|SetUnderperforming%20for%20Generations _returnvalue_2 (.underperformingforgenerations (Utilities|Array|Get(acopy) (.species _populationstruct2) _index)))
    (bind _returnvalue_3 (Game|ConstructObjectfromClass "/Game/Blueprints/NN/Brain.Brain_C" _returnvalue_2 (Variables|/Game/Blueprints/NN/Population.Population_C|GetNeuron%20Counts (Variables|Default|GetPopulation))))
    (bind _output_get_2 (Variables|/Game/Blueprints/NN/Specie.Specie_C|SetBrain _returnvalue_2 _returnvalue_3))
    (for (_array_element _array_index) (Variables|/Game/Blueprints/NN/Population.Population_C|GetNeuron%20Counts (Variables|Default|GetPopulation))
      (for _index_2 (range 0 (- _array_element 1))
        (if (== _array_index 0)
          (bind _returnvalue_4 (Game|ConstructObjectfromClass "/Game/Blueprints/NN/Node.Node_C" _output_get_2))
          (Utilities|Array|Add (Variables|/Game/Blueprints/NN/Brain.Brain_C|GetNeurons _output_get_2) _returnvalue_4)
          (else
            (bind _returnvalue_5 (Game|ConstructObjectfromClass "/Game/Blueprints/NN/Neuron.Neuron_C" _output_get_2))
            (Utilities|Array|Add (Variables|/Game/Blueprints/NN/Brain.Brain_C|GetNeurons _output_get_2) _returnvalue_5)))))
    (for (_array_element_2 _array_index_2) (.neuronbiases (Utilities|Array|Get(acopy) (.species _populationstruct2) _index))
      (bind _asneuron (Utilities|Casting|CastToNeuron (Utilities|Array|Get(acopy) (Variables|/Game/Blueprints/NN/Brain.Brain_C|GetNeurons _output_get_2) (+ _array_index_2 (Utilities|Array|Get(acopy) (Variables|/Game/Blueprints/NN/Population.Population_C|GetNeuron%20Counts (Variables|Default|GetPopulation)))))))
      (Variables|/Game/Blueprints/NN/Neuron.Neuron_C|SetBias _asneuron _array_element_2))
    (for _array_element_3 (.synapses (Utilities|Array|Get(acopy) (.species _populationstruct2) _index))
      (bind _returnvalue_6 (Game|ConstructObjectfromClass "/Game/Blueprints/NN/Synapse.Synapse_C" _output_get_2))
      (Variables|/Game/Blueprints/NN/Synapse.Synapse_C|SetWeight _returnvalue_6 (.Weight (Utilities|Struct|BreakSynapseStruct _array_element_3)))
      (Variables|/Game/Blueprints/NN/Synapse.Synapse_C|SetSource _returnvalue_6 (Utilities|Array|Get(acopy) (Variables|/Game/Blueprints/NN/Brain.Brain_C|GetNeurons _output_get_2) (.SourceIndex (Utilities|Struct|BreakSynapseStruct _array_element_3))))
      (Variables|/Game/Blueprints/NN/Synapse.Synapse_C|SetTarget _returnvalue_6 (Utilities|Array|Get(acopy) (Variables|/Game/Blueprints/NN/Brain.Brain_C|GetNeurons _output_get_2) (.TargetIndex (Utilities|Struct|BreakSynapseStruct _array_element_3))))
      (bind _asneuron_2 (Utilities|Casting|CastToNeuron (Utilities|Array|Get(acopy) (Variables|/Game/Blueprints/NN/Brain.Brain_C|GetNeurons _output_get_2) (.TargetIndex (Utilities|Struct|BreakSynapseStruct _array_element_3)))))
      (Utilities|Array|Add (Variables|/Game/Blueprints/NN/Neuron.Neuron_C|GetSynapses _asneuron_2) _returnvalue_6))))