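; AT_SaveVendors is a task that saves player vendors to the AllPlayerVendors save slot.
; Execute converts each vendor into a struct through MakeVendorStuct, capturing transform, owner, money, catalogue, stored items, appearance and class.
; Catalogue entries are flattened into parallel arrays of items, stock and price multipliers.
; The struct array is written with SaveGameToSlot, with debug prints around the write; a transform duplicate-check helper is unused.
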(event EventExecute
  (bind _vendorstructs (Variables|Default|GetVendorStructs))
  (bind _savegame (Variables|Default|GetSaveGame))
  (for _array_element (Variables|Default|GetVendors)
    (bind _stuct_playervendors (CallFunction|MakeVendorStuct _array_element))
    (Utilities|Array|Add (Variables|Default|GetVendorStructs) _stuct_playervendors))
  (Variables|/Game/Blueprints/Server/SG_PlayerVendors.SG_PlayerVendors_C|Setvendors _savegame _vendorstructs)
  (Development|PrintString 0 "Start Writing")
  (SaveGame|SaveGametoSlot _savegame "AllPlayerVendors")
  (Development|PrintString 0 "Finish Writing")
  (Development|PrintString 0 (Utilities|String|Append "DONE SAVING " (Utilities|String|ToString(Integer) (Utilities|Array|Length _vendorstructs)) " PLAYER VENDORS")))

(fn MakeVendorStuct
  (params (vendor :type A%20Vendor%20Player%20Placed%20Object%20Reference))
  (bind _solditems (LocalVariables|GetSoldItems))
  (bind _itemstock (LocalVariables|GetItemStock))
  (bind _prices (LocalVariables|GetPrices))
  (bind _boughtitems (LocalVariables|GetBoughtItems))
  (for _array_element (Variables|/Game/Blueprints/Vendor/A_Vendor.A_Vendor_C|GetVendorCatalogue vendor)
    (Utilities|Array|Add _solditems (.VendorItem (Utilities|Struct|BreakS_VendorListing _array_element)))
    (Utilities|Array|Add _itemstock (.remainingStock (Utilities|Struct|BreakS_VendorListing _array_element)))
    (Utilities|Array|Add _prices (.priceMultiplier (Utilities|Struct|BreakS_VendorListing _array_element)))
    (Utilities|Array|Add _boughtitems (.PlayerItem (Utilities|Struct|BreakS_VendorListing _array_element))))
  (return (Utilities|Struct|MakeStuct_PlayerVendors (Transformation|GetActorTransform vendor) (Variables|/Game/Blueprints/Vendor/A_Vendor_PlayerPlaced.A_Vendor_PlayerPlaced_C|GetOwnerId vendor) (Variables|/Game/Blueprints/Vendor/A_Vendor_PlayerPlaced.A_Vendor_PlayerPlaced_C|GetstoredMoney vendor) _solditems _itemstock _prices (Variables|/Game/Blueprints/Vendor/A_Vendor.A_Vendor_C|GetVendor%20Name vendor) (Variables|/Game/Blueprints/Vendor/A_Vendor.A_Vendor_C|GetVendorDescription vendor) (Variables|/Game/Blueprints/Vendor/A_Vendor.A_Vendor_C|GetVendorWorldColor vendor) _boughtitems (Variables|/Game/Blueprints/Vendor/A_Vendor_PlayerPlaced.A_Vendor_PlayerPlaced_C|GetStoredItems vendor) (Utilities|GetClass vendor))))