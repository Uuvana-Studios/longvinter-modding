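; Large planting box placeable that makes the plants within it drop their items when the box is right-clicked.
; On RightClicked it runs a box overlap query over the PlantArea component's location and extent, then passes each hit actor to DropPlant.
; DropPlant calls DropItemOnDestruction on A_Placeable_Plant actors and ignores others, after which the parent RightClicked handler runs.
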(event EventBeginPlay
  (|CallParentFunction))

(event Collision|EventActorBeginOverlap
  (params (OtherActor :type Actor%20Object%20Reference))
  (|CallParentFunction OtherActor) ; This node is disabled and will not be called.\nDrag off pins to build functionality.
)

(event EventTick
  (params (DeltaSeconds :type Float%20%28single-precision%29))
  (|CallParentFunction DeltaSeconds) ; This node is disabled and will not be called.\nDrag off pins to build functionality.
)

(event EventRightClicked
  (params (Player :type Third%20Person%20Character%20Object%20Reference) (SteamId :type String))
  (bind _plantarea (Variables|Default|GetPlantArea))
  (bind _outactors (Collision|BoxOverlapActors (Transformation|GetWorldLocation _plantarea) (Variables|/Script/Engine.BoxComponent|GetBoxExtent _plantarea) (Utilities|Array|MakeArray "ObjectTypeQuery1" "ObjectTypeQuery2" "ObjectTypeQuery8" "ObjectTypeQuery7") 0 :!class /Script/Engine.KismetSystemLibrary))
  (for _array_element _outactors
    (CallFunction|DropPlant _array_element))
  (|CallParentFunction Player SteamId))

(fn ConstructionScript
  (|CallParentFunction))

(fn DropPlant
  (params (Object :type Actor%20Object%20Reference))
  (bind _asa_placeable_plant (Utilities|Casting|CastToA_Placeable_Plant Object))
  (Default|DropItemonDestruction _asa_placeable_plant))