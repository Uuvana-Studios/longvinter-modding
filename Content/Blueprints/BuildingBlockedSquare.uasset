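; Rectangular building-blocked area actor for Longvinter, using a box volume and a decal sized from BoxExtend.
; Construction zeroes BlockingRadius and sizes both, SetExtent resizes them at runtime, and the decal scale swaps the extent's X and Z.
; Entering shows the instigating player controller a hint about selling items at recyclers.
; Characters' capsules ignore the Pawn channel while inside and block it again on exit.
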(event OnComponentBeginOverlap(BlockBox)
  (params (OverlappedComponent :type Primitive%20Component%20Object%20Reference) (OtherActor :type Actor%20Object%20Reference) (OtherComp :type Primitive%20Component%20Object%20Reference) (OtherBodyIndex :type Integer) (bFromSweep :type Boolean) (SweepResult :type Hit%20Result%20Structure%20%28by%20ref%29))
  (bind _aspc_longvinter (Utilities|Casting|CastToPC_Longvinter (Game|GetInstigatorController OtherActor)))
  (Default|ShowGameplayHint _aspc_longvinter "All the items can be sold in James recycler machines, these are found in some outposts and points of interests.")
  (bind _asthird_person_character (Utilities|Casting|CastToThirdPersonCharacter OtherActor))
  (Collision|SetCollisionResponsetoChannel (Variables|/Script/Engine.Character|GetCapsuleComponent _asthird_person_character) "ECC_Pawn" "ECR_Ignore"))

(event OnComponentEndOverlap(BlockBox)
  (params (OverlappedComponent :type Primitive%20Component%20Object%20Reference) (OtherActor :type Actor%20Object%20Reference) (OtherComp :type Primitive%20Component%20Object%20Reference) (OtherBodyIndex :type Integer))
  (bind _asthird_person_character (Utilities|Casting|CastToThirdPersonCharacter OtherActor))
  (Collision|SetCollisionResponsetoChannel (Variables|/Script/Engine.Character|GetCapsuleComponent _asthird_person_character) "ECC_Pawn" "ECR_Block"))

(event EventBeginPlay
  (bind _boxextend (Variables|Default|GetBoxExtend))
  (bind (_x _y _z) (Math|Vector|BreakVector _boxextend))
  (|CallParentFunction)
  (Transformation|SetWorldScale3D (Variables|Default|GetDecal) (Math|Vector|MakeVector _z _y _x)))

(event Collision|EventActorBeginOverlap
  (params (OtherActor :type Actor%20Object%20Reference))
  (|CallParentFunction OtherActor) ; This node is disabled and will not be called.\nDrag off pins to build functionality.
)

(event EventTick
  (params (DeltaSeconds :type Float%20%28single-precision%29))
  (|CallParentFunction DeltaSeconds) ; This node is disabled and will not be called.\nDrag off pins to build functionality.
)

(fn ConstructionScript
  (bind _boxextend (Variables|Default|GetBoxExtend))
  (bind (_x _y _z) (Math|Vector|BreakVector _boxextend))
  (Variables|Default|SetBlocking%20Radius 0.0)
  (|CallParentFunction)
  (Components|Box|SetBoxExtent (Variables|Default|GetBlockBox) _boxextend true)
  (Transformation|SetWorldScale3D (Variables|Default|GetDecal) (Math|Vector|MakeVector _z _y _x)))

(fn SetExtent
  (params (BoxExtend :type Vector))
  (Variables|Default|SetBoxExtend BoxExtend)
  (Components|Box|SetBoxExtent (Variables|Default|GetBlockBox) (Variables|Default|GetBoxExtend) true)
  (Transformation|SetWorldScale3D (Variables|Default|GetDecal) (Math|Vector|MakeVector (.Z (Math|Vector|BreakVector (Variables|Default|GetBoxExtend))) (.Y (Math|Vector|BreakVector (Variables|Default|GetBoxExtend))) (.X (Math|Vector|BreakVector (Variables|Default|GetBoxExtend))))))