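; VendorDebugComponent is a helper component that fills in item name text on its owning vendor's catalogue listings, apparently for debugging.
; Its setNames event casts the owner to A_Vendor and loops over VendorCatalogue.
; For each listing it converts the vendor item and player item names to strings, stores them in the listing's name fields and writes the struct back into the array.
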(event Custom|setNames
  (params (vendor :type A%20Vendor%20Object%20Reference))
  (bind _asa_vendor (Utilities|Casting|CastToA_Vendor (Components|GetOwner)))
  (for (_array_element _array_index) (Variables|/Game/Blueprints/Vendor/A_Vendor.A_Vendor_C|GetVendorCatalogue _asa_vendor)
    (bind _structout (Utilities|Struct|SetmembersinS_VendorListing _array_element (Utilities|String|ToString(Text) (.Name (Utilities|Struct|BreakS_ItemData_Rename2 (.VendorItem (Utilities|Struct|BreakS_VendorListing _array_element))))) (Utilities|String|ToString(Text) (.Name (Utilities|Struct|BreakS_ItemData_Rename2 (.PlayerItem (Utilities|Struct|BreakS_VendorListing _array_element)))))))
    (Utilities|Array|SetArrayElem (Variables|/Game/Blueprints/Vendor/A_Vendor.A_Vendor_C|GetVendorCatalogue _asa_vendor) _array_index _structout)))

(event EventTick
  (params (DeltaSeconds :type Float%20%28single-precision%29)))