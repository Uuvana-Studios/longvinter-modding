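; Placeable tent that stands in during placement and is replaced by a player-owned home actor once placed.
; A looping timer traces vertically and enlarges BuildingArea over wood water platforms, with debug drawing left on.
; On placement, the server spawns the UGC-registry override of A_Home with the placer's SteamID, hides itself, then polls until HomeID is set before destroying itself.
; Instances flagged SpawnedByGameMode destroy themselves on BeginPlay.
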(event EventBeginPlay
  (if (Variables|Default|GetSpawnedByGameMode)
    (Actor|DestroyActor)
    (else
      (Utilities|Time|SetTimerbyFunctionName 0 "CheckWaterPlatform" 0.2 true))))

(event EventPlaced
  (params (SteamID :type String))
  (Rendering|SetVisibility (Variables|Default|GetSM_Placeable) false false)
  (Networking|SwitchHasAuthority
    (:Authority
      (bind _asa_home (Utilities|Casting|CastToA_HomeClass (Class|UGCRegistry|GetOverrideforActorClass (Class|UGCBlueprintLibrary|GetUGCRegistry) "/Game/Blueprints/A_Home.A_Home_C")))
      (bind _returnvalue (Game|SpawnActorfromClass _asa_home (Transformation|GetWorldTransform (Variables|Default|GetSM_Placeable)) "AlwaysSpawn" 0 0 0 "" false SteamID 0 "0.000000,0.000000,0.000000" (Utilities|Array|MakeArray SteamID) 0 0 0 0 0 0 false 0))
      (Rendering|SetActorHiddenInGame true)
      (if (Utilities|Array|IsEmpty (Variables|/Game/Blueprints/A_Home.A_Home_C|GetHomeID _returnvalue)) :!label _label
        (Utilities|FlowControl|Delay 0.2)
        (goto _label)
        (else
          (Actor|DestroyActor)
          (Networking|FlushNetDormancy))))
    (:Remote
      (Rendering|SetVisibility (Variables|Default|GetBuildingArea) false false))))

(fn ConstructionScript
  (|CallParentFunction))

(fn CheckWaterPlatform
  (bind _returnvalue (Transformation|GetActorLocation))
  (bind _outhit (Collision|LineTraceByChannel (+ _returnvalue "0, 0,100.000000") (- _returnvalue "0, 0,100.000000") "TraceTypeQuery1" false 0 "ForDuration" true "(R=1.000000,G=0.000000,B=0.000000,A=1.000000)" "(R=0.000000,G=1.000000,B=0.000000,A=1.000000)" 0.2))
  (if (Utilities|ClassIsChildOf (Utilities|GetClass (.hitactor _outhit)) "/Game/Blueprints/Placeables/WaterPlatforms/A_Placeable_WoodWaterPlatform.A_Placeable_WoodWaterPlatform_C")
    (Transformation|SetWorldScale3D (Variables|Default|GetBuildingArea) "20.700001,18.629999,0.360000")
    (else
      (Transformation|SetWorldScale3D (Variables|Default|GetBuildingArea) "17.250000,15.525000,0.300000"))))