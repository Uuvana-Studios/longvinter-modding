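; Placeable crafting workbench in Longvinter that binds to the home beneath it and tracks wood deposited toward an upgrade.
; On BeginPlay it traces downward, retrying each second until it finds an A_Home and destroying any workbench it hits.
; Clicking opens crafting only for the home's saved Steam IDs, then reruns the trace.
; Wood is stored as text in Comment, restored on BeginPlay, with dormancy flushed on changes.
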(event EventBeginPlay
  (bind _returnvalue (Transformation|GetActorLocation))
  (|CallParentFunction)
  (Variables|Default|SetWoodCurrent (Math|Conversions|ToInteger(Byte) (Utilities|String|ToString(Text) (Variables|Default|GetComment))))
  (Variables|Default|SetWoodCurrent (Variables|Default|GetWoodCurrent))
  (bind (_outhit _returnvalue_2) (Collision|LineTraceByChannel (Math|Vector|MakeVector (.x _returnvalue) (.y _returnvalue) (+ (.z _returnvalue) 2e+01)) (Math|Vector|MakeVector (.x _returnvalue) (.y _returnvalue) (- (.z _returnvalue) 6e+02)) "TraceTypeQuery1" false (Utilities|Array|MakeArray self) "ForDuration" :!label _label))
  (if _returnvalue_2
    (bind _asa_home (Utilities|Casting|CastToA_Home (Actor|GetParentActor (.HitActor (Collision|BreakHitResult _outhit))))
      (:then
        (Variables|Default|SetA_Home _asa_home)
        (Development|PrintString "HOME SUCCESS")
        (Networking|FlushNetDormancy))
      (:CastFailed
        (bind _asplaceable_workbench (Utilities|Casting|CastToPlaceable_Workbench (.HitActor (Collision|BreakHitResult _outhit)))
          (:then
            (Actor|DestroyActor _asplaceable_workbench))
          (:CastFailed
            _))
        (Utilities|FlowControl|Delay 1.0 :!label _label_2)
        (goto _label)))
    (else
      (goto _label_2))))

(event Collision|EventActorBeginOverlap
  (params (OtherActor :type Actor%20Object%20Reference))
  (|CallParentFunction OtherActor) ; This node is disabled and will not be called.\nDrag off pins to build functionality.
)

(event EventTick
  (params (DeltaSeconds :type Float%20%28single-precision%29))
  (|CallParentFunction DeltaSeconds) ; This node is disabled and will not be called.\nDrag off pins to build functionality.
)

(event EventClicked
  (params (Player :type Third%20Person%20Character%20Object%20Reference))
  (bind _returnvalue (Transformation|GetActorLocation))
  (bind _self self)
  (Utilities|IsValid (Variables|Default|GetA_Home)
    (:Is%20Valid
      (if (Utilities|Array|ContainsItem (Variables|/Game/Blueprints/A_Home.A_Home_C|GetsavedSteamID's (Variables|Default|GetA_Home)) (Class|AdvancedSessionsLibrary|UniqueNetIdtoString (Class|AdvancedSessionsLibrary|GetUniqueNetIDfromPlayerState (Variables|/Script/Engine.Pawn|GetPlayerState Player))))
        (Networking|FlushNetDormancy)
        (Utilities|FlowControl|Sequence
          (:then_0
            (Default|SetCooking Player false)
            (Default|OpenCrafting Player "NewEnumerator1" _self)
            (bind _aspc_longvinter (Utilities|Casting|CastToPC_Longvinter (Pawn|GetController Player)))
            (Default|ShowGameplayHint _aspc_longvinter "Some vendors sell crafting book item that shows every craftable item in the game. There is also a cooking book!"))
          (:then_1
            (Variables|/Game/ThirdPersonCPP/Blueprints/ThirdPersonCharacter.ThirdPersonCharacter_C|SetCurrentWorkbench Player _self))
          (:then_2
            (Variables|Default|SetWoodCurrent (Variables|Default|GetWoodCurrent))
            (bind (_outhit _returnvalue_2) (Collision|LineTraceByChannel (Math|Vector|MakeVector (.x _returnvalue) (.y _returnvalue) (+ (.z _returnvalue) 2e+01)) (Math|Vector|MakeVector (.x _returnvalue) (.y _returnvalue) (- (.z _returnvalue) 6e+02)) "TraceTypeQuery1" false (Utilities|Array|MakeArray self) "ForDuration" :!label _label))
            (if _returnvalue_2
              (bind _asa_home (Utilities|Casting|CastToA_Home (Actor|GetParentActor (.HitActor (Collision|BreakHitResult _outhit))))
                (:then
                  (Variables|Default|SetA_Home _asa_home)
                  (Development|PrintString "HOME SUCCESS")
                  (Networking|FlushNetDormancy))
                (:CastFailed
                  (bind _asplaceable_workbench (Utilities|Casting|CastToPlaceable_Workbench (.HitActor (Collision|BreakHitResult _outhit)))
                    (:then
                      (Actor|DestroyActor _asplaceable_workbench))
                    (:CastFailed
                      _))
                  (Utilities|FlowControl|Delay 1.0 :!label _label_2)
                  (goto _label)))
              (else
                (goto _label_2)))))))
    (:Is%20Not%20Valid
      (Default|RunonClientErrorMessage Player "Workbench could not find home, place the workbench again."))))

(fn ConstructionScript
  (|CallParentFunction))

(fn DepositWood
  (params (Amount :type Integer))
  (bind _output_get (Variables|Default|SetWoodCurrent (Math|Integer|Clamp(Integer) (+ (Variables|Default|GetWoodCurrent) Amount) 0 (Variables|Default|GetWoodToUpgrade))))
  (Variables|Default|SetComment (Utilities|Text|ToText(String) (Utilities|String|ToString(Integer) _output_get)))
  (Networking|FlushNetDormancy))

(fn OnRepWoodCurrent)