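; Placeable electricity transfer station that powers a linked receiver station and opens its own interaction window when clicked.
; Toggling it sets the receiver's generating state and rechecks electricity; its replicated offset adjusts required electricity and passes to the receiver.
; On authority, it restores StationID from item data or assigns the station count, after a random frame delay if game-mode spawned.
; Destruction removes the cable and receiver, while EndPlay removes only the cable.
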(event EventBeginPlay
  (|CallParentFunction)
  (if (Variables|Default|GetSpawnedByGameMode)
    (Class|LowEntryExtendedStandardLibrary|DelayFrames (Math|Random|RandomIntegerinRange 61 90)))
  (Networking|SwitchHasAuthority
    (:Authority
      (CallFunction|LoadStationValues))))

(event EventDropItemonDestruction
  (Utilities|Struct|SetmembersinS_ItemData_Rename2 (Variables|Default|GetItemData))
  (Actor|DestroyActor (Variables|/Game/Blueprints/Placeables/Placeable_ElectricityReceiverStation.Placeable_ElectricityReceiverStation_C|GetCableActor (Variables|Default|GetReceiverStation)))
  (|CallParentFunction))

(event EventEndPlay
  (params (EndPlayReason :type EEndPlayReason%20Enum :default "Destroyed"))
  (bind _receiverstation (Variables|Default|GetReceiverStation))
  (bind _cableactor (Variables|/Game/Blueprints/Placeables/Placeable_ElectricityReceiverStation.Placeable_ElectricityReceiverStation_C|GetCableActor _receiverstation))
  (Utilities|IsValid _receiverstation
    (:Is%20Valid
      (Utilities|IsValid _cableactor
        (:Is%20Valid
          (Actor|DestroyActor _cableactor))
        (:Is%20Not%20Valid
          _)))
    (:Is%20Not%20Valid
      _))
  (|CallParentFunction EndPlayReason))

(event EventOnReponOff
  (params (OnOff :type Boolean))
  (bind _receiverstation (Variables|Default|GetReceiverStation))
  (Utilities|IsValid _receiverstation
    (:Is%20Valid
      (Variables|/Game/Blueprints/Placeables/ElectricityDevice/A_PlaceableGenerator.A_PlaceableGenerator_C|SetGeneratingElectricity _receiverstation OnOff)
      (Default|CheckElectricity _receiverstation (Variables|/Game/Blueprints/Placeables/A_Placeable.A_Placeable_C|GetElectricityActor _receiverstation))
      (|CallParentFunction OnOff))))

(event EventClicked
  (params (Player :type Third%20Person%20Character%20Object%20Reference))
  (bind _instigator (Variables|/Script/Engine.Actor|GetInstigator Player))
  (Utilities|IsValid _instigator
    (:Is%20Valid
      (bind _aspc_longvinter (Utilities|Casting|CastToPC_Longvinter (Pawn|GetController _instigator)))
      (Default|OpenPlacebleInteractWindow _aspc_longvinter self "/Game/Blueprints/Placeables/ElectricityDevice/UMG_ElectricityTransferStation.UMG_ElectricityTransferStation_C"))))

(fn ConstructionScript
  (|CallParentFunction))

(fn LoadStationValues
  (bind _itemdataparams (Variables|Default|GetItemDataParams))
  (bind _value (CallFunction|GetItemStringField :Field "StationID" :JsonOverride _itemdataparams))
  (if (Utilities|Array|IsEmpty _value)
    (bind _outactors (Actor|GetAllActorsOfClass "Placeable_ElectricityTransferStation_C"))
    (Variables|Default|SetStationID (Utilities|Array|Length _outactors))
    (else
      (Variables|Default|SetStationID (Math|Conversions|ToInteger(Byte) _value))))
  (CallFunction|SaveStationParams))

(fn SaveStationParams
  (CallFunction|SetItemStringField (Variables|Default|GetItemData) "StationID" (Utilities|String|ToString(Integer) (Variables|Default|GetStationID))))

(fn OnRepReceiverStation)

(fn OnRepElectricityOffset
  (bind _receiverstation (Variables|Default|GetReceiverStation))
  (Variables|Default|SetrequiredElectricity (+ (Class|KismetSystemLibrary|MakeLiteralInteger 75) (Variables|Default|GetElectricityOffset)))
  (Utilities|IsValid _receiverstation
    (:Is%20Valid
      (Variables|/Game/Blueprints/Placeables/Placeable_ElectricityReceiverStation.Placeable_ElectricityReceiverStation_C|SetElectricityOffset _receiverstation (Variables|Default|GetElectricityOffset)))))