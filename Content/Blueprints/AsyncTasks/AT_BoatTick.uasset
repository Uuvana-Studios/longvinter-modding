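; Async task that ticks a boat's buoyancy off a timed sleep, computing its own delta time from UTC timestamps.
; While the boat is active and simulating physics, it runs three water traces through FloatComponent, the middle one at double strength, and sets InWater if any succeeds.
; It then snaps excessive roll and pitch back within limits, using much tighter limits when delta time is long to prevent flipping.
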(event EventExecute
  (bind _boat (Variables|Default|GetBoat))
  (Class|AsyncLibrary|Sleep 0.05)
  (Variables|Default|SetDeltaSeconds (/ (Math|Conversions|ToFloat(Integer) (Class|KismetMathLibrary|GetMilliseconds (- (Math|DateTime|UTCNow) (Variables|Default|GetLastTime)))) (Math|Float|MakeLiteralFloat 1e+03)))
  (Variables|Default|SetLastTime (Math|DateTime|UTCNow))
  (if (and (Variables|/Game/Blueprints/Vehicles/Boats/A_Boat.A_Boat_C|GetActive _boat) (Physics|IsSimulatingPhysics (Variables|/Game/Blueprints/Vehicles/Boats/A_Boat.A_Boat_C|GetCube _boat) "None"))
    (CallFunction|FloatonWater (Variables|Default|GetDeltaSeconds))
    (|PreventFlipping_2 (Variables|Default|GetDeltaSeconds))))

(event EventInitialization
  (Variables|Default|SetLastTime (Math|DateTime|UTCNow)))

(fn FloatonWater
  (params (deltaSeconds :type Float%20%28single-precision%29))
  (bind _array (Utilities|Array|MakeArray "ObjectTypeQuery9"))
  (bind _floatcomponent (Variables|Default|GetFloatComponent))
  (bind _boat (Variables|Default|GetBoat))
  (bind _tracelength (LocalVariables|GetTraceLength))
  (bind _cube (Variables|/Game/Blueprints/Vehicles/Boats/A_Boat.A_Boat_C|GetCube _boat))
  (LocalVariables|SetDelta deltaSeconds)
  (Utilities|FlowControl|Sequence
    (:then_0
      (Variables|/Game/Blueprints/Vehicles/Boats/A_Boat.A_Boat_C|SetInWater _boat false))
    (:then_1
      (bind _returnvalue (Class|FloatonWaterComponent|FloatonWater _floatcomponent (LocalVariables|GetDelta) _tracelength 1.0 _array (Variables|/Game/Blueprints/Vehicles/Boats/A_Boat.A_Boat_C|GetTrace1 _boat) _cube))
      (bind _returnvalue_2 (Class|FloatonWaterComponent|FloatonWater _floatcomponent (LocalVariables|GetDelta) _tracelength 2.0 _array (Variables|/Game/Blueprints/Vehicles/Boats/A_Boat.A_Boat_C|GetTrace2 _boat) _cube))
      (bind _returnvalue_3 (Class|FloatonWaterComponent|FloatonWater _floatcomponent (LocalVariables|GetDelta) _tracelength 1.0 _array (Variables|/Game/Blueprints/Vehicles/Boats/A_Boat.A_Boat_C|GetTrace3 _boat) _cube))
      (Variables|/Game/Blueprints/Vehicles/Boats/A_Boat.A_Boat_C|SetInWater _boat (Math|Boolean|ORBoolean _returnvalue _returnvalue_2 _returnvalue_3)))))