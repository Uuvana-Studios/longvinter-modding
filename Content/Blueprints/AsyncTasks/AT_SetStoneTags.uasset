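; An async task Blueprint that tags large stone static mesh actors with "stone".
; On Execute it loops over its StaticMeshActors array and checks each mesh component's first material slot against a hard-coded set of LargeStone materials, including snow and sand variants.
; Any match gets the tag through a unique add, so the tag is never duplicated.
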(event EventExecute
  (for _array_element (Variables|Default|GetStaticMeshActors)
    (if (Math|Boolean|ORBoolean (== (Rendering|Material|GetMaterial (Variables|/Script/Engine.StaticMeshActor|GetStaticMeshComponent _array_element) 0) "/Game/Meshes/LargeStones/Materials/MI_LargeStone01.MI_LargeStone01") (== (Rendering|Material|GetMaterial (Variables|/Script/Engine.StaticMeshActor|GetStaticMeshComponent _array_element) 0) "/Game/Meshes/LargeStones/Materials/M_LargeStoneSnow.M_LargeStoneSnow") (== (Rendering|Material|GetMaterial (Variables|/Script/Engine.StaticMeshActor|GetStaticMeshComponent _array_element) 0) "/Game/Meshes/LargeStones/Materials/M_LargeStone.M_LargeStone") (== (Rendering|Material|GetMaterial (Variables|/Script/Engine.StaticMeshActor|GetStaticMeshComponent _array_element) 0) "/Game/Meshes/LargeStones/Materials/M_LargeStoneSnow_Inst.M_LargeStoneSnow_Inst") (== (Rendering|Material|GetMaterial (Variables|/Script/Engine.StaticMeshActor|GetStaticMeshComponent _array_element) 0) "/Game/Meshes/LargeStones/Materials/MI_LargeStone01Sand.MI_LargeStone01Sand") (== (Rendering|Material|GetMaterial (Variables|/Script/Engine.StaticMeshActor|GetStaticMeshComponent _array_element) 0) "/Game/Meshes/LargeStones/Materials/MI_LargeStone01Snow.MI_LargeStone01Snow"))
      (Utilities|Array|AddUnique (Variables|/Script/Engine.Actor|GetTags _array_element) "stone"))))