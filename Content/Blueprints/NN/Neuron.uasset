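; Neuron Blueprint that computes the activation value of a single node in a neural network.
; Activate sums the weighted values from its Synapses, adds Bias and squashes the result with the logistic Sigmoid function, storing it in Value.
; A ReLU-style Max node is present in the graph but unused.
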(event Custom|Activate
  (Variables|Default|SetValue 0.0)
  (for _array_element (Variables|Default|GetSynapses)
    (bind _value (Default|GetWeightedValue _array_element))
    (Variables|Default|SetValue (+ _value (Variables|Default|GetValue))))
  (bind _output_get (Variables|Default|SetValue (+ (Variables|Default|GetValue) (Variables|Default|GetBias))))
  (Variables|Default|SetValue (CallFunction|Sigmoid _output_get)))

(fn Sigmoid
  (params (In :type Float%20%28single-precision%29))
  (return (/ 1.0 (+ 1.0 (Class|KismetMathLibrary|Exp (* In -1.0))))))