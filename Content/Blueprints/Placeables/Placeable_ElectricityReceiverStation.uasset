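; Placeable electricity receiver station that pairs with a transfer station sharing the StationID stored in its item data.
; On placement, or after a random frame delay when game-mode spawned, the server finds that station and cross-links both.
; The TransferStation RepNotify makes clients spawn a distance-sized cable between them, whose component tick later stops to settle it.
; Destruction with item drop also destroys the transfer station and cable.
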(event Custom|CreateCable
  (bind _cableend (Variables|Default|GetCableEnd))
  (bind _transferstation (Variables|Default|GetTransferStation))
  (Utilities|FlowControl|Delay 0.2)
  (Utilities|IsValid (Variables|Default|GetCableActor)
    (:Is%20Not%20Valid
      (bind _returnvalue (Game|SpawnActorfromClass "/Script/CableComponent.CableActor" (Transformation|GetWorldTransform _cableend) "AlwaysSpawn" 0 0))
      (bind _output_get (Variables|Default|SetCableActor _returnvalue))
      (Variables|/Script/CableComponent.CableComponent|SetCableLength (Variables|/Script/CableComponent.CableActor|GetCableComponent _output_get) (* (Math|Vector|Distance(Vector) (Transformation|GetWorldLocation _cableend) (Transformation|GetWorldLocation (Variables|/Game/Blueprints/Placeables/Placeable_ElectricityTransferStation.Placeable_ElectricityTransferStation_C|GetCableEnd _transferstation))) 1.15))
      (Class|CableComponent|SetAttachEndto (Variables|/Script/CableComponent.CableActor|GetCableComponent _output_get) _transferstation "CableEnd" "None")
      (Utilities|FlowControl|Delay 2e+01)
      (Components|Tick|SetComponentTickEnabled (Variables|/Script/CableComponent.CableActor|GetCableComponent _output_get) false))))

(event EventBeginPlay
  (|CallParentFunction)
  (if (Variables|Default|GetSpawnedByGameMode)
    (Class|LowEntryExtendedStandardLibrary|DelayFrames (Math|Random|RandomIntegerinRange 61 90))
    (Networking|SwitchHasAuthority
      (:Authority
        (CallFunction|LoadStationValues)))))

(event EventDropItemonDestruction
  (Utilities|Struct|SetmembersinS_ItemData_Rename2 (Variables|Default|GetItemData))
  (Actor|DestroyActor (Variables|Default|GetTransferStation))
  (|CallParentFunction))

(event EventEndPlay
  (params (EndPlayReason :type EEndPlayReason%20Enum :default "Destroyed"))
  (bind _cableactor (Variables|Default|GetCableActor))
  (Utilities|IsValid _cableactor
    (:Is%20Valid
      (Actor|DestroyActor _cableactor))
    (:Is%20Not%20Valid
      _))
  (|CallParentFunction EndPlayReason))

(event EventPlaced
  (params (SteamID :type String))
  (|CallParentFunction SteamID)
  (Networking|SwitchHasAuthority
    (:Authority
      (CallFunction|LoadStationValues))))

(fn ConstructionScript
  (|CallParentFunction))

(fn LoadStationValues
  (bind _output_get (Variables|Default|SetStationID (Math|Conversions|ToInteger(Byte) (CallFunction|GetItemStringField :Field "StationID" :JsonOverride (Variables|Default|GetItemDataParams)))))
  (bind _outactors (Actor|GetAllActorsOfClass "/Game/Blueprints/Placeables/Placeable_ElectricityTransferStation.Placeable_ElectricityTransferStation_C"))
  (bind _array_element (Utilities|Array|ForEachLoopwithBreak _outactors :!label _label)
    (:LoopBody
      (if (== (Variables|/Game/Blueprints/Placeables/Placeable_ElectricityTransferStation.Placeable_ElectricityTransferStation_C|GetStationID _array_element) (Math|Conversions|ToInteger(Byte) (Utilities|String|ToString(Integer) _output_get)))
        (Variables|Default|SetTransferStation _array_element)
        (Variables|/Game/Blueprints/Placeables/Placeable_ElectricityTransferStation.Placeable_ElectricityTransferStation_C|SetReceiverStation _array_element self)
        (goto _label Break)))))

(fn SaveStationParams
  (CallFunction|SetItemStringField (Variables|Default|GetItemData) "SelfStationID" (Utilities|String|ToString(Integer) (Variables|Default|GetStationID))))

(fn OnRepTransferStation
  (Networking|SwitchHasAuthority
    (:Remote
      (Utilities|IsValid (Variables|Default|GetTransferStation)
        (:Is%20Valid
          (CallFunction|CreateCable))))))

(fn OnRepElectricityOffset
  (Variables|Default|SetrequiredElectricity (+ (Class|KismetSystemLibrary|MakeLiteralInteger 75) (Variables|Default|GetElectricityOffset))))