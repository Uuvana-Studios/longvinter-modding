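; Brain Blueprint that builds and runs a layered, fully connected neural network sized by NeuronCounts.
; SetupBrain runs once, creating plain Nodes for the input layer and Neurons for later layers, each linked by Synapses to every member of the previous layer.
; All units share one flat array in layer order, which Fire walks to activate each Neuron.
; GetInputs and GetOutputs slice the first and last layers from that array.
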(event Custom|Setup%20Brain
  (bind _self self)
  (bind _neurons (Variables|Default|GetNeurons))
  (Utilities|FlowControl|DoOnce false
    (:Completed
      (for (_array_element _array_index) (Variables|Default|GetNeuron%20Counts)
        (for _index (range 0 (- _array_element 1))
          (if (== _array_index 0)
            (bind _returnvalue (Game|ConstructObjectfromClass "/Game/Blueprints/NN/Node.Node_C" _self))
            (Utilities|Array|Add _neurons _returnvalue)
            (else
              (bind _returnvalue_2 (Game|ConstructObjectfromClass "/Game/Blueprints/NN/Neuron.Neuron_C" _self))
              (Utilities|Array|Add _neurons _returnvalue_2)
              (bind _number_of_neurons (CallFunction|CountNeuronsinLayers 0 (- _array_index 1)))
              (for _index_2 (range (- _number_of_neurons (Utilities|Array|Get(acopy) (Variables|Default|GetNeuron%20Counts) (- _array_index 1))) (- _number_of_neurons 1))
                (bind _returnvalue_3 (Game|ConstructObjectfromClass "/Game/Blueprints/NN/Synapse.Synapse_C" self))
                (Default|SetupSynapse _returnvalue_3 (Utilities|Array|Get(acopy) (Variables|Default|GetNeurons) _index_2) _returnvalue_2)
                (Utilities|Array|Add (Variables|/Game/Blueprints/NN/Neuron.Neuron_C|GetSynapses _returnvalue_2) _returnvalue_3)))))))))

(event Custom|Fire
  (for _array_element (Variables|Default|GetNeurons)
    (bind _asneuron (Utilities|Casting|CastToNeuron _array_element))
    (Default|Activate _asneuron)))

(fn CountNeuronsinLayers
  (params (Start%20Layer :type Integer) (End%20Layer :type Integer))
  (for _index (range Start%20Layer End%20Layer)
    (LocalVariables|SetNeuron%20Count (+ (Utilities|Array|Get(acopy) (Variables|Default|GetNeuron%20Counts) _index) (LocalVariables|GetNeuron%20Count))))
  (return (LocalVariables|GetNeuron%20Count)))

(fn GetOutputs
  (bind _neurons (Variables|Default|GetNeurons))
  (bind _neuron_counts (Variables|Default|GetNeuron%20Counts))
  (for _index (range (- (Utilities|Array|Length _neurons) (Utilities|Array|Get(acopy) _neuron_counts (Utilities|Array|LastIndex _neuron_counts))) (Utilities|Array|LastIndex _neurons))
    (Utilities|Array|Add (LocalVariables|Get_Outputs) (.AsNeuron (Utilities|Casting|CastToNeuron (Utilities|Array|Get(acopy) (Variables|Default|GetNeurons) _index)))))
  (return (LocalVariables|Get_Outputs)))

(fn GetInputs
  (for _index (range 0 (- (Utilities|Array|Get(acopy) (Variables|Default|GetNeuron%20Counts)) 1))
    (Utilities|Array|Add (LocalVariables|Get_Inputs) (Utilities|Array|Get(acopy) (Variables|Default|GetNeurons) _index)))
  (return (LocalVariables|Get_Inputs)))