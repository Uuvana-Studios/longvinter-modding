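; Placeable shop gate whose door swings open and closed with sound.
; A RotateAnim event takes a Reverse flag, plays one of two door sounds at the gate's location, then restarts a timeline forward from the start or backward from the end.
; The timeline's negated Rotation track drives the Door component's relative pitch at a fixed yaw.
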(event EventBeginPlay
  (|CallParentFunction) ; This node is disabled and will not be called.\nDrag off pins to build functionality.
)

(event Collision|EventActorBeginOverlap
  (params (OtherActor :type Actor%20Object%20Reference))
  (|CallParentFunction OtherActor) ; This node is disabled and will not be called.\nDrag off pins to build functionality.
)

(event EventTick
  (params (DeltaSeconds :type Float%20%28single-precision%29))
  (|CallParentFunction DeltaSeconds) ; This node is disabled and will not be called.\nDrag off pins to build functionality.
)

(event EventRotateAnim
  (params (Reverse :type Boolean))
  (bind _returnvalue (Transformation|GetActorLocation))
  (if Reverse
    (Audio|PlaySoundatLocation "/Game/Audio/Misc/WAV_DoorOpen_02.WAV_DoorOpen_02" _returnvalue "0, 0, 0" 1.0 1.0 0.0 0 0 0)
    (Utilities|FlowControl|Sequence
      (:then_0
        (bind _rotation (Timeline|Timeline_0 Stop)
          (:Update
            (Transformation|SetRelativeRotation (Variables|Default|GetDoor) (Math|Rotator|MakeRotator 0.0 (* _rotation -1.0) -9e+01) false false))))
      (:then_1
        (Timeline|Timeline_0 ReverseFromEnd)))
    (else
      (Audio|PlaySoundatLocation "/Game/Audio/Misc/WAV_DoorOpen_01.WAV_DoorOpen_01" _returnvalue "0, 0, 0" 1.0 1.0 0.0 0 0 0)
      (Utilities|FlowControl|Sequence
        (:then_0
          (Timeline|Timeline_0 Stop))
        (:then_1
          (Timeline|Timeline_0 PlayFromStart))))))

(fn ConstructionScript
  (|CallParentFunction))